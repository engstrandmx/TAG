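; TAGGameMode_BP is the game mode Blueprint that toggles start-game objects across round phases and adjusts soundtrack parameters at game end.
; Pre-game start calls Trigger with true on each StartGameObjects entry, and round start calls it with false.
; Game end sets the Time and Win/Lose parameters on a Soundtrack event instance.
; The code that would play and store that soundtrack is disconnected, so BeginPlay only checks a flag.
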(event EventBeginPlay
  (if (Variables|Default|GetSoundtrackStarted)
    _))

(event EventTick
  (params (DeltaSeconds :type Float%20%28single-precision%29)))

(event EventOnRoundStart
  (for _array_element (Variables|Default|GetStartGameObjects)
    (Default|Trigger _array_element false)))

(event EventOnGameEnd
  (bind _soundtrack (Variables|Default|GetSoundtrack))
  (Class|FMODBlueprintStatics|EventInstanceSetParameter _soundtrack "Time" 1.0)
  (Class|FMODBlueprintStatics|EventInstanceSetParameter _soundtrack "Win/Lose" 0.0))

(event EventOnPreGameStart
  (for _array_element (Variables|Default|GetStartGameObjects)
    (Default|Trigger _array_element true)))

(fn ConstructionScript)