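; Trumpet spawner that summons the level's cow knight by teleporting the existing CowBP_Base actor to its SpawnPoint rather than creating one.
; PressSpawn is Busy-guarded, plays the call sound, waits briefly, then moves the cow and resets its water, follow and movement state to Wandering.
; SpawnCowKnight optionally shifts the destination sideways when gnome or troll is too close.
; The troll's first extras flag enlarges the cow; the scale timeline is unused.
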(event Custom|Press%20Spawn
  (if (not (Variables|Default|GetBusy))
    (Variables|Default|SetBusy true)
    (Class|FMODBlueprintStatics|PlayEventatLocation "/Game/FMOD/Events/Sfx/Cow_call.Cow_call" (Math|Conversions|ToTransform(Vector) (Transformation|GetActorLocation)))
    (Utilities|FlowControl|Delay 0.8)
    (bind _success (CallFunction|SpawnCowKnight))
    (if _success
      (bind _outactors (Actor|GetAllActorsOfClass "/Game/Blueprints/Characters/CowBP_Base.CowBP_Base_C"))
      (bind _outactors_2 (Actor|GetAllActorsOfClass "/Script/TAG.WaterField"))
      (Class|WaterField|RemovefromWaterActors _outactors_2 (Utilities|Array|Get(acopy) _outactors))
      (Transformation|SetActorRotation (Utilities|Array|Get(acopy) _outactors) (Transformation|GetWorldRotation (Variables|Default|GetSpawnPoint)))
      (Default|ChangeState (Utilities|Array|Get(acopy) _outactors) "VE_Wandering")
      (Components|Movement|StopMovementImmediately (Variables|/Script/Engine.Character|GetCharacterMovement (Utilities|Array|Get(acopy) _outactors)))
      (Default|StopFollowing (Utilities|Array|Get(acopy) _outactors))
      (bind _outactors_3 (Actor|GetAllActorsOfClass "/Game/Blueprints/Characters/TrollCharacter_Base.TrollCharacter_Base_C"))
      (if (Utilities|Array|Get(acopy) (Variables|/Game/Blueprints/Characters/TrollCharacter_Base.TrollCharacter_Base_C|GetExtrasActivated (Utilities|Array|Get(acopy) _outactors_3)))
        (Transformation|SetActorRelativeScale3D (Utilities|Array|Get(acopy) _outactors) "3.000000,3.000000,3.000000")
        (Variables|Default|SetBusy false)
        (else
          (Variables|Default|SetBusy false))))))

(event Custom|ResetCollision
  (bind _sphere (Variables|Default|GetSphere))
  (Transformation|SetWorldScale3D _sphere "0, 0, 0")
  (Transformation|SetWorldScale3D _sphere (Variables|Default|GetHitboxScale)))

(event Collision|EventActorBeginOverlap
  (params (OtherActor :type Actor%20Object%20Reference)))

(event EventTick
  (params (DeltaSeconds :type Float%20%28single-precision%29)))

(fn ConstructionScript
  (Transformation|SetWorldScale3D (Variables|Default|GetSphere) (Variables|Default|GetHitboxScale)))

(fn SpawnCowKnight
  (bind _returnvalue (Transformation|GetActorRightVector))
  (Variables|Default|SetAdjusted%20Location "0, 0, 0")
  (if (Variables|Default|GetAutoAdjustSpawn)
    (Utilities|FlowControl|Sequence
      (:then_0
        (bind _outactors (Actor|GetAllActorsOfClass "/Game/Blueprints/Characters/Instances/GnomeCharacter_Instance.GnomeCharacter_Instance_C"))
        (if (> (Utilities|Array|Length _outactors) 0)
          (bind _is_close (CallFunction|CheckDistance (Utilities|Array|Get(acopy) _outactors) 1e+02))
          (if _is_close
            (if (Variables|Default|GetAutoAdjustRightSide) :!label _label
              (Variables|Default|SetAdjusted%20Location (* _returnvalue 2e+02))
              (else
                (Variables|Default|SetAdjusted%20Location (* _returnvalue -2e+02)))))))
      (:then_1
        (bind _outactors_2 (Actor|GetAllActorsOfClass "/Game/Blueprints/Characters/Instances/TrollCharacter_Instance.TrollCharacter_Instance_C"))
        (bind _is_close_2 (CallFunction|CheckDistance (Utilities|Array|Get(acopy) _outactors_2) 1e+02))
        (if _is_close_2
          (goto _label)))
      (:then_2
        (bind _outactors_3 (Actor|GetAllActorsOfClass "/Game/Blueprints/Characters/CowBP_Base.CowBP_Base_C" :!label _label_2))
        (Transformation|SetActorLocation (Utilities|Array|Get(acopy) _outactors_3) (+ (Transformation|GetWorldLocation (Variables|Default|GetSpawnPoint)) (Variables|Default|GetAdjusted%20Location)) false true)
        (return true)))
    (else
      (goto _label_2))))

(fn CheckDistance
  (params (Other%20Actor :type Actor%20Object%20Reference) (Distance :type Float%20%28single-precision%29))
  (return (< (Math|Vector|VectorLength (- (Transformation|GetWorldLocation (Variables|/Script/Engine.Actor|GetRootComponent Other%20Actor)) (Transformation|GetWorldLocation (Variables|Default|GetSpawnPoint)))) Distance)))