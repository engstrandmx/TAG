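; TriggerableWall is a wall actor that can be switched on and off through its Trigger event.
; An active trigger shows the mesh and enables query and physics collision, while an inactive one hides it and disables collision.
; On BeginPlay it adds itself to the StartGameObjects list on TAGGameMode_BP, provided that game mode is in use.
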(event EventBeginPlay
  (bind _astaggame_mode_bp (Utilities|Casting|CastToTAGGameMode_BP (Game|GetGameMode)))
  (Utilities|Array|Add (Variables|/Game/Blueprints/TAGGameMode_BP.TAGGameMode_BP_C|GetStartGameObjects _astaggame_mode_bp) self))

(event Collision|EventActorBeginOverlap
  (params (OtherActor :type Actor%20Object%20Reference)))

(event EventTick
  (params (DeltaSeconds :type Float%20%28single-precision%29)))

(event EventTrigger
  (params (Active :type Boolean))
  (bind _mesh (Variables|Default|GetMesh))
  (Rendering|SetVisibility _mesh Active false)
  (if Active
    (Collision|SetCollisionEnabled _mesh "QueryAndPhysics")
    (else
      (Collision|SetCollisionEnabled _mesh "NoCollision"))))

(fn ConstructionScript
  (|CallParentFunction))