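; Lookat_Trigger_BP is a one-shot trigger volume that fires a linked Sweep or Lookat object when overlapped.
; The first overlap sets Active, optionally resets the collectible count through TAGGameMode_BP, then waits briefly.
; It can then start crater music via Music_handlerlvl6 before triggering Sweep if set, otherwise Lookat.
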(event OnComponentBeginOverlap(TriggerBox)
  (params (OverlappedComponent :type Primitive%20Component%20Object%20Reference) (OtherActor :type Actor%20Object%20Reference) (OtherComp :type Primitive%20Component%20Object%20Reference) (OtherBodyIndex :type Integer) (bFromSweep :type Boolean) (SweepResult :type Hit%20Result%20Structure%20%28by%20ref%29))
  (if (not (Variables|Default|GetActive))
    (Variables|Default|SetActive true)
    (if (Variables|Default|GetResetCollectibles)
      (bind _astaggame_mode_bp (Utilities|Casting|CastToTAGGameMode_BP (Game|GetGameMode)))
      (Default|ResetCollectibleCount _astaggame_mode_bp))
    (Utilities|FlowControl|Delay 0.1)
    (if (Variables|Default|GetStartCraterMusic)
      (bind _outactors (Actor|GetAllActorsOfClass "/Game/Blueprints/Audio/Music_handlerlvl6.Music_handlerlvl6_C"))
      (Default|StartCrater _outactors))
    (if (!= (Variables|Default|GetSweep) 0)
      (Default|Trigger (Variables|Default|GetSweep))
      (else
        (Default|Trigger (Variables|Default|GetLookat))))))

(event EventBeginPlay)

(event Collision|EventActorBeginOverlap
  (params (OtherActor :type Actor%20Object%20Reference)))

(event EventTick
  (params (DeltaSeconds :type Float%20%28single-precision%29)))

(fn ConstructionScript)