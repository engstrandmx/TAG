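; Log actor that toggles a forest ("Skog") snapshot audio component for lumber sound, depending on the active character.
; StartTriggering and StopTriggering set an active flag and play or stop the audio.
; While active, SnapshotCharacterSwitch asks TAGGameMode_BP for the current player type, playing for Gnome and stopping for Troll.
; Capsule overlap events are empty, and the gnome class checks are disconnected.
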(event OnComponentBeginOverlap(Capsule)
  (params (OverlappedComponent :type Primitive%20Component%20Object%20Reference) (OtherActor :type Actor%20Object%20Reference) (OtherComp :type Primitive%20Component%20Object%20Reference) (OtherBodyIndex :type Integer) (bFromSweep :type Boolean) (SweepResult :type Hit%20Result%20Structure%20%28by%20ref%29)))

(event OnComponentEndOverlap(Capsule)
  (params (OverlappedComponent :type Primitive%20Component%20Object%20Reference) (OtherActor :type Actor%20Object%20Reference) (OtherComp :type Primitive%20Component%20Object%20Reference) (OtherBodyIndex :type Integer)))

(event Custom|Mumma)

(event Custom|Start%20Triggering
  (Variables|Default|SetlumberSoundActive true)
  (Class|FMODAudioComponent|Play (Variables|/Script/FMODStudio.FMODAmbientSound|GetAudioComponent (Variables|Default|Getsnapshot_skog))))

(event Custom|Stop%20Triggering
  (Variables|Default|SetlumberSoundActive false)
  (Class|FMODAudioComponent|Stop (Variables|/Script/FMODStudio.FMODAmbientSound|GetAudioComponent (Variables|Default|Getsnapshot_skog))))

(event Custom|SnapshotCharacterSwitch
  (bind _snapshot_skog (Variables|Default|Getsnapshot_skog))
  (bind _audiocomponent (Variables|/Script/FMODStudio.FMODAmbientSound|GetAudioComponent _snapshot_skog))
  (if (Variables|Default|GetlumberSoundActive)
    (bind _astaggame_mode_bp (Utilities|Casting|CastToTAGGameMode_BP (Game|GetGameMode)))
    (bind _returnvalue (Class|TAGGameMode|GetCurrentPlayerType _astaggame_mode_bp))
    (switch Utilities|FlowControl|Switch|SwitchonEPlayerType _returnvalue
      (:Troll
        (Class|FMODAudioComponent|Stop _audiocomponent))
      (:Gnome
        (Class|FMODAudioComponent|Play _audiocomponent)))))

(event EventBeginPlay)

(event Collision|EventActorBeginOverlap
  (params (OtherActor :type Actor%20Object%20Reference)))

(event EventTick
  (params (DeltaSeconds :type Float%20%28single-precision%29)))

(fn ConstructionScript)