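; Triggerable camera-beat actor that turns the player characters' view toward itself, detaches their follow cameras, then triggers a linked Lookat after a delay.
; Trigger, called directly or via TriggerActor, uses the game mode's player type: Troll affects only the troll, Gnome affects both.
; It can disable character input.
; The start-to-forward-offset sweep is unfinished: MoveToTarget gets set, but the lerp move never runs.
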(event OnTrigger(TriggerActor)
  (Utilities|FlowControl|Sequence
    (:then_0
      (bind _astaggame_mode_bp (Utilities|Casting|CastToTAGGameMode_BP (Game|GetGameMode)))
      (Variables|Default|SetGameMode%20Ref _astaggame_mode_bp)
      (bind _returnvalue (Class|TAGGameMode|GetCurrentPlayerType _astaggame_mode_bp))
      (switch Utilities|FlowControl|Switch|SwitchonEPlayerType _returnvalue
        (:Troll
          (bind _returnvalue_2 (Class|TAGGameMode|GetTrollCharacter _astaggame_mode_bp :!label _label))
          (Class|TAGCharacter|LookatActor _returnvalue_2 self 5e+01 3.0 false)
          (Transformation|DetachFromComponent (Variables|/Script/TAG.TAGCharacter|GetFollowCamera _returnvalue_2) "KeepWorld" "KeepWorld" "KeepRelative" true)
          (Utilities|FlowControl|Delay (Variables|Default|GetTimeStill)))
        (:Gnome
          (Utilities|FlowControl|Sequence
            (:then_0
              (goto _label))
            (:then_1
              (bind _returnvalue_3 (Class|TAGGameMode|GetGnomeCharacter _astaggame_mode_bp))
              (Class|TAGCharacter|LookatActor _returnvalue_3 self 5e+01 3.0 false)
              (Transformation|DetachFromComponent (Variables|/Script/TAG.TAGCharacter|GetFollowCamera _returnvalue_3) "KeepWorld" "KeepWorld" "KeepRelative" true)
              (Utilities|FlowControl|Delay (Variables|Default|GetTimeStill))))))
      (Default|Trigger (Variables|Default|GetLookat)))
    (:then_1
      (Variables|Default|SetMoveToTarget true))
    (:then_2
      (if (Variables|Default|GetDisable%20Input)
        (bind _returnvalue_4 (Class|TAGGameMode|GetTrollCharacter (Variables|Default|GetGameMode%20Ref)))
        (Input|DisableInput _returnvalue_4 0)
        (bind _outactors (Actor|GetAllActorsOfClass "/Game/Blueprints/Characters/Instances/GnomeCharacter_Instance.GnomeCharacter_Instance_C"))
        (if (== (Utilities|Array|Length _outactors) 1)
          (bind _returnvalue_5 (Class|TAGGameMode|GetGnomeCharacter (Variables|Default|GetGameMode%20Ref)))
          (Input|DisableInput _returnvalue_5 0))))))

(event Custom|Trigger
  (Utilities|FlowControl|Sequence
    (:then_0
      (bind _astaggame_mode_bp (Utilities|Casting|CastToTAGGameMode_BP (Game|GetGameMode)))
      (Variables|Default|SetGameMode%20Ref _astaggame_mode_bp)
      (bind _returnvalue (Class|TAGGameMode|GetCurrentPlayerType _astaggame_mode_bp))
      (switch Utilities|FlowControl|Switch|SwitchonEPlayerType _returnvalue
        (:Troll
          (bind _returnvalue_2 (Class|TAGGameMode|GetTrollCharacter _astaggame_mode_bp :!label _label))
          (Class|TAGCharacter|LookatActor _returnvalue_2 self 5e+01 3.0 false)
          (Transformation|DetachFromComponent (Variables|/Script/TAG.TAGCharacter|GetFollowCamera _returnvalue_2) "KeepWorld" "KeepWorld" "KeepRelative" true)
          (Utilities|FlowControl|Delay (Variables|Default|GetTimeStill)))
        (:Gnome
          (Utilities|FlowControl|Sequence
            (:then_0
              (goto _label))
            (:then_1
              (bind _returnvalue_3 (Class|TAGGameMode|GetGnomeCharacter _astaggame_mode_bp))
              (Class|TAGCharacter|LookatActor _returnvalue_3 self 5e+01 3.0 false)
              (Transformation|DetachFromComponent (Variables|/Script/TAG.TAGCharacter|GetFollowCamera _returnvalue_3) "KeepWorld" "KeepWorld" "KeepRelative" true)
              (Utilities|FlowControl|Delay (Variables|Default|GetTimeStill))))))
      (Default|Trigger (Variables|Default|GetLookat)))
    (:then_1
      (Variables|Default|SetMoveToTarget true))
    (:then_2
      (if (Variables|Default|GetDisable%20Input)
        (bind _returnvalue_4 (Class|TAGGameMode|GetTrollCharacter (Variables|Default|GetGameMode%20Ref)))
        (Input|DisableInput _returnvalue_4 0)
        (bind _outactors (Actor|GetAllActorsOfClass "/Game/Blueprints/Characters/Instances/GnomeCharacter_Instance.GnomeCharacter_Instance_C"))
        (if (== (Utilities|Array|Length _outactors) 1)
          (bind _returnvalue_5 (Class|TAGGameMode|GetGnomeCharacter (Variables|Default|GetGameMode%20Ref)))
          (Input|DisableInput _returnvalue_5 0))))))

(event EventBeginPlay
  (bind _returnvalue (Transformation|GetActorLocation))
  (Variables|Default|SetInitialLocation _returnvalue)
  (Variables|Default|SetEndLocation (+ _returnvalue (* (Transformation|GetActorForwardVector) (Variables|Default|GetMoveDistance)))))

(event Collision|EventActorBeginOverlap
  (params (OtherActor :type Actor%20Object%20Reference)))

(event EventTick
  (params (DeltaSeconds :type Float%20%28single-precision%29)))

(fn ConstructionScript)