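; A triggerable look-at point that briefly draws the player characters' cameras to itself.
; Trigger or TriggerActor's OnTrigger gets the current player type from TAGGameMode_BP: Troll affects only the Troll, Gnome affects both.
; LookAtActor runs with the FollowCamera detached, then a delay precedes reattachment and reset, with optional input lock on both characters.
; Movement toward EndLocation is unfinished: MoveToTarget is set but the lerp never runs.
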(event OnTrigger(TriggerActor)
  (bind _time (Variables|Default|GetTime))
  (bind _time_2 (Variables|Default|GetTime))
  (Utilities|FlowControl|Sequence
    (:then_0
      (bind _astaggame_mode_bp (Utilities|Casting|CastToTAGGameMode_BP (Game|GetGameMode)))
      (Variables|Default|SetGameMode%20Ref _astaggame_mode_bp)
      (bind _returnvalue (Class|TAGGameMode|GetCurrentPlayerType _astaggame_mode_bp))
      (switch Utilities|FlowControl|Switch|SwitchonEPlayerType _returnvalue
        (:Troll
          (bind _returnvalue_2 (Class|TAGGameMode|GetTrollCharacter _astaggame_mode_bp :!label _label))
          (Class|TAGCharacter|LookatActor _returnvalue_2 self _time (Variables|Default|GetSmoothness) false)
          (Transformation|DetachFromComponent (Variables|/Script/TAG.TAGCharacter|GetFollowCamera _returnvalue_2) "KeepWorld" "KeepWorld" "KeepRelative" true)
          (Utilities|FlowControl|Delay _time)
          (Transformation|AttachComponentToComponent (Variables|/Script/TAG.TAGCharacter|GetFollowCamera _returnvalue_2) (Variables|/Script/TAG.TAGCharacter|GetCameraBoom _returnvalue_2) (Transformation|GetAttachSocketName (Variables|/Script/TAG.TAGCharacter|GetCameraBoom _returnvalue_2)) "KeepWorld" "KeepWorld" "KeepRelative" true)
          (Class|TAGCharacter|ResetCamera _returnvalue_2))
        (:Gnome
          (Utilities|FlowControl|Sequence
            (:then_0
              (goto _label))
            (:then_1
              (bind _returnvalue_3 (Class|TAGGameMode|GetGnomeCharacter _astaggame_mode_bp))
              (Class|TAGCharacter|LookatActor _returnvalue_3 self _time_2 (Variables|Default|GetSmoothness) false)
              (Transformation|DetachFromComponent (Variables|/Script/TAG.TAGCharacter|GetFollowCamera _returnvalue_3) "KeepWorld" "KeepWorld" "KeepRelative" true)
              (Utilities|FlowControl|Delay _time_2)
              (Transformation|AttachComponentToComponent (Variables|/Script/TAG.TAGCharacter|GetFollowCamera _returnvalue_3) (Variables|/Script/TAG.TAGCharacter|GetCameraBoom _returnvalue_3) (Transformation|GetAttachSocketName (Variables|/Script/TAG.TAGCharacter|GetCameraBoom _returnvalue_3)) "KeepWorld" "KeepWorld" "KeepRelative" true)
              (Class|TAGCharacter|ResetCamera _returnvalue_3)))))
      (if (Variables|Default|GetDisable%20Input)
        (bind _returnvalue_4 (Class|TAGGameMode|GetTrollCharacter (Variables|Default|GetGameMode%20Ref)))
        (Input|EnableInput _returnvalue_4 0)
        (bind _returnvalue_5 (Class|TAGGameMode|GetGnomeCharacter (Variables|Default|GetGameMode%20Ref)))
        (Input|EnableInput _returnvalue_5 0)))
    (:then_1
      (Variables|Default|SetMoveToTarget true))
    (:then_2
      (if (Variables|Default|GetDisable%20Input)
        (bind _returnvalue_6 (Class|TAGGameMode|GetTrollCharacter (Variables|Default|GetGameMode%20Ref)))
        (Input|DisableInput _returnvalue_6 0)
        (bind _returnvalue_7 (Class|TAGGameMode|GetGnomeCharacter (Variables|Default|GetGameMode%20Ref)))
        (Input|DisableInput _returnvalue_7 0)))))

(event Custom|Trigger
  (bind _time (Variables|Default|GetTime))
  (bind _time_2 (Variables|Default|GetTime))
  (Utilities|FlowControl|Sequence
    (:then_0
      (bind _astaggame_mode_bp (Utilities|Casting|CastToTAGGameMode_BP (Game|GetGameMode)))
      (Variables|Default|SetGameMode%20Ref _astaggame_mode_bp)
      (bind _returnvalue (Class|TAGGameMode|GetCurrentPlayerType _astaggame_mode_bp))
      (switch Utilities|FlowControl|Switch|SwitchonEPlayerType _returnvalue
        (:Troll
          (bind _returnvalue_2 (Class|TAGGameMode|GetTrollCharacter _astaggame_mode_bp :!label _label))
          (Class|TAGCharacter|LookatActor _returnvalue_2 self _time (Variables|Default|GetSmoothness) false)
          (Transformation|DetachFromComponent (Variables|/Script/TAG.TAGCharacter|GetFollowCamera _returnvalue_2) "KeepWorld" "KeepWorld" "KeepRelative" true)
          (Utilities|FlowControl|Delay _time)
          (Transformation|AttachComponentToComponent (Variables|/Script/TAG.TAGCharacter|GetFollowCamera _returnvalue_2) (Variables|/Script/TAG.TAGCharacter|GetCameraBoom _returnvalue_2) (Transformation|GetAttachSocketName (Variables|/Script/TAG.TAGCharacter|GetCameraBoom _returnvalue_2)) "KeepWorld" "KeepWorld" "KeepRelative" true)
          (Class|TAGCharacter|ResetCamera _returnvalue_2))
        (:Gnome
          (Utilities|FlowControl|Sequence
            (:then_0
              (goto _label))
            (:then_1
              (bind _returnvalue_3 (Class|TAGGameMode|GetGnomeCharacter _astaggame_mode_bp))
              (Class|TAGCharacter|LookatActor _returnvalue_3 self _time_2 (Variables|Default|GetSmoothness) false)
              (Transformation|DetachFromComponent (Variables|/Script/TAG.TAGCharacter|GetFollowCamera _returnvalue_3) "KeepWorld" "KeepWorld" "KeepRelative" true)
              (Utilities|FlowControl|Delay _time_2)
              (Transformation|AttachComponentToComponent (Variables|/Script/TAG.TAGCharacter|GetFollowCamera _returnvalue_3) (Variables|/Script/TAG.TAGCharacter|GetCameraBoom _returnvalue_3) (Transformation|GetAttachSocketName (Variables|/Script/TAG.TAGCharacter|GetCameraBoom _returnvalue_3)) "KeepWorld" "KeepWorld" "KeepRelative" true)
              (Class|TAGCharacter|ResetCamera _returnvalue_3)))))
      (if (Variables|Default|GetDisable%20Input)
        (bind _returnvalue_4 (Class|TAGGameMode|GetTrollCharacter (Variables|Default|GetGameMode%20Ref)))
        (Input|EnableInput _returnvalue_4 0)
        (bind _returnvalue_5 (Class|TAGGameMode|GetGnomeCharacter (Variables|Default|GetGameMode%20Ref)))
        (Input|EnableInput _returnvalue_5 0)))
    (:then_1
      (Variables|Default|SetMoveToTarget true))
    (:then_2
      (if (Variables|Default|GetDisable%20Input)
        (bind _returnvalue_6 (Class|TAGGameMode|GetTrollCharacter (Variables|Default|GetGameMode%20Ref)))
        (Input|DisableInput _returnvalue_6 0)
        (bind _returnvalue_7 (Class|TAGGameMode|GetGnomeCharacter (Variables|Default|GetGameMode%20Ref)))
        (Input|DisableInput _returnvalue_7 0)))))

(event EventBeginPlay
  (bind _returnvalue (Transformation|GetActorLocation))
  (Variables|Default|SetInitialLocation _returnvalue)
  (Variables|Default|SetEndLocation (+ _returnvalue (* (Transformation|GetActorForwardVector) (Variables|Default|GetMoveDistance)))))

(event Collision|EventActorBeginOverlap
  (params (OtherActor :type Actor%20Object%20Reference)))

(event EventTick
  (params (DeltaSeconds :type Float%20%28single-precision%29)))

(fn ConstructionScript)