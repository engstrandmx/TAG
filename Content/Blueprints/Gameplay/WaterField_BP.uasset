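; WaterField_BP is a water area that slows entering actors and makes cows float.
; OnActorEnter turns on gravity, resets movement gravity scale, damps velocity to a fifth and plays an event at the actor's transform.
; Entering actors derived from CowBP_Base switch to the Floating state.
; The construction script keeps a referenced WaterVolume matched to the field's location and scale.
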(event EventBeginPlay)

(event Collision|EventActorBeginOverlap
  (params (OtherActor :type Actor%20Object%20Reference)))

(event EventTick
  (params (DeltaSeconds :type Float%20%28single-precision%29)))

(event EventOnActorEnter
  (params (EnteringActor :type Actor%20Object%20Reference))
  (bind _returnvalue (Actor|GetComponentbyClass EnteringActor "/Script/Engine.CharacterMovementComponent"))
  (bind _asprimitive_component (Utilities|Casting|CastToPrimitiveComponent (VehicleSound|GetRootComponent EnteringActor)))
  (Physics|SetEnableGravity _asprimitive_component true)
  (Variables|/Script/Engine.CharacterMovementComponent|SetGravityScale _returnvalue 1.0)
  (Variables|/Script/Engine.MovementComponent|SetVelocity _returnvalue (* (Variables|/Script/Engine.MovementComponent|GetVelocity _returnvalue) 0.2))
  (Class|FMODBlueprintStatics|PlayEventatLocation 0 (Transformation|GetActorTransform EnteringActor))
  (bind _ascow_bp_base (Utilities|Casting|CastToCowBP_Base EnteringActor))
  (Default|ChangeState _ascow_bp_base "VE_Floating"))

(fn ConstructionScript
  (bind _self self)
  (bind _watervolume (Variables|Default|GetWaterVolume))
  (if (!= (Variables|Default|GetWaterVolume) 0)
    (Transformation|SetActorLocation _watervolume (Transformation|GetActorLocation _self) false false)
    (Transformation|SetActorScale3D _watervolume (Transformation|GetActorScale3D _self))))