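; Fairy ring trigger that holds tagged doors open while it is occupied.
; Start and stop triggering events update a touch count, set the StandingOnTrigger blackboard key on cows and drive spore effects and sound; Tick calls open or close on DoorToggleBP actors matching its first tag when occupancy changes.
; Incoming signals control ring particles by neighbor count, while a linked TriggerActor toggles the disabled state and RingColor-tinted light.
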(event OnComponentBeginOverlap(TriggerBox)
  (params (OverlappedComponent :type Primitive%20Component%20Object%20Reference) (OtherActor :type Actor%20Object%20Reference) (OtherComp :type Primitive%20Component%20Object%20Reference) (OtherBodyIndex :type Integer) (bFromSweep :type Boolean) (SweepResult :type Hit%20Result%20Structure%20%28by%20ref%29))
  ;[1 1 1] Count Touching Components
)

(event OnComponentEndOverlap(TriggerBox)
  (params (OverlappedComponent :type Primitive%20Component%20Object%20Reference) (OtherActor :type Actor%20Object%20Reference) (OtherComp :type Primitive%20Component%20Object%20Reference) (OtherBodyIndex :type Integer))
  ;[1 1 1] Count Touching Components
)

(event OnTrigger(TriggerActor)
  (bind _pointlight (Variables|Default|GetPointLight))
  ;[1 1 1] On Trigger
  (bind _output_get (Variables|Default|SetbDisabled (not (Variables|Default|GetbDisabled))))
  (if _output_get
    (Rendering|SetVisibility _pointlight false false)
    (else
      (Rendering|SetVisibility _pointlight true false))))

(event Custom|Start%20Triggering
  (bind _returnvalue (Transformation|GetActorTransform))
  ;[1 1 1] Count Touching Components
  (Variables|Default|SetTouchingComponents (+ (Variables|Default|GetTouchingComponents) 1))
  ;[1 1 1] Set Cow Bool
  (if (and (== (Utilities|GetClass (stale OnComponentBeginOverlap(TriggerBox) OtherActor)) "/Script/TAG.CowCharacter") (not (Variables|Default|GetbTriggerFinished)))
    (bind _ascow_bp_base (Utilities|Casting|CastToCowBP_Base (stale OnComponentBeginOverlap(TriggerBox) OtherActor)))
    (AI|Components|Blackboard|SetValueasBool (AI|GetBlackboard (Variables|/Game/Blueprints/Characters/CowBP_Base.CowBP_Base_C|GetCowController _ascow_bp_base)) (Utilities|Name|MakeLiteralName "StandingOnTrigger") true))
  ;[1 1 1] Activation Effect
  (if (not (or (Variables|Default|GetbTriggerFinished) (Variables|Default|GetbDisabled)))
    (bind _returnvalue_2 (Effects|SpawnEmitteratLocation "/Game/ParticleSystems/FairyRingEffects/P_Magicalspores_Burst.P_Magicalspores_Burst" (Transformation|GetActorLocation)))
    (Effects|Components|ParticleSystem|SetColorParameter _returnvalue_2 "Color" (Variables|Default|GetRingColor))
    (Effects|Components|ParticleSystem|SetFloatParameter (Variables|Default|GetParticles) "Rate" 3e+01)
    (switch int (Variables|Default|GetNeighborTriggerCount)
      (:0
        (Class|FMODBlueprintStatics|PlayEventatLocation 0 _returnvalue))
      (:1
        (Class|FMODBlueprintStatics|PlayEventatLocation 0 _returnvalue)))
    (if (not (Variables|Default|GetbIsStandOnTrigger))
      (Variables|Default|SetbTriggerFinished false))))

(event Custom|Stop%20Triggering
  (bind _returnvalue (Transformation|GetActorTransform))
  ;[1 1 1] Count Touching Components
  (Variables|Default|SetTouchingComponents (- (Variables|Default|GetTouchingComponents) 1))
  ;[1 1 1] Set Cow Bool
  (if (and (== (Utilities|GetClass (stale OnComponentEndOverlap(TriggerBox) OtherActor)) "/Script/TAG.CowCharacter") (not (Variables|Default|GetbTriggerFinished)))
    (bind _ascow_bp_base (Utilities|Casting|CastToCowBP_Base (stale OnComponentEndOverlap(TriggerBox) OtherActor)))
    (AI|Components|Blackboard|SetValueasBool (AI|GetBlackboard (Variables|/Game/Blueprints/Characters/CowBP_Base.CowBP_Base_C|GetCowController _ascow_bp_base)) (Utilities|Name|MakeLiteralName "StandingOnTrigger") false))
  ;[1 1 1] Activation Effect
  (if (and (not (Variables|Default|GetActorEntered)) (not (Variables|Default|GetbTriggerFinished)))
    (Effects|Components|ParticleSystem|SetFloatParameter (Variables|Default|GetParticles) "Rate" 5.0)
    (if (not (or (Variables|Default|GetbTriggerFinished) (Variables|Default|GetbDisabled)))
      (bind _returnvalue_2 (Effects|SpawnEmitteratLocation "/Game/ParticleSystems/FairyRingEffects/P_Magicalspores_Burst.P_Magicalspores_Burst" (Transformation|GetActorLocation)))
      (Effects|Components|ParticleSystem|SetColorParameter _returnvalue_2 "Color" (Variables|Default|GetRingColor))
      (Effects|Components|ParticleSystem|SetFloatParameter (Variables|Default|GetParticles) "Rate" 3e+01)
      (switch int (Variables|Default|GetNeighborTriggerCount)
        (:0
          (Class|FMODBlueprintStatics|PlayEventatLocation 0 _returnvalue))
        (:1
          (Class|FMODBlueprintStatics|PlayEventatLocation 0 _returnvalue)))
      (if (not (Variables|Default|GetbIsStandOnTrigger))
        (Variables|Default|SetbTriggerFinished false)))))

(event EventBeginPlay
  (Components|Activation|Deactivate (Variables|Default|GetParticles))
  (if (Variables|Default|GetbDisabled)
    (Rendering|SetVisibility (Variables|Default|GetPointLight) false false)))

(event EventOnReceiveSignal
  (params (Signal :type Trigger%20Signal%20Structure))
  (bind _particles (Variables|Default|GetParticles))
  ;[1 1 1] Trigger Signal Handling
  (if (not (.bTriggerSequenceFinished (Utilities|Struct|BreakTriggerSignal Signal)))
    (if (< 0 (Variables|Default|GetNeighborTriggerCount))
      (Utilities|FlowControl|DoOnce false :!label _label
        (:Completed
          (Effects|Components|ParticleSystem|SetColorParameter _particles "Color" (Variables|Default|GetRingColor))
          (Components|Activation|Activate _particles false)
          (if (not (Variables|Default|GetActorEntered))
            (Effects|Components|ParticleSystem|SetFloatParameter (Variables|Default|GetParticles) "Rate" 5.0))
          (if (not (Variables|Default|GetbIsStandOnTrigger))
            (Variables|Default|SetbTriggerFinished false)
            (Components|Activation|Deactivate (Variables|Default|GetParticles)))))
      (else
        (Components|Activation|Deactivate (Variables|Default|GetParticles))
        (goto _label Reset)))))

(event EventTick
  (params (DeltaSeconds :type Float%20%28single-precision%29))
  ;[1 1 1] Call Open and Close
  (if (> (Variables|Default|GetTouchingComponents) 0)
    (if (not (Variables|Default|GetlastCommandOpen))
      (Variables|Default|SetlastCommandOpen true)
      (bind _outactors (Actor|GetAllActorswithTag (Utilities|Array|Get(acopy) (Variables|Default|GetTags))))
      (for _array_element _outactors
        (bind _asdoor_toggle_bp (Utilities|Casting|CastToDoorToggleBP _array_element))
        (Default|OnOpen _asdoor_toggle_bp)))
    (elif (Variables|Default|GetlastCommandOpen)
      (Variables|Default|SetlastCommandOpen false)
      (bind _outactors_2 (Actor|GetAllActorswithTag (Utilities|Array|Get(acopy) (Variables|Default|GetTags))))
      (for _array_element_2 _outactors_2
        (bind _asdoor_toggle_bp_2 (Utilities|Casting|CastToDoorToggleBP _array_element_2))
        (Default|OnClose _asdoor_toggle_bp_2)))))

(event EventOnTrigger)

(event EventOnLeave)

(fn ConstructionScript
  (Rendering|Components|Light|SetLightColor (Variables|Default|GetPointLight) (Variables|Default|GetRingColor) true)
  (Variables|Default|SetbTriggerFinished false))