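; End-level door that opens once, when enough cows are counted, its trigger actor fires, or it is told to open directly.
; Opening fires an optional Lookat, plays a sound, then after short delays runs a timeline moving the mesh from start to end.
; With ScaleObject enabled, the timeline also scales the mesh and sets an "End" parameter on audio started at BeginPlay.
; The construction script shows a green preview mesh at the end position.
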(event OnTrigger(TriggerActor)
  (bind _lookat (Variables|Default|GetLookat))
  (if (not (Variables|Default|GetIsFinished))
    (if (!= _lookat 0)
      (Default|Trigger _lookat))
    (Variables|Default|SetIsFinished true)
    (Utilities|FlowControl|Delay 0.1)
    (Class|FMODBlueprintStatics|PlayEventatLocation (Variables|Default|GetAudio%20Event) (Math|Conversions|ToTransform(Vector) (Transformation|GetActorLocation)))
    (Utilities|FlowControl|Delay 0.5)
    (bind _driver (Timeline|Door%20Timeline Play)
      (:Update
        (Transformation|SetRelativeLocation (Variables|Default|GetStaticMesh) (Math|Vector|Lerp(Vector) (Variables|Default|GetDoorStart) (Variables|Default|GetDoorEnd) _driver) false false)
        (if (Variables|Default|GetScaleObject)
          (Transformation|SetRelativeScale3D (Variables|Default|GetStaticMesh) (Math|Vector|Lerp(Vector) (Variables|Default|GetScaleStart) (Variables|Default|GetScaleEnd) _driver))
          (Class|FMODBlueprintStatics|EventInstanceSetParameter (stale EventBeginPlay _returnvalue) "End" 1.0))))))

(event Custom|OpenEndDoor
  (bind _lookat (Variables|Default|GetLookat))
  (if (not (Variables|Default|GetIsFinished))
    (if (!= _lookat 0)
      (Default|Trigger _lookat))
    (Variables|Default|SetIsFinished true)
    (Utilities|FlowControl|Delay 0.1)
    (Class|FMODBlueprintStatics|PlayEventatLocation (Variables|Default|GetAudio%20Event) (Math|Conversions|ToTransform(Vector) (Transformation|GetActorLocation)))
    (Utilities|FlowControl|Delay 0.5)
    (bind _driver (Timeline|Door%20Timeline Play)
      (:Update
        (Transformation|SetRelativeLocation (Variables|Default|GetStaticMesh) (Math|Vector|Lerp(Vector) (Variables|Default|GetDoorStart) (Variables|Default|GetDoorEnd) _driver) false false)
        (if (Variables|Default|GetScaleObject)
          (Transformation|SetRelativeScale3D (Variables|Default|GetStaticMesh) (Math|Vector|Lerp(Vector) (Variables|Default|GetScaleStart) (Variables|Default|GetScaleEnd) _driver))
          (Class|FMODBlueprintStatics|EventInstanceSetParameter (stale EventBeginPlay _returnvalue) "End" 1.0))))))

(event Custom|CheckOpenEndDoor
  (params (NumberOfCows :type Integer))
  (bind _lookat (Variables|Default|GetLookat))
  (if (>= NumberOfCows (Variables|Default|GetRequiredCows))
    (if (not (Variables|Default|GetIsFinished))
      (if (!= _lookat 0)
        (Default|Trigger _lookat))
      (Variables|Default|SetIsFinished true)
      (Utilities|FlowControl|Delay 0.1)
      (Class|FMODBlueprintStatics|PlayEventatLocation (Variables|Default|GetAudio%20Event) (Math|Conversions|ToTransform(Vector) (Transformation|GetActorLocation)))
      (Utilities|FlowControl|Delay 0.5)
      (bind _driver (Timeline|Door%20Timeline Play)
        (:Update
          (Transformation|SetRelativeLocation (Variables|Default|GetStaticMesh) (Math|Vector|Lerp(Vector) (Variables|Default|GetDoorStart) (Variables|Default|GetDoorEnd) _driver) false false)
          (if (Variables|Default|GetScaleObject)
            (Transformation|SetRelativeScale3D (Variables|Default|GetStaticMesh) (Math|Vector|Lerp(Vector) (Variables|Default|GetScaleStart) (Variables|Default|GetScaleEnd) _driver))
            (Class|FMODBlueprintStatics|EventInstanceSetParameter (stale EventBeginPlay _returnvalue) "End" 1.0)))))))

(event EventBeginPlay
  (Variables|Default|SetScaleStart (Variables|/Script/Engine.SceneComponent|GetRelativeScale3D (Variables|Default|GetStaticMesh)))
  (bind _returnvalue (Class|FMODBlueprintStatics|PlayEventatLocation 0 (Math|Conversions|ToTransform(Vector) (Transformation|GetActorLocation)))))

(fn ConstructionScript
  (Components|StaticMesh|SetStaticMesh (Variables|Default|GetPreviewMesh) (Variables|/Script/Engine.StaticMeshComponent|GetStaticMesh (Variables|Default|GetStaticMesh)))
  (for _index (range 0 (Rendering|Material|GetNumMaterials (Variables|Default|GetPreviewMesh)))
    (Rendering|Material|SetMaterial (Variables|Default|GetPreviewMesh) _index "/Game/OtherTextures/Materials/mat_debug_green.mat_debug_green"))
  (Transformation|SetRelativeLocation (Variables|Default|GetPreviewMesh) (+ (Variables|Default|GetDoorEnd) (Variables|/Script/Engine.SceneComponent|GetRelativeLocation (Variables|Default|GetStaticMesh))) false false))

(fn PreviewChange
  (Components|StaticMesh|SetStaticMesh (Variables|Default|GetPreviewMesh) (Variables|/Script/Engine.StaticMeshComponent|GetStaticMesh (Variables|Default|GetStaticMesh)))
  (for _index (range 0 (Rendering|Material|GetNumMaterials (Variables|Default|GetPreviewMesh)))
    (Rendering|Material|SetMaterial (Variables|Default|GetPreviewMesh) _index "/Game/OtherTextures/Materials/mat_debug_green.mat_debug_green"))
  (Transformation|SetRelativeLocation (Variables|Default|GetPreviewMesh) (+ (Variables|Default|GetDoorEnd) (Variables|/Script/Engine.SceneComponent|GetRelativeLocation (Variables|Default|GetStaticMesh))) false false))