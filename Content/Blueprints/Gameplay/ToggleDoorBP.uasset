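; Toggle door that alternates its mesh between start and end states whenever its linked TriggerActor fires.
; A Busy flag blocks retriggering while one of two timelines, chosen by IsFinished, lerps relative location, scale or both.
; Each toggle plays an audio event, and scale updates set an "End" parameter on the event instance created at BeginPlay.
; The construction script shows a green debug copy of the mesh offset by DoorEnd.
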(event OnTrigger(TriggerActor)
  (if (not (Variables|Default|GetBusy))
    (Variables|Default|SetBusy true)
    (Utilities|FlowControl|Delay 0.2)
    (Class|FMODBlueprintStatics|PlayEventatLocation (Variables|Default|GetAudio%20Event) (Math|Conversions|ToTransform(Vector) (Transformation|GetActorLocation)))
    (Utilities|FlowControl|Delay 0.2)
    (if (Variables|Default|GetIsFinished)
      (Variables|Default|SetIsFinished false)
      (bind _driver (Timeline|Timeline_0 PlayFromStart)
        (:Update
          (if (Variables|Default|GetMoveObject)
            (Transformation|SetRelativeLocation (Variables|Default|GetStaticMesh) (Math|Vector|Lerp(Vector) (Variables|Default|GetDoorEnd) (Variables|Default|GetDoorStart) _driver) false false))
          (if (Variables|Default|GetScaleObject)
            (Transformation|SetRelativeScale3D (Variables|Default|GetStaticMesh) (Math|Vector|Lerp(Vector) (Variables|Default|GetScaleEnd) (Variables|Default|GetScaleStart) _driver))
            (Class|FMODBlueprintStatics|EventInstanceSetParameter (stale EventBeginPlay _returnvalue) "End" 1.0 :!label _label)))
        (:Finished
          (Variables|Default|SetBusy false)))
      (else
        (Variables|Default|SetIsFinished true)
        (bind _driver_2 (Timeline|Door%20Timeline PlayFromStart)
          (:Update
            (if (Variables|Default|GetMoveObject)
              (Transformation|SetRelativeLocation (Variables|Default|GetStaticMesh) (Math|Vector|Lerp(Vector) (Variables|Default|GetDoorStart) (Variables|Default|GetDoorEnd) _driver_2) false false))
            (if (Variables|Default|GetScaleObject)
              (Transformation|SetRelativeScale3D (Variables|Default|GetStaticMesh) (Math|Vector|Lerp(Vector) (Variables|Default|GetScaleStart) (Variables|Default|GetScaleEnd) _driver_2))
              (goto _label)))
          (:Finished
            (Variables|Default|SetBusy false)))))))

(event EventBeginPlay
  (Variables|Default|SetScaleStart (Variables|/Script/Engine.SceneComponent|GetRelativeScale3D (Variables|Default|GetStaticMesh)))
  (bind _returnvalue (Class|FMODBlueprintStatics|PlayEventatLocation 0 (Math|Conversions|ToTransform(Vector) (Transformation|GetActorLocation)))))

(fn ConstructionScript
  (Components|StaticMesh|SetStaticMesh (Variables|Default|GetPreviewMesh) (Variables|/Script/Engine.StaticMeshComponent|GetStaticMesh (Variables|Default|GetStaticMesh)))
  (for _index (range 0 (Rendering|Material|GetNumMaterials (Variables|Default|GetPreviewMesh)))
    (Rendering|Material|SetMaterial (Variables|Default|GetPreviewMesh) _index "/Game/OtherTextures/Materials/mat_debug_green.mat_debug_green"))
  (Transformation|SetRelativeLocation (Variables|Default|GetPreviewMesh) (+ (Variables|Default|GetDoorEnd) (Variables|/Script/Engine.SceneComponent|GetRelativeLocation (Variables|Default|GetStaticMesh))) false false))

(fn PreviewChange
  (Components|StaticMesh|SetStaticMesh (Variables|Default|GetPreviewMesh) (Variables|/Script/Engine.StaticMeshComponent|GetStaticMesh (Variables|Default|GetStaticMesh)))
  (for _index (range 0 (Rendering|Material|GetNumMaterials (Variables|Default|GetPreviewMesh)))
    (Rendering|Material|SetMaterial (Variables|Default|GetPreviewMesh) _index "/Game/OtherTextures/Materials/mat_debug_green.mat_debug_green"))
  (Transformation|SetRelativeLocation (Variables|Default|GetPreviewMesh) (+ (Variables|Default|GetDoorEnd) (Variables|/Script/Engine.SceneComponent|GetRelativeLocation (Variables|Default|GetStaticMesh))) false false))