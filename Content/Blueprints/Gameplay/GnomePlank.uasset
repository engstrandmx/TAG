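; GnomePlank is a plank actor whose capsule collision is meant to differ between troll and gnome.
; Every Tick compares the display name of its troll character reference to a fixed string.
; A match calls WhenTroll, enabling query and physics collision; otherwise WhenGnome disables it.
; The cast that would supply the troll reference sits in unconnected nodes that never run.
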(event EventBeginPlay)

(event Collision|EventActorBeginOverlap
  (params (OtherActor :type Actor%20Object%20Reference)))

(event EventTick
  (params (DeltaSeconds :type Float%20%28single-precision%29))
  (if (Utilities|Enum|Equal(Enum) (Utilities|GetDisplayName (stale _astroll_character_instance)) "As Troll Character Instance")
    (CallFunction|WhenTroll)
    (else
      (CallFunction|WhenGnome))))

(fn ConstructionScript)

(fn WhenTroll
  (Collision|SetCollisionEnabled (Variables|Default|GetCapsule) "QueryAndPhysics"))

(fn WhenGnome
  (Collision|SetCollisionEnabled (Variables|Default|GetCapsule) "NoCollision"))