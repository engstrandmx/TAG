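; Pickupable item actor that plays feedback and removes itself from the world when picked up.
; OnPickup fires only once, guarded by a Triggered flag, spawning a particle burst at the mesh and playing a pickup audio event.
; A ScaleDown timeline then drives the actor's relative scale between zero and full size, destroying it when finished.
; The construction script tints the idle particle's color and edge color with IlluminateColor.
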(event EventBeginPlay)

(event Collision|EventActorBeginOverlap
  (params (OtherActor :type Actor%20Object%20Reference)))

(event EventTick
  (params (DeltaSeconds :type Float%20%28single-precision%29)))

(event EventOnPickup
  (if (not (Variables|Default|GetTriggered))
    (Variables|Default|SetTriggered true)
    (Effects|SpawnEmitteratLocation (Variables|Default|GetPickupParticles) (Transformation|GetWorldLocation (Variables|Default|GetStaticMeshComponent)))
    (Class|FMODBlueprintStatics|PlayEventatLocation "/Game/FMOD/Events/Sfx/Pickup/Pickup.Pickup" (Transformation|GetActorTransform))
    (bind _driver (Timeline|ScaleDown Play)
      (:Update
        (Transformation|SetActorRelativeScale3D (Math|Vector|Lerp(Vector) "0, 0, 0" "1.000000,1.000000,1.000000" _driver)))
      (:Finished
        (Actor|DestroyActor)))))

(fn ConstructionScript
  (bind _idleparticlecomponent (Variables|Default|GetIdleParticleComponent))
  (bind _illuminatecolor (Variables|Effects|GetIlluminateColor))
  (Effects|Components|ParticleSystem|SetColorParameter _idleparticlecomponent "Color" _illuminatecolor)
  (Effects|Components|ParticleSystem|SetColorParameter _idleparticlecomponent "EdgeColor" _illuminatecolor))