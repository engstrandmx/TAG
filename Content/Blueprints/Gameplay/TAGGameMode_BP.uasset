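; Game mode for a troll and gnome game, managing HUD widgets, pause menu, cow collectible count and level transitions.
; The count loads from HyssInstance; pickups update HUD and menu, then check end doors after a retriggerable delay.
; Level-sequence fades cover level loads and deaths, where death can reset the first cow, fairy rings, doors and destructibles.
; Tick detects character switches, playing a 2D sound event and notifying log actors.
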(event Custom|Load%20Level
  (params (LevelName :type Name))
  (bind _fadeinref (Variables|Default|GetFadeInRef))
  (Class|MovieSceneSequencePlayer|PlayReverse _fadeinref)
  (Utilities|FlowControl|Delay (- (Class|MovieSceneSequencePlayer|GetLength _fadeinref) 0.2))
  (Game|OpenLevel(byName) LevelName))

(event Custom|On%20Death%20Fade
  ;[1 1 1] Death Fade
  (Class|TAGGameMode|OnFadeOut)
  (Utilities|FlowControl|Delay 1.0)
  (bind _outactors (Actor|GetAllActorsOfClass "/Game/Blueprints/Characters/CowBP_Base.CowBP_Base_C"))
  (if (Variables|/Game/Blueprints/Characters/CowBP_Base.CowBP_Base_C|GetResetObjects (Utilities|Array|Get(acopy) _outactors))
    (bind _outactors_2 (Actor|GetAllActorsOfClass "/Game/Blueprints/Characters/CowBP_Base.CowBP_Base_C"))
    (Transformation|SetActorLocation (Utilities|Array|Get(acopy) _outactors_2) (Variables|/Game/Blueprints/Characters/CowBP_Base.CowBP_Base_C|GetStartingPosition (Utilities|Array|Get(acopy) _outactors_2)) false true)
    (bind _outactors_3 (Actor|GetAllActorsOfClass "/Game/Blueprints/Gameplay/Fairyring_BP.Fairyring_BP_C"))
    (Default|ResetRing _outactors_3)
    (bind _outactors_4 (Actor|GetAllActorsOfClass "/Game/Blueprints/Gameplay/SimpleDoorBP.SimpleDoorBP_C"))
    (Default|ResetDoor _outactors_4)
    (bind _outactors_5 (Actor|GetAllActorsOfClass "/Game/Blueprints/Gameplay/DoorToggleBP.DoorToggleBP_C"))
    (Default|ResetDoor _outactors_5)
    (bind _outactors_6 (Actor|GetAllActorsOfClass "/Game/Blueprints/Gameplay/NewDestructible_Plank.NewDestructible_Plank_C"))
    (for _array_element _outactors_6
      (Class|DestructibleComponent|SetDestructibleMesh (Variables|/Script/ApexDestruction.DestructibleActor|GetDestructibleComponent _array_element) "/Game/Geometry/WoodStructure/Barn/Models/mesh_barn_plank_01_DM.mesh_barn_plank_01_DM"))
    (bind _outactors_7 (Actor|GetAllActorsOfClass "/Game/Blueprints/Gameplay/NewDestructible_Barrel_BP.NewDestructible_Barrel_BP_C"))
    (for _array_element_2 _outactors_7
      (Class|DestructibleComponent|SetDestructibleMesh (Variables|/Script/ApexDestruction.DestructibleActor|GetDestructibleComponent _array_element_2) "/Game/Geometry/WoodStructure/Barn/Models/mesh_barn_barrel_03_DM.mesh_barn_barrel_03_DM")))
  (Utilities|FlowControl|Delay 0.3)
  (Class|TAGGameMode|OnFadein))

(event Custom|AddTooltip
  (params (Tooltip :type Tooltip%20Area%20BP%20Object%20Reference))
  (Default|TriggerTooltip Tooltip))

(event Custom|ShowActions
  (Development|PrintString "Hello")
  (Default|ShowAction (Variables|Default|GetGnomeActionUI)))

(event Custom|ToggleMenu
  (bind _ingamemenu (Variables|Default|GetIngameMenu))
  (Game|SetGamePaused (not (Variables|Default|GetMenuOpen)))
  (Default|OpenMenu (Variables|Default|GetIngameMenu))
  (bind _output_get (Variables|Default|SetMenuOpen (not (Variables|Default|GetMenuOpen))))
  (Variables|/Script/Engine.PlayerController|SetbShowMouseCursor (Game|GetPlayerController 0) _output_get)
  (if (not (Variables|Default|GetMenuOpen))
    (Class|WidgetBlueprintLibrary|SetFocustoGameViewport)
    (Default|CloseOptions _ingamemenu)
    (Default|CloseActualOptions _ingamemenu)))

(event Custom|DisplayNextTooltip
  ;[1 1 1] Disabled to avoid error
)

(event EventOnFadeOut
  (Class|MovieSceneSequencePlayer|PlayReverse (Variables|Default|GetFadeInRef)))

(event EventOnFadein
  (if (!= (Variables|Default|GetFadeInRef) 0)
    _
    (else
      (bind _returnvalue (Sequencer|Player|CreateLevelSequencePlayer "/Game/Cutscenes/Fade/FadeIn.FadeIn"))
      (Variables|Default|SetFadeInRef _returnvalue)))
  (Sequencer|Player|Play (Variables|Default|GetFadeInRef) :!class /Script/MovieScene.MovieSceneSequencePlayer))

(event EventOnCollectiblePickup
  (Default|SetCurrentCount (Variables|Default|GetCollectibleHUD) (Variables|Default|GetCollectibleCount))
  (Default|PlayPickupAnim (Variables|Default|GetCollectibleHUD))
  (Default|SetCurrentCollectibleCount (Variables|Default|GetIngameMenu) (Variables|Default|GetCollectibleCount) (Variables|Default|GetCollectiblesInLevel))
  (if (Variables|Default|GetCollectibleCountVisible)
    _
    (else
      (Variables|Default|SetCollectibleCountVisible true)
      (Default|PlayFadeAnimation (Variables|Default|GetCollectibleHUD) false)))
  (Utilities|FlowControl|RetriggerableDelay 1.5)
  (Default|PlayFadeAnimation (Variables|Default|GetCollectibleHUD) true)
  (Variables|Default|SetCollectibleCountVisible false)
  (bind _outactors (Actor|GetAllActorsOfClass "/Game/Blueprints/Gameplay/DoorEndBP.DoorEndBP_C"))
  (Default|CheckOpenEndDoor _outactors (Variables|Default|GetCollectibleCount)))

(event EventBeginPlay
  (bind _returnvalue (Game|GetPlayerController 0))
  (bind _ashyss_instance (Utilities|Casting|CastToHyssInstance (Game|GetGameInstance)))
  (Variables|Default|SetCollectibleCount (Variables|/Game/Blueprints/HyssInstance.HyssInstance_C|GetCurrentCows _ashyss_instance))
  (bind _returnvalue_2 (UserInterface|CreateWidget "/Game/Blueprints/UI/Tooltip_BP.Tooltip_BP_C" _returnvalue))
  (bind _output_get (Variables|Default|SetTooltipUBP _returnvalue_2))
  (UserInterface|Viewport|AddtoViewport _output_get 0)
  (bind _returnvalue_3 (UserInterface|CreateWidget "/Game/Blueprints/UI/Watermark_UBP.Watermark_UBP_C" _returnvalue))
  (UserInterface|Viewport|AddtoViewport _returnvalue_3 0)
  (bind _returnvalue_4 (UserInterface|CreateWidget "/Game/Blueprints/UI/CollectibleHUD_BP.CollectibleHUD_BP_C" _returnvalue))
  (bind _output_get_2 (Variables|Default|SetCollectibleHUD _returnvalue_4))
  (UserInterface|Viewport|AddtoViewport _output_get_2 0)
  (Default|SetMaxCount _returnvalue_4 (Class|KismetSystemLibrary|MakeLiteralInteger 50))
  (bind _returnvalue_5 (UserInterface|CreateWidget "/Game/Blueprints/UI/MainMenu/IngameMenuUBP.IngameMenuUBP_C" _returnvalue))
  (bind _output_get_3 (Variables|Default|SetIngameMenu _returnvalue_5))
  (UserInterface|Viewport|AddtoViewport _output_get_3 0)
  (Default|SetCurrentCollectibleCount (Variables|Default|GetIngameMenu) (Variables|Default|GetCollectibleCount) (Variables|Default|GetCollectiblesInLevel))
  (bind _returnvalue_6 (UserInterface|CreateWidget "/Game/Blueprints/UI/GnomeActionHUD_BP.GnomeActionHUD_BP_C" _returnvalue))
  (bind _output_get_4 (Variables|Default|SetGnomeActionUI _returnvalue_6))
  (UserInterface|Viewport|AddtoViewport _output_get_4 0))

(event EventTick
  (params (DeltaSeconds :type Float%20%28single-precision%29))
  ;[1 1 1] Call event on logs
  (bind _astaggame_mode_bp (Utilities|Casting|CastToTAGGameMode_BP (Game|GetGameMode)))
  (bind _returnvalue (Class|TAGGameMode|GetCurrentPlayerType _astaggame_mode_bp))
  (switch Utilities|FlowControl|Switch|SwitchonEPlayerType _returnvalue
    (:Troll
      (if (not (Variables|Default|GetCurrentTroll))
        (Variables|Default|SetCurrentTroll true)
        (Class|FMODBlueprintStatics|PlayEvent2D :!label _label)
        (bind _outactors (Actor|GetAllActorsOfClass "/Game/Blueprints/Gameplay/Log_blueprint.Log_blueprint_C"))
        (Default|SnapshotCharacterSwitch _outactors)))
    (:Gnome
      (if (Variables|Default|GetCurrentTroll)
        (Variables|Default|SetCurrentTroll false)
        (goto _label)))))

(fn ConstructionScript)