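; Stump actor that teleports the gnome character to a linked OtherStump.
; TeleportGnome plays a 2D audio event, waits briefly, then moves the first GnomeCharacter instance found.
; With Fall set, the gnome lands at a height offset lowered by the construction script.
; Otherwise it appears at a random horizontal offset around the destination plus HeightDifference and jumps.
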(event Custom|Teleport%20Gnome
  (bind _outactors (Actor|GetAllActorsOfClass "/Game/Blueprints/Characters/Instances/GnomeCharacter_Instance.GnomeCharacter_Instance_C"))
  (Class|FMODBlueprintStatics|PlayEvent2D)
  (Utilities|FlowControl|Delay 0.2)
  (if (Variables|Default|GetFall)
    (Transformation|SetActorLocation (Utilities|Array|Get(acopy) _outactors) (+ (Transformation|GetActorLocation (Variables|Default|GetOtherStump)) (Variables|Default|GetHeightDifference)) false true)
    (else
      (Transformation|SetActorLocation (Utilities|Array|Get(acopy) _outactors) (+ (Transformation|GetActorLocation (Variables|Default|GetOtherStump)) (+ (* (Math|Vector|Normalize (Math|Vector|MakeVector (Math|Random|RandomFloatinRange -1.0 1.0) (Math|Random|RandomFloatinRange -1.0 1.0) 0.0)) 40) (Variables|Default|GetHeightDifference))) false true)
      (Character|Jump (Utilities|Array|Get(acopy) _outactors)))))

(event EventBeginPlay)

(event Collision|EventActorBeginOverlap
  (params (OtherActor :type Actor%20Object%20Reference)))

(event EventTick
  (params (DeltaSeconds :type Float%20%28single-precision%29)))

(fn ConstructionScript
  (if (Variables|Default|GetFall)
    (Variables|Default|SetHeightDifference "0, 0,-90.000000")))