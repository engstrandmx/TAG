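; Toggleable door actor that slides and/or scales its static mesh between start and end values, with audio on opening and closing.
; OnOpen, guarded against repeats, plays a timeline that lerps the transform; OnClose reverses it.
; Each toggle multiplies the timeline's current play rate by SpeedMultiplier, so the change compounds.
; The construction script and a duplicate PreviewChange function show a green preview mesh at the end position.
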(event OnTrigger(TriggerActor))

(event Custom|On%20Open
  (bind _door_timeline (Variables|Default|GetDoor%20Timeline))
  (if (not (Variables|Default|GetStandingOn))
    (Variables|Default|SetStandingOn true)
    (Class|FMODBlueprintStatics|PlayEventatLocation (Variables|Default|GetAudio%20Event) (Math|Conversions|ToTransform(Vector) (Transformation|GetActorLocation)))
    (Components|Timeline|SetPlayRate _door_timeline (* (Components|Animation|GetPlayRate _door_timeline) (Variables|Default|GetSpeed%20Multiplier)))
    (bind _driver (Timeline|Door%20Timeline Play)
      (:Update
        (if (Variables|Default|GetMoveObject)
          (Transformation|SetRelativeLocation (Variables|Default|GetStaticMesh) (Math|Vector|Lerp(Vector) (Variables|Default|GetDoorStart) (Variables|Default|GetDoorEnd) _driver) false false))
        (if (Variables|Default|GetScaleObject)
          (Transformation|SetRelativeScale3D (Variables|Default|GetStaticMesh) (Math|Vector|Lerp(Vector) (Variables|Default|GetScaleStart) (Variables|Default|GetScaleEnd) _driver))
          (Class|FMODBlueprintStatics|EventInstanceSetParameter (stale EventBeginPlay _returnvalue) "End" 1.0))))))

(event Custom|On%20Close
  (bind _door_timeline (Variables|Default|GetDoor%20Timeline))
  (Variables|Default|SetStandingOn false)
  (Class|FMODBlueprintStatics|PlayEventatLocation (Variables|Default|GetAudio%20Event) (Math|Conversions|ToTransform(Vector) (Transformation|GetActorLocation)))
  (Components|Timeline|SetPlayRate _door_timeline (* (Components|Animation|GetPlayRate _door_timeline) (Variables|Default|GetSpeed%20Multiplier)))
  (bind _driver (Timeline|Door%20Timeline Reverse)
    (:Update
      (if (Variables|Default|GetMoveObject)
        (Transformation|SetRelativeLocation (Variables|Default|GetStaticMesh) (Math|Vector|Lerp(Vector) (Variables|Default|GetDoorStart) (Variables|Default|GetDoorEnd) _driver) false false))
      (if (Variables|Default|GetScaleObject)
        (Transformation|SetRelativeScale3D (Variables|Default|GetStaticMesh) (Math|Vector|Lerp(Vector) (Variables|Default|GetScaleStart) (Variables|Default|GetScaleEnd) _driver))
        (Class|FMODBlueprintStatics|EventInstanceSetParameter (stale EventBeginPlay _returnvalue) "End" 1.0)))))

(event EventBeginPlay
  (Variables|Default|SetScaleStart (Variables|/Script/Engine.SceneComponent|GetRelativeScale3D (Variables|Default|GetStaticMesh)))
  (bind _returnvalue (Class|FMODBlueprintStatics|PlayEventatLocation 0 (Math|Conversions|ToTransform(Vector) (Transformation|GetActorLocation)))))

(fn ConstructionScript
  (Components|StaticMesh|SetStaticMesh (Variables|Default|GetPreviewMesh) (Variables|/Script/Engine.StaticMeshComponent|GetStaticMesh (Variables|Default|GetStaticMesh)))
  (for _index (range 0 (Rendering|Material|GetNumMaterials (Variables|Default|GetPreviewMesh)))
    (Rendering|Material|SetMaterial (Variables|Default|GetPreviewMesh) _index "/Game/OtherTextures/Materials/mat_debug_green.mat_debug_green"))
  (Transformation|SetRelativeLocation (Variables|Default|GetPreviewMesh) (+ (Variables|Default|GetDoorEnd) (Variables|/Script/Engine.SceneComponent|GetRelativeLocation (Variables|Default|GetStaticMesh))) false false))

(fn PreviewChange
  (Components|StaticMesh|SetStaticMesh (Variables|Default|GetPreviewMesh) (Variables|/Script/Engine.StaticMeshComponent|GetStaticMesh (Variables|Default|GetStaticMesh)))
  (for _index (range 0 (Rendering|Material|GetNumMaterials (Variables|Default|GetPreviewMesh)))
    (Rendering|Material|SetMaterial (Variables|Default|GetPreviewMesh) _index "/Game/OtherTextures/Materials/mat_debug_green.mat_debug_green"))
  (Transformation|SetRelativeLocation (Variables|Default|GetPreviewMesh) (+ (Variables|Default|GetDoorEnd) (Variables|/Script/Engine.SceneComponent|GetRelativeLocation (Variables|Default|GetStaticMesh))) false false))