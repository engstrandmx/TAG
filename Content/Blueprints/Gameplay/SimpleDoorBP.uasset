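; One-shot door that, when its TriggerActor fires, moves and/or scales its static mesh toward configured end values.
; After short delays around an audio event, a timeline lerps relative location and scale according to MoveObject and ScaleObject.
; The scale branch also sets the "End" parameter on an audio instance created at BeginPlay.
; The construction script and PreviewChange show a green debug copy of the mesh offset by DoorEnd.
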(event OnTrigger(TriggerActor)
  (if (not (Variables|Default|GetIsFinished))
    (Variables|Default|SetIsFinished true)
    (Utilities|FlowControl|Delay 1.0)
    (Class|FMODBlueprintStatics|PlayEventatLocation (Variables|Default|GetAudio%20Event) (Math|Conversions|ToTransform(Vector) (Transformation|GetActorLocation)))
    (Utilities|FlowControl|Delay 0.5)
    (bind _driver (Timeline|Door%20Timeline Play)
      (:Update
        (if (Variables|Default|GetMoveObject)
          (Transformation|SetRelativeLocation (Variables|Default|GetStaticMesh) (Math|Vector|Lerp(Vector) (Variables|Default|GetDoorStart) (Variables|Default|GetDoorEnd) _driver) false false))
        (if (Variables|Default|GetScaleObject)
          (Transformation|SetRelativeScale3D (Variables|Default|GetStaticMesh) (Math|Vector|Lerp(Vector) (Variables|Default|GetScaleStart) (Variables|Default|GetScaleEnd) _driver))
          (Class|FMODBlueprintStatics|EventInstanceSetParameter (stale EventBeginPlay _returnvalue) "End" 1.0))))))

(event EventBeginPlay
  (Variables|Default|SetScaleStart (Variables|/Script/Engine.SceneComponent|GetRelativeScale3D (Variables|Default|GetStaticMesh)))
  (bind _returnvalue (Class|FMODBlueprintStatics|PlayEventatLocation 0 (Math|Conversions|ToTransform(Vector) (Transformation|GetActorLocation)))))

(fn ConstructionScript
  (Components|StaticMesh|SetStaticMesh (Variables|Default|GetPreviewMesh) (Variables|/Script/Engine.StaticMeshComponent|GetStaticMesh (Variables|Default|GetStaticMesh)))
  (for _index (range 0 (Rendering|Material|GetNumMaterials (Variables|Default|GetPreviewMesh)))
    (Rendering|Material|SetMaterial (Variables|Default|GetPreviewMesh) _index "/Game/OtherTextures/Materials/mat_debug_green.mat_debug_green"))
  (Transformation|SetRelativeLocation (Variables|Default|GetPreviewMesh) (+ (Variables|Default|GetDoorEnd) (Variables|/Script/Engine.SceneComponent|GetRelativeLocation (Variables|Default|GetStaticMesh))) false false))

(fn PreviewChange
  (Components|StaticMesh|SetStaticMesh (Variables|Default|GetPreviewMesh) (Variables|/Script/Engine.StaticMeshComponent|GetStaticMesh (Variables|Default|GetStaticMesh)))
  (for _index (range 0 (Rendering|Material|GetNumMaterials (Variables|Default|GetPreviewMesh)))
    (Rendering|Material|SetMaterial (Variables|Default|GetPreviewMesh) _index "/Game/OtherTextures/Materials/mat_debug_green.mat_debug_green"))
  (Transformation|SetRelativeLocation (Variables|Default|GetPreviewMesh) (+ (Variables|Default|GetDoorEnd) (Variables|/Script/Engine.SceneComponent|GetRelativeLocation (Variables|Default|GetStaticMesh))) false false))