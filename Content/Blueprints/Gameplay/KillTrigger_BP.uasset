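; Kill volume trigger that deals lethal damage to any Pawn that overlaps it.
; On overlap it applies a large fixed amount of generic damage with itself as the damage causer.
; When its water flag is set, it also spawns a splash particle just below the victim with slightly randomised scale, except for cow characters.
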(event EventBeginPlay)

(event Collision|EventActorBeginOverlap
  (params (OtherActor :type Actor%20Object%20Reference))
  (bind _aspawn (Utilities|Casting|CastToPawn OtherActor))
  (Game|Damage|ApplyDamage _aspawn 1e+03 0 self "/Script/Engine.DamageType")
  (if (and (not (Utilities|ClassIsChildOf (Utilities|GetClass OtherActor) "/Script/TAG.CowCharacter")) (Variables|Default|GetIsWater))
    (Effects|SpawnEmitteratLocation "/Game/ParticleSystems/P_Splash.P_Splash" (- (Transformation|GetActorLocation OtherActor) "0, 0,50.000000") "0, 0, 0" (+ "2.000000,2.000000,2.000000" (* (Math|Random|RandomUnitVector) 0.2)))))

(event EventTick
  (params (DeltaSeconds :type Float%20%28single-precision%29)))

(fn ConstructionScript)