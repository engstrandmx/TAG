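; Collectible secret pickup that spins in the world and removes itself on BeginPlay if its SecretID is already found in the "Secrets" save slot.
; BeginPlay creates that save if missing; OnPickup fires once, writing the found flag into an existing save.
; Pickup then spawns particles, plays an audio event and runs a ScaleDown timeline before destroying the actor.
; The construction script tints idle particles with IlluminateColor and hides StaticMeshComponent.
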(event EventBeginPlay
  (bind _returnvalue (SaveGame|DoesSaveGameExist "Secrets"))
  (if _returnvalue
    (bind _returnvalue_2 (SaveGame|LoadGamefromSlot "Secrets"))
    (bind _ashyss_save_game (Utilities|Casting|CastToHyssSaveGame _returnvalue_2))
    (if (Utilities|Array|Get(acopy) (Variables|/Game/Blueprints/HyssSaveGame.HyssSaveGame_C|GetSecretsFound _ashyss_save_game) (Variables|Default|GetSecretID))
      (Actor|DestroyActor))
    (else
      (bind _returnvalue_3 (SaveGame|CreateSaveGameObject "/Game/Blueprints/HyssSaveGame.HyssSaveGame_C"))
      (SaveGame|SaveGametoSlot _returnvalue_3 "Secrets"))))

(event Collision|EventActorBeginOverlap
  (params (OtherActor :type Actor%20Object%20Reference)))

(event EventTick
  (params (DeltaSeconds :type Float%20%28single-precision%29))
  (bind _staticmesh (Variables|Default|GetStaticMesh))
  (bind _returnvalue (Transformation|GetWorldRotation _staticmesh))
  (bind (_roll _pitch _yaw) (Math|Rotator|BreakRotator _returnvalue))
  (Transformation|SetWorldRotation (Variables|Default|GetStaticMesh) (Math|Rotator|MakeRotator _roll _pitch (+ (* DeltaSeconds 45.0) _yaw)) false false))

(event EventOnPickup
  (if (not (Variables|Default|GetTriggered))
    (Variables|Default|SetTriggered true)
    (bind _returnvalue (SaveGame|DoesSaveGameExist "Secrets"))
    (if _returnvalue
      (bind _returnvalue_2 (SaveGame|LoadGamefromSlot "Secrets"))
      (bind _ashyss_save_game (Utilities|Casting|CastToHyssSaveGame _returnvalue_2))
      (Utilities|Array|SetArrayElem (Variables|/Game/Blueprints/HyssSaveGame.HyssSaveGame_C|GetSecretsFound _ashyss_save_game) (Variables|Default|GetSecretID) true)
      (bind _returnvalue_3 (SaveGame|CreateSaveGameObject "/Game/Blueprints/HyssSaveGame.HyssSaveGame_C"))
      (Variables|/Game/Blueprints/HyssSaveGame.HyssSaveGame_C|SetSecretsFound _returnvalue_3 (Variables|/Game/Blueprints/HyssSaveGame.HyssSaveGame_C|GetSecretsFound _ashyss_save_game))
      (SaveGame|SaveGametoSlot _returnvalue_3 "Secrets"))
    (Effects|SpawnEmitteratLocation (Variables|Default|GetPickupParticles) (Transformation|GetWorldLocation (Variables|Default|GetStaticMeshComponent)))
    (Class|FMODBlueprintStatics|PlayEventatLocation 0 (Transformation|GetActorTransform))
    (bind _driver (Timeline|ScaleDown Play)
      (:Update
        (Transformation|SetActorRelativeScale3D (Math|Vector|Lerp(Vector) "0, 0, 0" "1.000000,1.000000,1.000000" _driver)))
      (:Finished
        (Actor|DestroyActor)))))

(fn ConstructionScript
  (bind _idleparticlecomponent (Variables|Default|GetIdleParticleComponent))
  (bind _illuminatecolor (Variables|Effects|GetIlluminateColor))
  (Effects|Components|ParticleSystem|SetColorParameter _idleparticlecomponent "Color" _illuminatecolor)
  (Effects|Components|ParticleSystem|SetColorParameter _idleparticlecomponent "EdgeColor" _illuminatecolor)
  (Rendering|SetVisibility (Variables|Default|GetStaticMeshComponent) false false))