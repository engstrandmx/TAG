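; CowCleanupBP is an overlap-triggered actor that recycles cows, pulling them out of a referenced water field and putting them back into play.
; When a CowBP_Base overlaps it, the cow is removed from the field's water actors and teleported to a random navigable point near the Spawn component.
; The cow is then set to Wandering, ordered toward the MoveLocation component and has its gravity scale restored.
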(event EventBeginPlay)

(event Collision|EventActorBeginOverlap
  (params (OtherActor :type Actor%20Object%20Reference))
  (bind _ascow_bp_base (Utilities|Casting|CastToCowBP_Base OtherActor))
  (Class|WaterField|RemovefromWaterActors (Variables|Default|GetWaterFieldReference) OtherActor)
  (Transformation|SetActorLocation OtherActor (.RandomLocation (Class|NavigationSystem|GetRandomPointinNavigableRadius (Transformation|GetWorldLocation (Variables|Default|GetSpawn)) 5e+01)) false false)
  (Default|ChangeState _ascow_bp_base "VE_Wandering")
  (Default|OrderMoveto _ascow_bp_base (Transformation|GetWorldLocation (Variables|Default|GetMoveLocation)))
  (Variables|/Game/Blueprints/Characters/CowBP_Base.CowBP_Base_C|SetGravity%20Scale _ascow_bp_base 1.0))

(event EventTick
  (params (DeltaSeconds :type Float%20%28single-precision%29)))

(fn ConstructionScript)