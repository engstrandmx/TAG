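; Trigger-volume actor that fires a look-at or sweep once a condition on the overlapping actor is met.
; On box overlap while inactive, it stores the actor, waits briefly, then, if the cow condition is enabled, checks that the actor's class is the cow Blueprint.
; A match sets Active to block later overlaps and triggers the Sweep reference if assigned, otherwise the Lookat reference.
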(event OnComponentBeginOverlap(TriggerBox)
  (params (OverlappedComponent :type Primitive%20Component%20Object%20Reference) (OtherActor :type Actor%20Object%20Reference) (OtherComp :type Primitive%20Component%20Object%20Reference) (OtherBodyIndex :type Integer) (bFromSweep :type Boolean) (SweepResult :type Hit%20Result%20Structure%20%28by%20ref%29))
  (if (not (Variables|Default|GetActive))
    (Variables|Default|SetCurrentOtherActor OtherActor)
    (Utilities|FlowControl|Delay 0.1)
    (if (Variables|Default|GetConditionCow)
      (if (== (Utilities|GetClass (Variables|Default|GetCurrentOtherActor)) "/Game/Blueprints/Characters/Instances/CowBP_Instance.CowBP_Instance_C")
        (CallFunction|Trigger)))))

(event EventBeginPlay)

(event Collision|EventActorBeginOverlap
  (params (OtherActor :type Actor%20Object%20Reference)))

(event EventTick
  (params (DeltaSeconds :type Float%20%28single-precision%29)))

(fn ConstructionScript)

(fn Trigger
  (Variables|Default|SetActive true)
  (if (!= (Variables|Default|GetSweep) 0)
    (Default|Trigger (Variables|Default|GetSweep))
    (else
      (Default|Trigger (Variables|Default|GetLookat)))))