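; Level exit trigger that ends the current level when a troll or gnome character overlaps it, disabling that character's input.
; After a delay it copies the collectible count to the game instance, then runs a sequence: optional delayed widget, progress save, music handler ending and delayed level load.
; The "Levels" save is written only if missing or behind.
; ToLvl selects the music handler, with zero also showing timed credits before loading.
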(event EventBeginPlay)

(event Collision|EventActorBeginOverlap
  (params (OtherActor :type Actor%20Object%20Reference))
  (bind _astroll_character_base (Utilities|Casting|CastToTrollCharacter_Base OtherActor)
    (:then
      (Input|DisableInput _astroll_character_base 0))
    (:CastFailed
      (bind _asgnome_character_base (Utilities|Casting|CastToGnomeCharacter_Base OtherActor))
      (Input|DisableInput _asgnome_character_base 0)))
  (Utilities|FlowControl|Delay (Variables|Default|GetDelay))
  (bind _astaggame_mode_bp (Utilities|Casting|CastToTAGGameMode_BP (Game|GetGameMode)))
  (bind _ashyss_instance (Utilities|Casting|CastToHyssInstance (Game|GetGameInstance)))
  (Variables|/Game/Blueprints/HyssInstance.HyssInstance_C|SetCurrentCows _ashyss_instance (Variables|/Script/TAG.TAGGameMode|GetCollectibleCount _astaggame_mode_bp))
  (Utilities|FlowControl|Sequence
    (:then_0
      (if (Variables|Default|GetShowWidget)
        (Utilities|FlowControl|Delay (Variables|Default|GetWidgetDelay))
        (bind _returnvalue (UserInterface|CreateWidget (Variables|Default|GetWidget) (Game|GetPlayerController 0)))
        (UserInterface|Viewport|AddtoViewport _returnvalue -10)))
    (:then_1
      (bind _returnvalue_2 (SaveGame|DoesSaveGameExist "Levels"))
      (if _returnvalue_2
        (bind _returnvalue_3 (SaveGame|LoadGamefromSlot "Levels"))
        (bind _ashyss_save_game (Utilities|Casting|CastToHyssSaveGame _returnvalue_3))
        (if (< (Variables|/Game/Blueprints/HyssSaveGame.HyssSaveGame_C|GetLevelsCompleted _ashyss_save_game) (- (Variables|Default|GetToLvl) 1))
          (bind _returnvalue_4 (SaveGame|CreateSaveGameObject "/Game/Blueprints/HyssSaveGame.HyssSaveGame_C" :!label _label))
          (Variables|/Game/Blueprints/HyssSaveGame.HyssSaveGame_C|SetLevelsCompleted _returnvalue_4 (- (Variables|Default|GetToLvl) 1))
          (SaveGame|SaveGametoSlot _returnvalue_4 "Levels"))
        (else
          (goto _label))))
    (:then_2
      (switch int (Variables|Default|GetToLvl)
        (:0
          (bind _outactors (Actor|GetAllActorsOfClass "/Game/Blueprints/Audio/Music_handlerlvl6.Music_handlerlvl6_C"))
          (Default|EndLvl6 _outactors))
        (:2
          (bind _outactors_2 (Actor|GetAllActorsOfClass "/Game/Blueprints/Audio/Music_handler.Music_handler_C"))
          (Default|Endlvl1 _outactors_2))
        (:3
          (bind _outactors_3 (Actor|GetAllActorsOfClass "/Game/Blueprints/Audio/Music_handlerlvl2.Music_handlerlvl2_C"))
          (Default|EndLvl2 _outactors_3))
        (:4
          (bind _outactors_4 (Actor|GetAllActorsOfClass "/Game/Blueprints/Audio/Music_handlerlvl3.Music_handlerlvl3_C"))
          (Default|EndLvl3 _outactors_4))
        (:5
          (bind _outactors_5 (Actor|GetAllActorsOfClass "/Game/Blueprints/Audio/Music_handlerlvl4.Music_handlerlvl4_C"))
          (Default|EndLvl4 _outactors_5))
        (:6
          (bind _outactors_6 (Actor|GetAllActorsOfClass "/Game/Blueprints/Audio/Music_handlerlvl5.Music_handlerlvl5_C"))
          (Default|EndLvl5 _outactors_6))))
    (:then_3
      (Utilities|FlowControl|Delay (Variables|Default|GetLoadDelay))
      (if (== (Variables|Default|GetToLvl) 0)
        (bind _returnvalue_5 (UserInterface|CreateWidget "/Game/Blueprints/UI/Menu/Credits.Credits_C" (Game|GetPlayerController 0)))
        (UserInterface|Viewport|AddtoViewport _returnvalue_5 0)
        (Utilities|FlowControl|Delay 63.0)
        (Class|VictoryBPFunctionLibrary|RemoveAllWidgetsOfClass "/Game/Blueprints/UI/Menu/Credits.Credits_C"))
      (Default|LoadLevel _astaggame_mode_bp (Variables|Default|GetLevelName)))))

(fn ConstructionScript)