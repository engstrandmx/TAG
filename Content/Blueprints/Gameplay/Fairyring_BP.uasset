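; Fairy ring of mushrooms that lights up while triggered and can be deactivated, optionally sending a particle trail to a door.
; StartTriggering and StopTriggering count touching components, driving a reversible godray and decal glow timeline plus stand-on sound.
; DeactivateRing bursts spores, scales the mushrooms by timeline and kills the glow; ResetRing restores them.
; Construction script creates color-tinted dynamic materials; older signal-trigger logic remains largely disconnected.
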(event OnTrigger(TriggerActor)
  ;[1 1 1] On Trigger
  (bind _output_get (Variables|Default|SetbDisabled (not (Variables|Default|GetbDisabled))))
  (if _output_get
    _))

(event Custom|Deactivate%20Ring
  (params (DoorLocation :type Vector))
  ;[1 1 1] Deactivate Ring
  (Variables|Default|SetDone true)
  (Utilities|FlowControl|Sequence
    (:then_0
      (bind _returnvalue (Effects|SpawnEmitteratLocation "/Game/ParticleSystems/FairyRingEffects/P_Magicalspores_Burst.P_Magicalspores_Burst" (Transformation|GetActorLocation) "0, 0, 0" "4.000000,4.000000,4.000000"))
      (Effects|Components|ParticleSystem|SetColorParameter _returnvalue "Color" (Variables|Default|GetRingColor))
      (Components|Activation|Deactivate (Variables|Default|GetParticles))
      (CallFunction|StopSoundStandon)
      (CallFunction|PlaySoundDeactivate)
      (Utilities|FlowControl|Delay 1.0)
      (bind _driver (Timeline|LightFadeTimeline PlayFromStart)
        (:Update
          (Transformation|SetWorldScale3D (Variables|Default|GetMushroomCollection) (Math|Conversions|ToVector(Float) _driver))
          (Rendering|Material|SetScalarParameterValueonMaterials (Variables|Default|GetGodray) "GlowStrength" 0.0)
          (Rendering|Material|SetScalarParameterValue (Variables|Default|GetDecalLight) "Brightness" 0.0 :!class /Script/Engine.MaterialInstanceDynamic))))
    (:then_1
      (if (Variables|Default|GetShowPath)
        (Components|Activation|Activate (Variables|Default|GetParticlePath) false)
        (bind _newtrack_0 (Timeline|Path%20Fly PlayFromStart)
          (:Update
            (Transformation|SetWorldLocation (Variables|Default|GetParticlePath) (Math|Vector|Lerp(Vector) (Transformation|GetActorLocation) DoorLocation _newtrack_0) false false))
          (:Finished
            (Components|Activation|Deactivate (Variables|Default|GetParticlePath))))))))

(event Custom|ResetRing
  ;[1 1 1] Deactivate Ring
  ;;[1 1 1] Reset Ring
  (Variables|Default|SetActive false)
  (Variables|Default|SetDone false)
  (Utilities|FlowControl|Sequence
    (:then_0
      (bind _driver (Timeline|LightFadeTimeline Stop)
        (:Update
          (Transformation|SetWorldScale3D (Variables|Default|GetMushroomCollection) (Math|Conversions|ToVector(Float) _driver))
          (Rendering|Material|SetScalarParameterValueonMaterials (Variables|Default|GetGodray) "GlowStrength" 0.0)
          (Rendering|Material|SetScalarParameterValue (Variables|Default|GetDecalLight) "Brightness" 0.0 :!class /Script/Engine.MaterialInstanceDynamic))))
    (:then_1
      (Transformation|SetWorldScale3D (Variables|Default|GetMushroomCollection) "1.000000,1.000000,1.000000")
      (Rendering|Material|SetScalarParameterValueonMaterials (Variables|Default|GetGodray) "GlowStrength" (Variables|Default|GetGodrayOffLight))
      (Rendering|Material|SetScalarParameterValue (Variables|Default|GetDecalLight) "Brightness" (Variables|Default|GetDecalOffLight) :!class /Script/Engine.MaterialInstanceDynamic)
      (Components|Activation|Activate (Variables|Default|GetParticles) false))))

(event Custom|Start%20Triggering
  ;[1 1 1] Count Triggers
  (if (not (Variables|Default|GetDone))
    (Variables|Default|SetTouchingComponents (+ (Variables|Default|GetTouchingComponents) 1))
    (CallFunction|CheckActive)
    (CallFunction|OnEffect)))

(event Custom|On%20Effect
  (bind _returnvalue (Transformation|GetActorTransform))
  ;[1 1 1] On Trigger
  (bind _returnvalue_2 (Effects|SpawnEmitteratLocation "/Game/ParticleSystems/FairyRingEffects/P_Magicalspores_Burst.P_Magicalspores_Burst" (Transformation|GetActorLocation) "0, 0, 0" "0.000000,0.000000,0.000000"))
  (Effects|Components|ParticleSystem|SetColorParameter _returnvalue_2 "Color" (Variables|Default|GetRingColor))
  (Effects|Components|ParticleSystem|SetFloatParameter (Variables|Default|GetParticles) "Rate" 3e+01)
  (switch int (Variables|Default|GetNeighborTriggerCount)
    (:0
      (Class|FMODBlueprintStatics|PlayEventatLocation 0 _returnvalue))
    (:1
      (Class|FMODBlueprintStatics|PlayEventatLocation 0 _returnvalue)))
  (if (Variables|Default|GetbIsStandOnTrigger)
    _))

(event Custom|Check%20Active
  ;[1 1 1] Check Active
  (if (> (Variables|Default|GetTouchingComponents) 0)
    (if (not (Variables|Default|GetActive))
      ;[1 1 1] Set Active
      (CallFunction|PlaySoundStandon)
      (Variables|Default|SetActive true)
      (bind _newtrack_0 (Timeline|GodrayFade Play)
        (:Update
          (Rendering|Material|SetScalarParameterValueonMaterials (Variables|Default|GetGodray) "GlowStrength" (Math|Float|Lerp (Variables|Default|GetGodrayOffLight) (Variables|Default|GetGodrayOnLight) _newtrack_0))
          (Rendering|Material|SetScalarParameterValue (Variables|Default|GetDecalLight) "Brightness" (Math|Float|Lerp (Variables|Default|GetDecalOffLight) (Variables|Default|GetDecalOnLight) _newtrack_0) :!class /Script/Engine.MaterialInstanceDynamic))))
    (elif (Variables|Default|GetActive)
      (CallFunction|StopSoundStandon)
      (Variables|Default|SetActive false)
      (Timeline|GodrayFade Reverse))))

(event Custom|Stop%20Triggering
  ;[1 1 1] Count Triggers
  (if (not (Variables|Default|GetDone))
    (Variables|Default|SetTouchingComponents (- (Variables|Default|GetTouchingComponents) 1))
    (CallFunction|CheckActive)))

(event Custom|PlaySoundStandOn
  ;[1 1 1] Sound Events
  (bind _returnvalue (Class|FMODBlueprintStatics|PlayEventatLocation "/Game/FMOD/Events/Sfx/Alvring/Alvring_01.Alvring_01" (Math|Conversions|ToTransform(Vector) (Transformation|GetActorLocation)))))

(event Custom|StopSoundStandOn
  ;[1 1 1] Sound Events
  (Class|FMODBlueprintStatics|EventInstanceSetParameter (stale Custom|PlaySoundStandOn _returnvalue) "Stop" 1.0))

(event Custom|PlaySoundDeactivate
  ;[1 1 1] Sound Events
  (Class|FMODBlueprintStatics|PlayEventatLocation "/Game/FMOD/Events/Sfx/Alvring/Alvring_03.Alvring_03" (Transformation|GetActorTransform)))

(event EventBeginPlay
  ;[1 1 1] Begin Play
  (Components|Activation|Deactivate (Variables|Default|GetParticles))
  (Components|Activation|Deactivate (Variables|Default|GetParticlePath)))

(event EventOnReceiveSignal
  (params (Signal :type Trigger%20Signal%20Structure)))

(event EventOnTrigger
  ;[1 1 1] On Trigger
)

(event EventOnLeave)

(fn ConstructionScript
  (bind _decal (Variables|Default|GetDecal))
  (bind _path_fly (Variables|Default|GetPath%20Fly))
  ;[1 1 1] Set Mushroom Array
  (Variables|Default|SetMushroomCollection (Utilities|Array|MakeArray (Variables|Default|GetStaticMesh4) (Variables|Default|Getmodel_fairy_mushroom2) (Variables|Default|Getmodel_fairy_mushroom4) (Variables|Default|Getmodel_fairy_mushroom5) (Variables|Default|Getmodel_fairy_mushroom0) (Variables|Default|GetStaticMesh7) (Variables|Default|GetStaticMesh) (Variables|Default|GetStaticMesh1) (Variables|Default|GetStaticMesh2) (Variables|Default|Getmodel_fairy_mushroom1) (Variables|Default|GetStaticMesh5) (Variables|Default|GetStaticMesh6) (Variables|Default|GetStaticMesh14) (Variables|Default|GetStaticMesh8) (Variables|Default|GetStaticMesh9) (Variables|Default|GetStaticMesh10) (Variables|Default|GetStaticMesh3) (Variables|Default|GetStaticMesh12) (Variables|Default|GetStaticMesh13)))
  ;[1 1 1] Set Path Particle Speed
  (Components|Timeline|SetPlayRate _path_fly (* (Components|Animation|GetPlayRate _path_fly) (Variables|Default|GetPathParticlesSpeed)))
  ;[1 1 1] Check Big Trigger
  (if (Variables|Default|GetBigTrigger)
    (Components|Sphere|SetSphereRadius (Variables|Default|GetSphere) 1.1e+02 true))
  ;[1 1 1] init Godray
  (Rendering|Material|CreateDynamicMaterialInstance (Variables|Default|GetGodray) 0 "/Game/Environment/Decals/mat_godray_Inst.mat_godray_Inst" :!class /Script/Engine.PrimitiveComponent)
  (Rendering|Material|SetVectorParameterValueonMaterials (Variables|Default|GetGodray) "GlowColor" (Math|Conversions|ToVector(LinearColor) (Variables|Default|GetRingColor)))
  (Rendering|Material|SetScalarParameterValueonMaterials (Variables|Default|GetGodray) "GlowStrength" (Variables|Default|GetGodrayOffLight))
  ;[1 1 1] init Decal
  (Rendering|Components|Decal|SetDecalMaterial _decal (Variables|/Script/Engine.DecalComponent|GetDecalMaterial _decal))
  (bind _returnvalue (Rendering|Material|CreateDynamicMaterialInstance _decal :!class /Script/Engine.DecalComponent))
  (Rendering|Material|SetVectorParameterValue _returnvalue "Color" (Variables|Default|GetRingColor) :!class /Script/Engine.MaterialInstanceDynamic)
  (Rendering|Material|SetScalarParameterValue _returnvalue "Brightness" (Variables|Default|GetDecalOffLight) :!class /Script/Engine.MaterialInstanceDynamic)
  (Variables|Default|SetDecalLight _returnvalue)
  ;[1 1 1] ?
  (Variables|Default|SetbTriggerFinished false))