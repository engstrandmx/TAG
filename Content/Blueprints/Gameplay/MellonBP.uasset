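; MellonBP is a melon actor that attaches itself to a gnome character on overlap.
; On overlap it disables the sphere's collision and physics, snaps to the gnome's neck socket after a short delay, raises itself and plays the Gnom_mellon event.
; When the gnome reaches its jump apex, it detaches and applies a forward impulse to the sphere, without re-enabling collision or physics.
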(event OnReachedJumpApex(Gnome)
  (Transformation|DetachFromActor "KeepRelative" "KeepRelative" "KeepRelative")
  (Physics|AddImpulse (Variables|Default|GetSphere) (* (Transformation|GetActorForwardVector (Variables|Default|GetGnome)) 1.5e+02) "None" false))

(event EventBeginPlay)

(event Collision|EventActorBeginOverlap
  (params (OtherActor :type Actor%20Object%20Reference))
  (bind _asgnome_character (Utilities|Casting|CastToGnomeCharacter OtherActor))
  (Variables|Default|SetGnome _asgnome_character)
  (Collision|SetCollisionEnabled (Variables|Default|GetSphere) "NoCollision")
  (Physics|SetSimulatePhysics (Variables|Default|GetSphere) false)
  (Utilities|FlowControl|Delay 0.2)
  (Transformation|AttachActorToActor _asgnome_character "neck_socket" "SnapToTarget" "KeepRelative" "KeepRelative" true)
  (Transformation|SetActorRelativeLocation "0, 0,50.000000")
  (Class|FMODBlueprintStatics|PlayEventatLocation "/Game/FMOD/Events/Gnom/Gnom_mellon.Gnom_mellon" (Transformation|GetActorTransform)))

(event EventTick
  (params (DeltaSeconds :type Float%20%28single-precision%29)))

(fn ConstructionScript)