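; Door Blueprint that moves its mesh when a linked TriggerActor fires OnTrigger, playing DoorTimeline.
; Each timeline update adds the DoorStart-to-DoorEnd interpolation as a local offset, so movement accumulates rather than setting an absolute position.
; The construction script shows the end position with a preview mesh that copies the door's mesh, uses the Donut material and sits at DoorEnd.
; PreviewChange is an empty stub.
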(event OnTrigger(TriggerActor)
  (bind _driver (Timeline|Door%20Timeline Play)
    (:Update
      (Transformation|AddLocalOffset (Variables|Default|GetStaticMesh) (Math|Vector|Lerp(Vector) (Variables|Default|GetDoorStart) (Variables|Default|GetDoorEnd) _driver) false false))))

(fn ConstructionScript
  (Components|StaticMesh|SetStaticMesh (Variables|Default|GetPreviewMesh) (Variables|/Script/Engine.StaticMeshComponent|GetStaticMesh (Variables|Default|GetStaticMesh)))
  (for _index (range 0 (Rendering|Material|GetNumMaterials (Variables|Default|GetPreviewMesh)))
    (Rendering|Material|SetMaterial (Variables|Default|GetPreviewMesh) _index "/Game/Graphics/CuteFood/Donut.Donut"))
  (Transformation|SetRelativeLocation (Variables|Default|GetPreviewMesh) (Variables|Default|GetDoorEnd) false false))

(fn PreviewChange)