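; CowKnight spawner that respawns the cow by teleporting the first existing CowBP_Base to its SpawnPoint, rather than creating a new actor.
; PressSpawn calls SpawnCowKnight, which always succeeds, then removes the cow from WaterField actors, stops its movement and following, and sets it to Wandering.
; A timeline then scales the cow up from tiny to full size.
; Trigger-box overlap counting and spawn-occupancy checks are disconnected and never run.
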(event OnComponentEndOverlap(Triggerbox)
  (params (OverlappedComponent :type Primitive%20Component%20Object%20Reference) (OtherActor :type Actor%20Object%20Reference) (OtherComp :type Primitive%20Component%20Object%20Reference) (OtherBodyIndex :type Integer)))

(event OnComponentBeginOverlap(Triggerbox)
  (params (OverlappedComponent :type Primitive%20Component%20Object%20Reference) (OtherActor :type Actor%20Object%20Reference) (OtherComp :type Primitive%20Component%20Object%20Reference) (OtherBodyIndex :type Integer) (bFromSweep :type Boolean) (SweepResult :type Hit%20Result%20Structure%20%28by%20ref%29)))

(event Custom|Press%20Spawn
  (bind _success (CallFunction|SpawnCowKnight))
  (if _success
    (bind _outactors (Actor|GetAllActorsOfClass "/Game/Blueprints/Characters/CowBP_Base.CowBP_Base_C"))
    (bind _outactors_2 (Actor|GetAllActorsOfClass "/Script/TAG.WaterField"))
    (Class|WaterField|RemovefromWaterActors _outactors_2 (Utilities|Array|Get(acopy) _outactors))
    (Default|ChangeState (Utilities|Array|Get(acopy) _outactors) "VE_Wandering")
    (Components|Movement|StopMovementImmediately (Variables|/Script/Engine.Character|GetCharacterMovement (Utilities|Array|Get(acopy) _outactors)))
    (Default|StopFollowing (Utilities|Array|Get(acopy) _outactors))
    (bind _newtrack_0 (Timeline|ScaleTimeline PlayFromStart)
      (:Update
        (Transformation|SetActorRelativeScale3D (Utilities|Array|Get(acopy) _outactors) (Math|Vector|Lerp(Vector) "0.100000,0.100000,0.100000" "1.000000,1.000000,1.000000" _newtrack_0))))))

(event Collision|EventActorBeginOverlap
  (params (OtherActor :type Actor%20Object%20Reference)))

(event EventTick
  (params (DeltaSeconds :type Float%20%28single-precision%29)))

(fn ConstructionScript)

(fn SpawnCowKnight
  (bind _outactors (Actor|GetAllActorsOfClass "/Game/Blueprints/Characters/CowBP_Base.CowBP_Base_C"))
  (Transformation|SetActorLocation (Utilities|Array|Get(acopy) _outactors) (Transformation|GetWorldLocation (Variables|Default|GetSpawnPoint)) false false)
  (return true))