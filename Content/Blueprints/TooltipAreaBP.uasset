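; Trigger area that shows timed tutorial-style tooltips when a TAGCharacter enters, optionally only once.
; Overlap registers it with TAGGameMode_BP's tooltip queue; TriggerTooltip then steps through the text levels, each with its own delay, showing UI text and playing a sound.
; Tooltips hide after ShowTime or stay until the end area.
; The end area or TriggerActor's OnTrigger cancels the sequence, and finishing asks the game mode for the next tooltip.
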(event OnComponentBeginOverlap(TriggerArea)
  (params (OverlappedComponent :type Primitive%20Component%20Object%20Reference) (OtherActor :type Actor%20Object%20Reference) (OtherComp :type Primitive%20Component%20Object%20Reference) (OtherBodyIndex :type Integer) (bFromSweep :type Boolean) (SweepResult :type Hit%20Result%20Structure%20%28by%20ref%29))
  (if (not (Variables|Default|GetActive))
    (Variables|Default|SetActive true)
    (Utilities|Casting|CastToTAGCharacter OtherActor)
    (Math|Integer|IncrementInt (Variables|Default|GetActorsInArea)
      (:%20%20
        (Default|AddTooltip (Variables|Default|GetGameMode) self)))))

(event OnComponentEndOverlap(TriggerArea)
  (params (OverlappedComponent :type Primitive%20Component%20Object%20Reference) (OtherActor :type Actor%20Object%20Reference) (OtherComp :type Primitive%20Component%20Object%20Reference) (OtherBodyIndex :type Integer))
  (Utilities|Casting|CastToTAGCharacter OtherActor)
  (Math|Integer|DecrementInt (Variables|Default|GetActorsInArea)))

(event OnComponentBeginOverlap(TriggerEndArea)
  (params (OverlappedComponent :type Primitive%20Component%20Object%20Reference) (OtherActor :type Actor%20Object%20Reference) (OtherComp :type Primitive%20Component%20Object%20Reference) (OtherBodyIndex :type Integer) (bFromSweep :type Boolean) (SweepResult :type Hit%20Result%20Structure%20%28by%20ref%29))
  (if (not (or (Variables|Default|GetCancelShowTooltip) (Variables|Default|GetFinished)))
    (Utilities|Casting|CastToTAGCharacter OtherActor)
    (Variables|Default|SetCancelShowTooltip true)
    (Utilities|FlowControl|Delay (Variables|Default|GetDissapearDelay))
    (Default|HideTooltip (Variables|Default|GetTooltip%20UI))
    (if (Variables|Default|GetTriggerOnce)
      _
      (else
        (Variables|Default|SetActive false)))
    (Utilities|FlowControl|Delay 1.0)
    (CallFunction|FinishTooltip)))

(event OnTrigger(TriggerActor)
  (Variables|Default|SetCancelShowTooltip true)
  (Default|HideTooltip (Variables|Default|GetTooltip%20UI))
  (Utilities|FlowControl|Delay 1.0)
  (CallFunction|FinishTooltip))

(event Custom|Trigger%20Tooltip
  (bind _tooltiplevel (Variables|Default|GetTooltipLevel))
  (Utilities|FlowControl|Delay (Utilities|Array|Get(acopy) (Variables|Default|GetTriggerDelay) (Variables|Default|GetTooltipLevel)) :!label _label)
  (if (Variables|Default|GetCancelShowTooltip)
    (CallFunction|FinishTooltip)
    (else
      (Variables|Default|SetTooltip%20UI (Variables|/Game/Blueprints/Gameplay/TAGGameMode_BP.TAGGameMode_BP_C|GetTooltipUBP (Variables|Default|GetGameMode)))
      (Default|ShowTooltip (Variables|Default|GetTooltip%20UI) (Utilities|Array|Get(acopy) (Variables|Default|GetTooltip%20Text) (Variables|Default|GetTooltipLevel)))
      (bind _returnvalue (Class|FMODBlueprintStatics|PlayEvent2D 0 false))
      (Class|FMODBlueprintStatics|EventInstanceSetVolume _returnvalue 0.75)
      (Class|FMODBlueprintStatics|EventInstancePlay _returnvalue)
      (if (not (Variables|Default|GetStayUntilEndArea))
        (Utilities|FlowControl|Delay (Variables|Default|GetShowTime))
        (if (not (Variables|Default|GetCancelShowTooltip))
          (Default|HideTooltip (Variables|Default|GetTooltip%20UI))
          (Utilities|FlowControl|Delay 1.0)
          (Math|Integer|IncrementInt _tooltiplevel
            (:%20%20
              (if (== _tooltiplevel (Utilities|Array|Length (Variables|Default|GetTooltip%20Text)))
                (CallFunction|FinishTooltip)
                (Variables|Default|SetFinished true)
                (if (not (Variables|Default|GetTriggerOnce))
                  (Variables|Default|SetActive false))
                (else
                  (goto _label))))))))))

(event EventBeginPlay
  (bind _astaggame_mode_bp (Utilities|Casting|CastToTAGGameMode_BP (Game|GetGameMode)))
  (Variables|Default|SetGameMode _astaggame_mode_bp))

(fn ConstructionScript
  (Utilities|Array|Resize (Variables|Default|GetTriggerDelay) (Utilities|Array|Length (Variables|Default|GetTooltip%20Text))))

(fn FinishTooltip
  (Default|DisplayNextTooltip (Variables|Default|GetGameMode)))