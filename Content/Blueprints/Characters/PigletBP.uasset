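; Piglet character, driven by an AI controller, that bounces off other characters it bumps into.
; On BeginPlay it caches its PigletAIControllerBP and writes its CircleSpline to the blackboard's Spline key, presumably as a path for its AI.
; Capsule hits with any Character launch both apart and upward, scaled by BounceForce, rotating the vector half a turn for the piglet.
; Leftover Boar origin and game mode setup is unconnected.
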(event OnComponentHit(CapsuleComponent)
  (params (HitComponent :type Primitive%20Component%20Object%20Reference) (OtherActor :type Actor%20Object%20Reference) (OtherComp :type Primitive%20Component%20Object%20Reference) (NormalImpulse :type Vector :default "0, 0, 0") (Hit :type Hit%20Result%20Structure%20%28by%20ref%29))
  (if (Utilities|ClassIsChildOf (Utilities|GetClass OtherActor) "/Script/Engine.Character")
    (bind _ascharacter (Utilities|Casting|CastToCharacter OtherActor))
    (Character|LaunchCharacter _ascharacter (* (+ (Math|Vector|Normalize (- (Transformation|GetActorLocation _ascharacter) (Transformation|GetActorLocation))) "0, 0,1.000000") (Variables|Default|GetBounceForce)) false false)
    (Character|LaunchCharacter (Math|Vector|RotateVectorAroundAxis (* (+ (Math|Vector|Normalize (- (Transformation|GetActorLocation _ascharacter) (Transformation|GetActorLocation))) "0, 0,1.000000") (Variables|Default|GetBounceForce)) 1.8e+02 "0, 0,1.000000") false false)))

(event EventBeginPlay
  (bind _returnvalue (Pawn|GetController))
  ;[1 1 1] Init BB and vars
  (bind _aspiglet_aicontroller_bp (Utilities|Casting|CastToPigletAIControllerBP _returnvalue))
  (Variables|Default|SetPigletController _aspiglet_aicontroller_bp)
  (AI|Components|Blackboard|SetValueasObject (AI|GetBlackboard _returnvalue) (Utilities|Name|MakeLiteralName "Spline") (Variables|Default|GetCircleSpline)))

(event Collision|EventActorBeginOverlap
  (params (OtherActor :type Actor%20Object%20Reference)))

(event EventTick
  (params (DeltaSeconds :type Float%20%28single-precision%29)))

(fn ConstructionScript)