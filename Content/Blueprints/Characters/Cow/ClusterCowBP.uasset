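; ClusterCowBP is a cow character that works like a cluster bomb, bursting into mini cows after being hit hard enough.
; A sufficiently powerful hit on its HittableSceneComponent arms it, and the next landing or capsule hit detonates it with sound and smoke.
; Detonation spawns AI MiniCowBP pawns in a jittered ring, launches them outward and upward, then destroys the cow.
; The explosion-radius overlap query has an empty loop, affecting nothing.
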(event OnComponentHit(HittableSceneComponent)
  (params (HittingActor :type Actor%20Object%20Reference) (PowerMultiplier :type Float%20%28single-precision%29) (ForwardVector :type Vector :default "0, 0, 0"))
  (if (< 0.5 PowerMultiplier)
    (Variables|Default|SetArmed true)))

(event OnComponentHit(CapsuleComponent)
  (params (HitComponent :type Primitive%20Component%20Object%20Reference) (OtherActor :type Actor%20Object%20Reference) (OtherComp :type Primitive%20Component%20Object%20Reference) (NormalImpulse :type Vector :default "0, 0, 0") (Hit :type Hit%20Result%20Structure%20%28by%20ref%29))
  (bind _returnvalue (Transformation|GetActorLocation))
  (if (Variables|Default|GetArmed)
    (Variables|Default|SetArmed false)
    (Audio|PlaySoundatLocation "/Game/Engine/StarterContent/Audio/Explosion01.Explosion01" _returnvalue)
    (Effects|SpawnEmitteratLocation "/Game/ParticleSystems/P_SmokeSprayCircluar.P_SmokeSprayCircluar" _returnvalue "0, 0, 0" "5.000000,5.000000,5.000000")
    (Effects|SpawnEmitteratLocation "/Game/ParticleSystems/P_SmokeSpray.P_SmokeSpray" _returnvalue "0, 0, 0" "5.000000,5.000000,5.000000")
    (for _index (range 0 (Variables|Default|GetCowCount))
      (bind _returnvalue_2 (AI|SpawnAIFromClass "/Game/Blueprints/Characters/Cow/MiniCowBP.MiniCowBP_C" "/Game/Blueprints/Characters/Cow/Cow_BT.Cow_BT" (+ (Transformation|GetActorLocation) (Math|Vector|RotateVectorAroundAxis (* "1.000000, 0,0.000000" (Variables|Default|GetSpawnRadius)) (+ (* _index (/ 3.6e+02 (Math|Conversions|ToFloat(Integer) (Variables|Default|GetCowCount)))) (Math|Random|RandomFloatinRange -1e+01 1e+01)) "0, 0,1.000000")) (Math|Random|RandomRotator false) true))
      (bind _ascharacter (Utilities|Casting|CastToCharacter _returnvalue_2))
      (Character|LaunchCharacter _ascharacter (* (Math|Vector|Normalize (- (+ (Transformation|GetActorLocation _ascharacter) "0, 0,300.000000") (Transformation|GetActorLocation))) (Math|Random|RandomFloatinRange 5e+02 7.5e+02)) false false))
    (bind _outactors (Collision|SphereOverlapActors (Transformation|GetActorLocation) (Variables|Default|GetExplosionRadius) (Utilities|Array|MakeArray "ObjectTypeQuery2") 0))
    (for _array_element _outactors
      _)
    (Utilities|FlowControl|Delay 0.05)
    (Actor|DestroyActor)))

(event EventBeginPlay
  (|CallParentFunction) ; This node is disabled and will not be called.\nDrag off pins to build functionality.
)

(event Collision|EventActorBeginOverlap
  (params (OtherActor :type Actor%20Object%20Reference)))

(event EventOnLanded
  (params (Hit :type Hit%20Result%20Structure%20%28by%20ref%29))
  (bind _returnvalue (Transformation|GetActorLocation))
  (|CallParentFunction Hit)
  (if (Variables|Default|GetArmed)
    (Variables|Default|SetArmed false)
    (Audio|PlaySoundatLocation "/Game/Engine/StarterContent/Audio/Explosion01.Explosion01" _returnvalue)
    (Effects|SpawnEmitteratLocation "/Game/ParticleSystems/P_SmokeSprayCircluar.P_SmokeSprayCircluar" _returnvalue "0, 0, 0" "5.000000,5.000000,5.000000")
    (Effects|SpawnEmitteratLocation "/Game/ParticleSystems/P_SmokeSpray.P_SmokeSpray" _returnvalue "0, 0, 0" "5.000000,5.000000,5.000000")
    (for _index (range 0 (Variables|Default|GetCowCount))
      (bind _returnvalue_2 (AI|SpawnAIFromClass "/Game/Blueprints/Characters/Cow/MiniCowBP.MiniCowBP_C" "/Game/Blueprints/Characters/Cow/Cow_BT.Cow_BT" (+ (Transformation|GetActorLocation) (Math|Vector|RotateVectorAroundAxis (* "1.000000, 0,0.000000" (Variables|Default|GetSpawnRadius)) (+ (* _index (/ 3.6e+02 (Math|Conversions|ToFloat(Integer) (Variables|Default|GetCowCount)))) (Math|Random|RandomFloatinRange -1e+01 1e+01)) "0, 0,1.000000")) (Math|Random|RandomRotator false) true))
      (bind _ascharacter (Utilities|Casting|CastToCharacter _returnvalue_2))
      (Character|LaunchCharacter _ascharacter (* (Math|Vector|Normalize (- (+ (Transformation|GetActorLocation _ascharacter) "0, 0,300.000000") (Transformation|GetActorLocation))) (Math|Random|RandomFloatinRange 5e+02 7.5e+02)) false false))
    (bind _outactors (Collision|SphereOverlapActors (Transformation|GetActorLocation) (Variables|Default|GetExplosionRadius) (Utilities|Array|MakeArray "ObjectTypeQuery2") 0))
    (for _array_element _outactors
      _)
    (Utilities|FlowControl|Delay 0.05)
    (Actor|DestroyActor)))

(event EventTick
  (params (DeltaSeconds :type Float%20%28single-precision%29)))

(fn ConstructionScript
  (|CallParentFunction))