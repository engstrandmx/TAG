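; Base Blueprint for the gnome character, adding audio, effects and HUD feedback to gameplay events.
; Hit, death, gold pickup, jump and landing play FMOD events, with a particle spray on gold.
; Hit and death share a tail that retriggers the FMOD audio component with a Hit parameter.
; BeginPlay creates the gnome HUD for the TAG player controller and clears its blur; Escape quits the game.
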(event Custom|OnGoldPickup
  (Class|FMODBlueprintStatics|PlayEventatLocation "/Game/FMOD/Events/Sfx/Gnom_take_coins.Gnom_take_coins" (Transformation|GetActorTransform))
  (Effects|SpawnEmitteratLocation "/Game/ParticleSystems/P_GoldSpray.P_GoldSpray" (Transformation|GetActorLocation)))

(event EventBeginPlay
  (Class|FMODBlueprintStatics|PlayEventatLocation 0 (Transformation|GetActorTransform))
  (bind _astagplayer_controller (Utilities|Casting|CastToTAGPlayerController (Pawn|GetController)))
  (bind _returnvalue (UserInterface|CreateWidget "/Game/Blueprints/UI/GnomeHUD_BP.GnomeHUD_BP_C" _astagplayer_controller))
  (bind _output_get (Variables|Default|SetHUD _returnvalue))
  (UserInterface|Viewport|AddtoViewport _output_get 0)
  (Variables|/Game/Blueprints/UI/GnomeHUD_BP.GnomeHUD_BP_C|SetController (Variables|Default|GetHUD) _astagplayer_controller)
  (Default|BlurScreen (Variables|Default|GetHUD) false))

(event Collision|EventActorBeginOverlap
  (params (OtherActor :type Actor%20Object%20Reference)))

(event EventOnHit
  (bind _fmodaudio (Variables|Default|GetFMODAudio))
  (Class|FMODBlueprintStatics|PlayEventatLocation "/Game/FMOD/Events/Gnom/Gnom_gets_hit.Gnom_gets_hit" (Transformation|GetActorTransform))
  (Class|FMODAudioComponent|SetEvent _fmodaudio "/Game/FMOD/Events/Troll/Troll_hits_material.Troll_hits_material")
  (Class|FMODAudioComponent|SetParameter _fmodaudio "Hit" 1.0)
  (Class|FMODAudioComponent|Play _fmodaudio))

(event EventTick
  (params (DeltaSeconds :type Float%20%28single-precision%29)))

(event EventOnJumped
  (Class|FMODBlueprintStatics|PlayEventAttached "/Game/FMOD/Events/Gnom/Gnom_Jump.Gnom_Jump" (Variables|Character|GetMesh) "None" "0, 0, 0" "KeepRelativeOffset"))

(event EventOnLanded
  (params (Hit :type Hit%20Result%20Structure%20%28by%20ref%29))
  (Class|FMODBlueprintStatics|PlayEventAttached "/Game/FMOD/Events/Gnom/Gnom_Land.Gnom_Land" (Variables|Character|GetMesh) "None" "0, 0, 0" "KeepRelativeOffset"))

(event EventOnDeath
  (bind _fmodaudio (Variables|Default|GetFMODAudio))
  (Class|FMODBlueprintStatics|PlayEventatLocation "/Game/FMOD/Events/Gnom/Gnom_die.Gnom_die" (Transformation|GetActorTransform))
  (Default|BlurScreen (Variables|Default|GetHUD) false)
  (Class|FMODAudioComponent|SetEvent _fmodaudio "/Game/FMOD/Events/Troll/Troll_hits_material.Troll_hits_material")
  (Class|FMODAudioComponent|SetParameter _fmodaudio "Hit" 1.0)
  (Class|FMODAudioComponent|Play _fmodaudio))

(event Input|KeyboardEvents|Escape
  (params (Key :type Key%20Structure :default "AnyKey"))
  (:Pressed
    (Game|QuitGame 0 "Quit")))

(fn ConstructionScript
  (|CallParentFunction))