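; Gnome character Blueprint with a score HUD and a debug-style B key toggle for physics simulation on its mesh.
; BeginPlay adds the ScoreBlueprint widget to the viewport and caches the mesh's relative location.
; Turning physics off snaps the mesh to the capsule's world location plus that cached offset, matches the capsule's rotation, then runs a keep-relative component attach with the mesh as parent.
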(event EventBeginPlay
  (bind _returnvalue (UserInterface|CreateWidget "/Game/Blueprints/UI/ScoreBlueprint.ScoreBlueprint_C"))
  (bind _output_get (Variables|Default|SetHUD _returnvalue))
  (UserInterface|Viewport|AddtoViewport _output_get 0)
  (Variables|Default|SetInitialLocation (Variables|/Script/Engine.SceneComponent|GetRelativeLocation (Variables|Character|GetMesh))))

(event Collision|EventActorBeginOverlap
  (params (OtherActor :type Actor%20Object%20Reference)))

(event EventTick
  (params (DeltaSeconds :type Float%20%28single-precision%29)))

(event Input|KeyboardEvents|B
  (params (Key :type Key%20Structure :default "AnyKey"))
  (bind _capsulecomponent (Variables|Default|GetCapsuleComponent))
  (bind _mesh (Variables|Character|GetMesh))
  (:Pressed
    (bind _output_get (Variables|Default|SetSimulatePhysics (not (Variables|Default|GetSimulatePhysics))))
    (Physics|SetSimulatePhysics (Variables|Character|GetMesh) _output_get)
    (if (not _output_get)
      (Transformation|SetWorldLocationAndRotation _mesh (+ (Variables|Default|GetInitialLocation) (Transformation|GetWorldLocation _capsulecomponent)) (Transformation|GetWorldRotation _capsulecomponent) false false)
      (Transformation|AttachComponentToComponent _mesh "None" "KeepRelative" "KeepRelative" "KeepRelative" true))))

(fn ConstructionScript
  (|CallParentFunction))