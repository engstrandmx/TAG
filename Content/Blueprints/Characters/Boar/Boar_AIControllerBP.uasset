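; AI controller for the boar enemy that makes it change direction in response to perceiving a troll character.
; On BeginPlay it caches the controlled pawn as the boar base Blueprint.
; AI perception updates for troll-class actors trigger the boar's direction change unless it is charging, stunned or flipped over.
; A DoOnce reset after a short delay acts as a cooldown between reactions.
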(event OnTargetPerceptionUpdated(AIPerceptionComponent)
  (params (Actor :type Actor%20Object%20Reference) (Stimulus :type AI%20Stimulus%20Structure))
  (bind _boar (Variables|Default|GetBoar))
  (if (and (Utilities|ClassIsChildOf (Utilities|GetClass Actor) "/Script/TAG.TrollCharacter") (not (Math|Boolean|ORBoolean (Variables|/Script/TAG.BoarCharacter|GetbCharging _boar) (Variables|/Script/TAG.BoarCharacter|GetbStunned _boar) (Variables|/Game/Blueprints/Characters/BoarBP_Base.BoarBP_Base_C|GetFlippedOver _boar))))
    (Utilities|FlowControl|DoOnce false :!label _label
      (:Completed
        (Default|ChangeDircection (Variables|Default|GetBoar))
        (Utilities|FlowControl|Delay 2.0)
        (goto _label Reset)))))

(event EventTick
  (params (DeltaSeconds :type Float%20%28single-precision%29)))

(event EventBeginPlay
  (bind _asboar_bp_base (Utilities|Casting|CastToBoarBP_Base (Pawn|GetControlledPawn)))
  (Variables|Default|SetBoar _asboar_bp_base))

(fn ConstructionScript)