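; Base prisoner cow, a rescue collectible trapped in roots that a gnome or troll frees by touch.
; Mesh hit or pickup-sphere overlap triggers once, notifying TAGGameMode_BP and animating the roots' alpha threshold.
; It then plays a saved montage, shrinks and rises on a timeline, and bursts into particles before being destroyed.
; Inherited-looking cow behavior (troll launching, flee states, root material setup) is mostly disconnected or stubbed.
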(event OnInteract(InteractScene)
  (params (TriggeringActor :type Actor%20Object%20Reference)))

(event OnSimulateHit(HittableSceneComponent)
  (params (HittingActor :type Actor%20Object%20Reference) (PowerMultiplier :type Float%20%28single-precision%29) (ForwardVector :type Vector :default "0, 0, 0"))
  ;[1 1 1] On Simulate
)

(event OnComponentBeginOverlap(Box)
  (params (OverlappedComponent :type Primitive%20Component%20Object%20Reference) (OtherActor :type Actor%20Object%20Reference) (OtherComp :type Primitive%20Component%20Object%20Reference) (OtherBodyIndex :type Integer) (bFromSweep :type Boolean) (SweepResult :type Hit%20Result%20Structure%20%28by%20ref%29)))

(event OnComponentHit(HittableSceneComponent)
  (params (HittingActor :type Actor%20Object%20Reference) (PowerMultiplier :type Float%20%28single-precision%29) (ForwardVector :type Vector :default "0, 0, 0"))
  ;[1 1 1] On Component Hit
)

(event OnComponentBeginOverlap(PickupSphere)
  (params (OverlappedComponent :type Primitive%20Component%20Object%20Reference) (OtherActor :type Actor%20Object%20Reference) (OtherComp :type Primitive%20Component%20Object%20Reference) (OtherBodyIndex :type Integer) (bFromSweep :type Boolean) (SweepResult :type Hit%20Result%20Structure%20%28by%20ref%29))
  (bind _returnvalue (Utilities|GetClass OtherActor))
  (bind _mesh (Variables|Character|GetMesh))
  ;[1 1 1] Rescued
  (if (Utilities|ClassIsChildOf _returnvalue "/Script/TAG.GnomeCharacter")
    (if (not (Variables|Default|GetTriggered)) :!label _label
      (Variables|Default|SetTriggered true)
      (Class|FMODAudioComponent|SetParameter (stale EventBeginPlay _returnvalue) "End" 1.0)
      (bind _outactors (Actor|GetAllActorsOfClass "/Game/Blueprints/Gameplay/TAGGameMode_BP.TAGGameMode_BP_C"))
      (Class|TAGGameMode|PickupCollectible (Utilities|Array|Get(acopy) _outactors))
      (bind _newtrack_0 (Timeline|Timeline_0 Play)
        (:Update
          (Rendering|Material|SetScalarParameterValueonMaterials (Variables|Default|Getmodel_root1) "AlphaThresshold" (Math|Float|Lerp 0.0 1.0 _newtrack_0))
          (Rendering|Material|SetScalarParameterValueonMaterials (Variables|Default|Getmodel_root2) "AlphaThresshold" (Math|Float|Lerp 0.0 1.0 _newtrack_0)))
        (:Finished
          (Animation|Montage|PlayMontage (Variables|Character|GetMesh) "/Game/Characters/Cow/Animations/Cow_savedMontage.Cow_savedMontage"
            (:then
              (Class|FMODBlueprintStatics|PlayEventatLocation 0 (Transformation|GetActorTransform))
              (Class|FMODBlueprintStatics|PlayEvent2D)
              (Variables|Default|SetStartRotation (Transformation|GetActorRotation))
              (Variables|Default|SetStartLocation (Transformation|GetActorLocation))
              (bind _newtrack_0_2 (Timeline|FlyAway%20Timeline Play)
                (:Update
                  (Transformation|SetRelativeScale3D _mesh (Math|Vector|Lerp(Vector) "1.000000,1.000000,1.000000" "0.100000,0.100000,0.100000" _newtrack_0_2))
                  (Transformation|SetRelativeLocation _mesh (Math|Vector|Lerp(Vector) "0, 0,-50.000000" "0, 0,200.000000" _newtrack_0_2) false true))
                (:Finished
                  (Effects|SpawnEmitteratLocation (Variables|Default|GetPickup%20Particle) (+ (Transformation|GetActorLocation) "0, 0,200.000000"))
                  (Actor|DestroyActor))))))))
    (elif (Utilities|ClassIsChildOf _returnvalue "/Script/TAG.TrollCharacter")
      (goto _label))))

(event OnComponentHit(Mesh)
  (params (HitComponent :type Primitive%20Component%20Object%20Reference) (OtherActor :type Actor%20Object%20Reference) (OtherComp :type Primitive%20Component%20Object%20Reference) (NormalImpulse :type Vector :default "0, 0, 0") (Hit :type Hit%20Result%20Structure%20%28by%20ref%29))
  (bind _mesh (Variables|Character|GetMesh))
  ;[1 1 1] Rescued
  (if (Utilities|ClassIsChildOf (Utilities|GetClass (stale OnComponentBeginOverlap(PickupSphere) OtherActor)) "/Script/TAG.GnomeCharacter")
    (if (not (Variables|Default|GetTriggered)) :!label _label
      (Variables|Default|SetTriggered true)
      (Class|FMODAudioComponent|SetParameter (stale EventBeginPlay _returnvalue) "End" 1.0)
      (bind _outactors (Actor|GetAllActorsOfClass "/Game/Blueprints/Gameplay/TAGGameMode_BP.TAGGameMode_BP_C"))
      (Class|TAGGameMode|PickupCollectible (Utilities|Array|Get(acopy) _outactors))
      (bind _newtrack_0 (Timeline|Timeline_0 Play)
        (:Update
          (Rendering|Material|SetScalarParameterValueonMaterials (Variables|Default|Getmodel_root1) "AlphaThresshold" (Math|Float|Lerp 0.0 1.0 _newtrack_0))
          (Rendering|Material|SetScalarParameterValueonMaterials (Variables|Default|Getmodel_root2) "AlphaThresshold" (Math|Float|Lerp 0.0 1.0 _newtrack_0)))
        (:Finished
          (Animation|Montage|PlayMontage (Variables|Character|GetMesh) "/Game/Characters/Cow/Animations/Cow_savedMontage.Cow_savedMontage"
            (:then
              (Class|FMODBlueprintStatics|PlayEventatLocation 0 (Transformation|GetActorTransform))
              (Class|FMODBlueprintStatics|PlayEvent2D)
              (Variables|Default|SetStartRotation (Transformation|GetActorRotation))
              (Variables|Default|SetStartLocation (Transformation|GetActorLocation))
              (bind _newtrack_0_2 (Timeline|FlyAway%20Timeline Play)
                (:Update
                  (Transformation|SetRelativeScale3D _mesh (Math|Vector|Lerp(Vector) "1.000000,1.000000,1.000000" "0.100000,0.100000,0.100000" _newtrack_0_2))
                  (Transformation|SetRelativeLocation _mesh (Math|Vector|Lerp(Vector) "0, 0,-50.000000" "0, 0,200.000000" _newtrack_0_2) false true))
                (:Finished
                  (Effects|SpawnEmitteratLocation (Variables|Default|GetPickup%20Particle) (+ (Transformation|GetActorLocation) "0, 0,200.000000"))
                  (Actor|DestroyActor))))))))
    (elif (Utilities|ClassIsChildOf (Utilities|GetClass (stale OnComponentBeginOverlap(PickupSphere) OtherActor)) "/Script/TAG.TrollCharacter")
      (goto _label))))

(event Custom|InteractNoAoE
  (params (GnomeRef :type Actor%20Object%20Reference)))

(event EventBeginPlay
  (Components|Sphere|SetSphereRadius (Variables|Default|GetPickupSphere) (* (Variables|Default|GetRescueRange) 1e+02) true)
  (bind _returnvalue (Class|FMODBlueprintStatics|PlayEventAttached 0 (Variables|Character|GetMesh) "None" "0, 0, 0" "KeepRelativeOffset")))

(event EventOnLanded
  (params (Hit :type Hit%20Result%20Structure%20%28by%20ref%29))
  (Class|FMODBlueprintStatics|PlayEventatLocation 0 (Transformation|GetActorTransform))
  (if (Utilities|Enum|NotEqual(Enum) (Variables|Default|GetAI%20State) "VE_Floating")
    (CallFunction|ChangeState "VE_Wandering")))

(fn ConstructionScript
  (bind _charactermovement (Variables|Character|GetCharacterMovement))
  ;[1 1 1] Set speed variables and stuff
  (Variables|Default|SetIntialSpeed (Variables|/Script/Engine.CharacterMovementComponent|GetMaxWalkSpeed _charactermovement))
  (Variables|Default|SetIntialAcceleration (Class|CharacterMovementComponent|GetMaxAcceleration _charactermovement)))

(fn GenerateLine
  (bind _outpathpositions (Class|GameplayStatics|BlueprintPredictProjectilePathbyTraceChannel (Variables|Simulation|GetLaunchLocation) (Variables|Simulation|GetLaunchVelocity) true 1e+01 "ECC_WorldStatic" false 0 "ForOneFrame" 0.0 15.0 1.0))
  (for _array_element _outpathpositions
    (Effects|SpawnEmitteratLocation "/Game/ParticleSystems/Beam/P_ArcBall.P_ArcBall" _array_element)))

(fn ChangeState
  (params (ToState :type EAiState%20Enum :default "VE_Wandering")))

(fn SetSpeed
  (params (Amount :type Float%20%28single-precision%29) (Reset :type Boolean))
  (bind _charactermovement (Variables|Character|GetCharacterMovement))
  (if Reset
    (Variables|/Script/Engine.CharacterMovementComponent|SetMaxAcceleration _charactermovement (Variables|Default|GetIntialAcceleration))
    (Variables|/Script/Engine.CharacterMovementComponent|SetMaxWalkSpeed _charactermovement (Variables|Default|GetIntialSpeed))
    (else
      (Variables|/Script/Engine.CharacterMovementComponent|SetMaxAcceleration _charactermovement (+ (Variables|Default|GetIntialAcceleration) Amount))
      (Variables|/Script/Engine.CharacterMovementComponent|SetMaxWalkSpeed _charactermovement (+ (Variables|Default|GetIntialSpeed) Amount)))))

(fn GenerateHitVector
  (params (HittingActor :type Actor%20Object%20Reference) (PowerMultiplier :type Float%20%28single-precision%29) (ForwardVector :type Vector)))

(fn OrderMoveto
  (params (Location :type Vector))
  (AI|Components|Blackboard|SetValueasVector (AI|GetBlackboard 0) (Utilities|Name|MakeLiteralName "OrderMoveLocation") Location))