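; Cow AI character that wanders on random timers, flees seen gnomes and trolls, and gets launched away when a troll hits it.
; HittableSceneComponent supplies both real hits and simulated ones, using the same launch velocity formula.
; Simulated hits step a gravity arc with line traces to aim the PBeam target at the last trace result.
; A flag cleared every Tick shows the beam only while simulation keeps firing.
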(event OnSeePawn(PawnSensing)
  (params (Pawn :type Pawn%20Object%20Reference))
  (bind _returnvalue (Transformation|GetActorLocation))
  (bind _returnvalue_2 (Utilities|GetClass Pawn))
  ;[1 1 1] AI Run Away
  (if (AI|Components|NavMovement|IsMovingonGround (Variables|Character|GetCharacterMovement))
    (if (and (or (== _returnvalue_2 "/Game/Blueprints/Characters/GnomeCharacter.GnomeCharacter_C") (== _returnvalue_2 "/Game/Blueprints/Characters/TrollCharacter.TrollCharacter_C")) (not (Variables|Simulation|GetSimulatingHit)))
      (AI|AIMoveTo self (+ (* (Math|Vector|Normalize (- _returnvalue (Transformation|GetActorLocation Pawn))) (Variables|AI|GetRunAwayDistance)) _returnvalue) 0 0.1 false))))

(event OnSimulateHit(HittableSceneComponent)
  (params (HittingActor :type Actor%20Object%20Reference) (PowerMultiplier :type Float%20%28single-precision%29))
  ;[1 1 1] On Simulate
  (Variables|Simulation|SetLineRotation (Transformation|GetActorRotation))
  (Variables|Simulation|SetLaunchVelocity (* (* (Math|Vector|Normalize (- (Transformation|GetActorLocation) (+ (Transformation|GetActorLocation HittingActor) "0, 0,-300.000000"))) (Variables|/Game/Blueprints/HittableSceneComponent.HittableSceneComponent_C|GetHitForce (Variables|Default|GetHittableSceneComponent))) PowerMultiplier))
  (Variables|Simulation|SetLaunchLocation (Transformation|GetActorLocation))
  (CallFunction|GenerateLine)
  (Variables|Simulation|SetSimulatingHit true))

(event OnComponentHit(HittableSceneComponent)
  (params (HittingActor :type Actor%20Object%20Reference) (PowerMultiplier :type Float%20%28single-precision%29))
  ;[1 1 1] On Component Hit
  (if (== (Utilities|GetClass HittingActor) "/Game/Blueprints/Characters/TrollCharacter.TrollCharacter_C")
    (Components|Movement|StopMovementImmediately (Variables|Character|GetCharacterMovement))
    (Character|LaunchCharacter (* (* (Math|Vector|Normalize (- (Transformation|GetActorLocation) (+ (Transformation|GetActorLocation HittingActor) "0, 0,-300.000000"))) (Variables|/Game/Blueprints/HittableSceneComponent.HittableSceneComponent_C|GetHitForce (Variables|Default|GetHittableSceneComponent))) PowerMultiplier) false false)))

(event Custom|OnAIWander
  (bind _minwander (Variables|AI|GetMinWander))
  (bind _maxwander (Variables|AI|GetMaxWander))
  (bind (_x _y) (Math|Vector|BreakVector _minwander))
  (bind (_x_2 _y_2) (Math|Vector|BreakVector _maxwander))
  ;[1 1 1] AI Wander
  (if (not (Variables|Simulation|GetSimulatingHit))
    (AI|AIMoveTo self (+ (Transformation|GetActorLocation) (Math|Vector|MakeVector (Math|Random|RandomFloatinRange _x _x_2) (Math|Random|RandomFloatinRange _y _y_2) 0.0)) 0 5.0 false
      (:then
        (Variables|AI|SetRandomWanderTime (Math|Random|RandomFloatinRange 5.0 1e+01))
        (Utilities|Time|SetTimerbyEvent (delegate Custom|OnAIWander) (Variables|AI|GetRandomWanderTime))))))

(event EventBeginPlay
  (CallFunction|OnAIWander))

(event EventOnLanded
  (params (Hit :type Hit%20Result%20Structure%20%28by%20ref%29)))

(event EventTick
  (params (DeltaSeconds :type Float%20%28single-precision%29))
  ;[1 1 1] Arc Show/Hide
  (if (Variables|Simulation|GetSimulatingHit)
    (Variables|Simulation|SetSimulatingHit false)
    (Rendering|SetVisibility (Variables|Default|GetP_Beam) true false)
    (else
      (Rendering|SetVisibility (Variables|Default|GetP_Beam) false false))))

(fn ConstructionScript)

(fn GenerateLine
  (Variables|Simulation|SetVelocity (Variables|Simulation|GetLaunchVelocity))
  (Variables|Simulation|SetLocation (+ (Variables|Simulation|GetLaunchLocation) "0.000000,0.000000,0.000000"))
  (for _index (range 0 (Variables|Simulation|GetSimLength))
    (Variables|Simulation|SetVelocity (+ (Variables|Simulation|GetVelocity) (* (* (Variables|Simulation|GetGravity) (Variables|Simulation|GetGravity%20Scale)) (Variables|Simulation|GetDelta%20Sim))))
    (Variables|Simulation|SetNextLocation (+ (* (Variables|Simulation|GetVelocity) (Variables|Simulation|GetDelta%20Sim)) (Variables|Simulation|GetLocation)))
    (bind _outhit (Collision|LineTraceForObjects (Variables|Simulation|GetLocation) (Variables|Simulation|GetNextLocation) (Utilities|Array|MakeArray "ObjectTypeQuery1" "ObjectTypeQuery2" "ObjectTypeQuery4" "ObjectTypeQuery3") false 0 "None"))
    (LocalVariables|SetHitResult _outhit)
    (Variables|Simulation|SetLocation (Variables|Simulation|GetNextLocation)))
  (Class|ParticleSystemComponent|SetBeamTargetPoint (Variables|Default|GetP_Beam) 0 (.Location (Collision|BreakHitResult (LocalVariables|GetHitResult)))))