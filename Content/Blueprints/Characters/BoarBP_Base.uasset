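; Base boar boss Blueprint running a phased fight against the Troll and Gnome, with music tracking its state.
; Randomised timer loops wait until it is idle, then charge or turn it by driving AI blackboard keys.
; Hits while charging flip it over and launch the Troll, opening an interact window that drains phase health.
; Later phases add piglets, then smoke with spawned fog chargers, and the last plays its death.
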(event OnComponentBeginOverlap(SphereCollider)
  (params (OverlappedComponent :type Primitive%20Component%20Object%20Reference) (OtherActor :type Actor%20Object%20Reference) (OtherComp :type Primitive%20Component%20Object%20Reference) (OtherBodyIndex :type Integer) (bFromSweep :type Boolean) (SweepResult :type Hit%20Result%20Structure%20%28by%20ref%29))
  (bind _returnvalue (Utilities|GetClass OtherActor))
  ;[1 1 1] On Front Begin Overlap
  (if (not (Variables|Default|GetbStunned))
    (Utilities|FlowControl|Sequence
      (:then_0
        (bind _ascustom_destructible_actor (Utilities|Casting|CastToCustomDestructibleActor OtherActor))
        (if (and (not (Variables|/Script/TAG.CustomDestructibleActor|GetbDestroyed _ascustom_destructible_actor)) (== _returnvalue "/Script/TAG.CustomDestructibleActor"))
          (Class|CustomDestructibleActor|MarkDestroyed _ascustom_destructible_actor true)
          (Class|DestructibleComponent|ApplyRadiusDamage (Actor|GetComponentbyClass OtherActor "/Script/ApexDestruction.DestructibleComponent") 1e+03 (Transformation|GetActorLocation) 5e+02 1e+03 true)
          (CallFunction|Stun 2.0)
          (CallFunction|SetCharging false)))
      (:then_1
        (if (Utilities|ClassIsChildOf _returnvalue "/Script/TAG.TrollCharacter")
          (bind _astroll_character_base (Utilities|Casting|CastToTrollCharacter_Base OtherActor))
          (Default|Stun _astroll_character_base 1.5)
          (Character|LaunchCharacter _astroll_character_base (+ (* (+ (Math|Vector|Normalize (- (Transformation|GetActorLocation OtherActor) (Transformation|GetActorLocation))) (Math|Vector|GetUpVector "0, 0, 0")) 5e+02) (* (Transformation|GetActorRightVector) (Math|Random|RandomFloatinRange -3e+02 3e+02))) true true)
          (Utilities|FlowControl|Delay 1.0)
          (CallFunction|SetCharging false)
          (if (Variables|Default|GetbCharging)
            (AI|Components|Blackboard|ClearValue (AI|GetBlackboard (Variables|Default|GetBoarController)) (Utilities|Name|MakeLiteralName "ChargeTarget"))
            (CallFunction|SetCharging false)))))))

(event OnComponentHit(HittableSceneComponent)
  (params (HittingActor :type Actor%20Object%20Reference) (PowerMultiplier :type Float%20%28single-precision%29) (ForwardVector :type Vector :default "0, 0, 0"))
  (bind _returnvalue (Transformation|GetActorRotation))
  (bind _returnvalue_2 (Transformation|GetActorRotation))
  (bind (_roll _pitch _yaw) (Math|Rotator|BreakRotator _returnvalue))
  (bind (_roll_2 _pitch_2 _yaw_2) (Math|Rotator|BreakRotator _returnvalue_2))
  (if (and (> (Variables|Default|GetHitDelay) 0.5) (Variables|Default|GetbCharging))
    (Variables|Default|SetHitDelay 0.0)
    (Variables|Default|SetFlippedOver true)
    (Class|FMODBlueprintStatics|EventInstanceSetParameter (Variables|Default|GetMusic) "Lvl int" 0.0)
    (CallFunction|Stun (Variables|Timers|GetFlippedOverTime))
    (Utilities|FlowControl|Sequence
      (:then_0
        ;[1 1 1] Rotate boar back after delay
        (Utilities|FlowControl|Delay (- (Variables|Timers|GetFlippedOverTime) 1.0))
        (bind _driver (Timeline|Timeline_0 PlayFromStart)
          (:Update
            (Transformation|SetActorRotation (Math|Rotator|MakeRotator (* _driver 1.8e+02) _pitch _yaw))
            (Utilities|FlowControl|Delay (Variables|Timers|GetFlippedOverTime))
            (Variables|Default|SetFlippedOver false)
            (Class|FMODBlueprintStatics|EventInstanceSetParameter (Variables|Default|GetMusic) "Lvl int" (Math|Conversions|ToFloat(Integer) (Variables|Default|GetCurrentPhase))))))
      (:then_1
        ;[1 1 1] Rotate Boar
        (bind _driver_2 (Timeline|FlipTimeline PlayFromStart)
          (:Update
            (Transformation|SetActorRotation (Math|Rotator|MakeRotator (* _driver_2 1.8e+02) _pitch_2 _yaw_2)))))
      (:then_2
        ;[1 1 1] Apply Force To Troll and Boar
        (bind _returnvalue_3 (Class|TAGGameMode|GetTrollCharacter (Variables|Default|GetGameMode)))
        (bind _astroll_character_base (Utilities|Casting|CastToTrollCharacter_Base _returnvalue_3))
        (Default|Stun _astroll_character_base (Variables|Timers|GetFlippedOverTime))
        (Rendering|ToggleVisibility (Variables|/Game/Blueprints/Characters/TrollCharacter_Base.TrollCharacter_Base_C|GetGnomeMesh _astroll_character_base) false)
        (Class|TrollCharacter|FinishDismount _returnvalue_3 (+ (Transformation|GetActorLocation _returnvalue_3) "0, 0,200.000000"))
        (Character|LaunchCharacter _returnvalue_3 (* (+ (Math|Vector|Normalize (- (Transformation|GetActorLocation _returnvalue_3) (Transformation|GetActorLocation))) "0, 0,1.000000") 5e+02) false false)
        (Character|LaunchCharacter (* (+ (* (Math|Vector|Normalize (- (Transformation|GetActorLocation _returnvalue_3) (Transformation|GetActorLocation))) -1) "0, 0,1.000000") 5e+02) true true)
        (Effects|SpawnEmitteratLocation "/Game/ParticleSystems/P_ImpactLarge.P_ImpactLarge" (+ (/ (- (Transformation|GetActorLocation _returnvalue_3) (Transformation|GetActorLocation)) 2.0) (Transformation|GetActorLocation)) (Math|Conversions|RotationFromXVector (+ (/ (- (Transformation|GetActorLocation _returnvalue_3) (Transformation|GetActorLocation)) 2.0) (Transformation|GetActorLocation))) "2.000000,2.000000,2.000000")
        (bind _returnvalue_4 (Class|FMODBlueprintStatics|PlayEventatLocation "/Game/FMOD/Events/Troll/Troll_hits_material.Troll_hits_material" (Math|Conversions|ToTransform(Vector) (+ (/ (- (Transformation|GetActorLocation _returnvalue_3) (Transformation|GetActorLocation)) 2.0) (Transformation|GetActorLocation))) false))
        (Class|FMODBlueprintStatics|EventInstanceSetParameter _returnvalue_4 "Material" 4.0)
        (Class|FMODBlueprintStatics|EventInstancePlay _returnvalue_4)
        (if (Variables|Default|GetbCharging)
          (AI|Components|Blackboard|ClearValue (AI|GetBlackboard (Variables|Default|GetBoarController)) (Utilities|Name|MakeLiteralName "ChargeTarget"))
          (CallFunction|SetCharging false)
          (Audio|PlaySound2D "/Game/Engine/StarterContent/Audio/Explosion01.Explosion01"))))))

(event OnInteract(InteractScene)
  (params (TriggeringActor :type Actor%20Object%20Reference))
  ;[1 1 1] On Interact
  (if (Variables|Default|GetFlippedOver)
    (Effects|SpawnEmitteratLocation "/Game/ParticleSystems/P_HeartSprayNoLoop.P_HeartSprayNoLoop" (Transformation|GetActorLocation) "0, 0, 0" "4.000000,4.000000,4.000000")
    (bind _result (Math|Integer|DecrementInt (Variables|Default|GetHealth))
      (:%20%20
        (if (== _result 0)
          (Class|FMODBlueprintStatics|EventInstanceSetParameter (Variables|Default|GetMusic) "Win/Fail" 1.0)
          (Utilities|FlowControl|Delay 2.0)
          (CallFunction|StartNextPhase))))))

(event OnComponentHit(HittableSceneComponent2)
  (params (HittingActor :type Actor%20Object%20Reference) (PowerMultiplier :type Float%20%28single-precision%29) (ForwardVector :type Vector :default "0, 0, 0"))
  (bind _returnvalue (Transformation|GetActorRotation))
  (bind _returnvalue_2 (Transformation|GetActorRotation))
  (bind (_roll _pitch _yaw) (Math|Rotator|BreakRotator _returnvalue))
  (bind (_roll_2 _pitch_2 _yaw_2) (Math|Rotator|BreakRotator _returnvalue_2))
  (if (and (> (Variables|Default|GetHitDelay) 0.5) (Variables|Default|GetbCharging))
    (Variables|Default|SetHitDelay 0.0)
    (Variables|Default|SetFlippedOver true)
    (Class|FMODBlueprintStatics|EventInstanceSetParameter (Variables|Default|GetMusic) "Lvl int" 0.0)
    (CallFunction|Stun (Variables|Timers|GetFlippedOverTime))
    (Utilities|FlowControl|Sequence
      (:then_0
        ;[1 1 1] Rotate boar back after delay
        (Utilities|FlowControl|Delay (- (Variables|Timers|GetFlippedOverTime) 1.0))
        (bind _driver (Timeline|Timeline_0 PlayFromStart)
          (:Update
            (Transformation|SetActorRotation (Math|Rotator|MakeRotator (* _driver 1.8e+02) _pitch _yaw))
            (Utilities|FlowControl|Delay (Variables|Timers|GetFlippedOverTime))
            (Variables|Default|SetFlippedOver false)
            (Class|FMODBlueprintStatics|EventInstanceSetParameter (Variables|Default|GetMusic) "Lvl int" (Math|Conversions|ToFloat(Integer) (Variables|Default|GetCurrentPhase))))))
      (:then_1
        ;[1 1 1] Rotate Boar
        (bind _driver_2 (Timeline|FlipTimeline PlayFromStart)
          (:Update
            (Transformation|SetActorRotation (Math|Rotator|MakeRotator (* _driver_2 1.8e+02) _pitch_2 _yaw_2)))))
      (:then_2
        ;[1 1 1] Apply Force To Troll and Boar
        (bind _returnvalue_3 (Class|TAGGameMode|GetTrollCharacter (Variables|Default|GetGameMode)))
        (bind _astroll_character_base (Utilities|Casting|CastToTrollCharacter_Base _returnvalue_3))
        (Default|Stun _astroll_character_base (Variables|Timers|GetFlippedOverTime))
        (Rendering|ToggleVisibility (Variables|/Game/Blueprints/Characters/TrollCharacter_Base.TrollCharacter_Base_C|GetGnomeMesh _astroll_character_base) false)
        (Class|TrollCharacter|FinishDismount _returnvalue_3 (+ (Transformation|GetActorLocation _returnvalue_3) "0, 0,200.000000"))
        (Character|LaunchCharacter _returnvalue_3 (* (+ (Math|Vector|Normalize (- (Transformation|GetActorLocation _returnvalue_3) (Transformation|GetActorLocation))) "0, 0,1.000000") 5e+02) false false)
        (Character|LaunchCharacter (* (+ (* (Math|Vector|Normalize (- (Transformation|GetActorLocation _returnvalue_3) (Transformation|GetActorLocation))) -1) "0, 0,1.000000") 5e+02) true true)
        (Effects|SpawnEmitteratLocation "/Game/ParticleSystems/P_ImpactLarge.P_ImpactLarge" (+ (/ (- (Transformation|GetActorLocation _returnvalue_3) (Transformation|GetActorLocation)) 2.0) (Transformation|GetActorLocation)) (Math|Conversions|RotationFromXVector (+ (/ (- (Transformation|GetActorLocation _returnvalue_3) (Transformation|GetActorLocation)) 2.0) (Transformation|GetActorLocation))) "2.000000,2.000000,2.000000")
        (bind _returnvalue_4 (Class|FMODBlueprintStatics|PlayEventatLocation "/Game/FMOD/Events/Troll/Troll_hits_material.Troll_hits_material" (Math|Conversions|ToTransform(Vector) (+ (/ (- (Transformation|GetActorLocation _returnvalue_3) (Transformation|GetActorLocation)) 2.0) (Transformation|GetActorLocation))) false))
        (Class|FMODBlueprintStatics|EventInstanceSetParameter _returnvalue_4 "Material" 4.0)
        (Class|FMODBlueprintStatics|EventInstancePlay _returnvalue_4)
        (if (Variables|Default|GetbCharging)
          (AI|Components|Blackboard|ClearValue (AI|GetBlackboard (Variables|Default|GetBoarController)) (Utilities|Name|MakeLiteralName "ChargeTarget"))
          (CallFunction|SetCharging false)
          (Audio|PlaySound2D "/Game/Engine/StarterContent/Audio/Explosion01.Explosion01"))))))

(event Custom|Charge
  ;[1 1 1] Charge
  (bind _returnvalue (Class|TAGGameMode|GetTrollCharacter (Variables|Default|GetGameMode)))
  (CallFunction|SetCharging true)
  (CallFunction|Stun 1.5)
  (Utilities|FlowControl|Delay 0.5)
  (Variables|Default|SetFaceEnemy true)
  (Utilities|FlowControl|Delay 1.0)
  (Class|FMODBlueprintStatics|PlayEventatLocation "/Game/FMOD/Events/Gloson/Gloson_attack_scream.Gloson_attack_scream" (Transformation|GetActorTransform))
  (CallFunction|SetFireEffect false)
  (Variables|Default|SetFaceEnemy false)
  (AI|Components|Blackboard|SetValueasObject (AI|GetBlackboard (Variables|Default|GetBoarController)) (Utilities|Name|MakeLiteralName "ChargeTarget") _returnvalue)
  (Utilities|FlowControl|Delay (/ (* 2 (Variables|/Game/Blueprints/Characters/Boar/BoarCircleSpline.BoarCircleSpline_C|GetRadius (Variables|Default|GetCircleSpline))) (Class|MovementComponent|GetMaxSpeed (Variables|Character|GetCharacterMovement))))
  (AI|Components|Blackboard|ClearValue (AI|GetBlackboard (Variables|Default|GetBoarController)) (Utilities|Name|MakeLiteralName "ChargeTarget"))
  (CallFunction|SetFireEffect true)
  (Utilities|FlowControl|Delay 3.0)
  (CallFunction|SetCharging false))

(event Custom|Stun
  (params (Time :type Float%20%28single-precision%29))
  ;[1 1 1] Stun
  (Variables|Default|SetbStunned true)
  (AI|Components|Blackboard|SetValueasBool (AI|GetBlackboard (Variables|Default|GetBoarController)) (Utilities|Name|MakeLiteralName "Stop") true)
  (Utilities|FlowControl|RetriggerableDelay Time)
  (AI|Components|Blackboard|ClearValue (AI|GetBlackboard (Variables|Default|GetBoarController)) (Utilities|Name|MakeLiteralName "Stop"))
  (Variables|Default|SetbStunned false))

(event Custom|Fog%20Charge%20Loop
  (Utilities|FlowControl|Delay (+ (Variables|Timers|GetFogChargeInterval) (* (Math|Random|RandomFloatinRange -1.0 1.0) (Variables|Timers|GetFogChargeDilation))))
  (Utilities|WaitWhileBusy
    (:Complete
      (CallFunction|FogCharge)
      (CallFunction|FogChargeLoop))))

(event Custom|Charge%20Loop
  (Utilities|FlowControl|Delay (+ (Variables|Timers|GetChargeInterval) (* (Math|Random|RandomFloatinRange -1.0 1.0) (Variables|Timers|GetChargeDilation))))
  (Utilities|WaitWhileBusy
    (:Complete
      (CallFunction|Charge)
      (CallFunction|ChargeLoop))))

(event Custom|Change%20Dircection
  ;[1 1 1] Change Direction
  (AI|Components|Blackboard|SetValueasBool (AI|GetBlackboard (Variables|Default|GetBoarController)) (Utilities|Name|MakeLiteralName "Stop") true)
  (AI|AIMoveTo self (+ (* (Transformation|GetActorForwardVector) -25) (Transformation|GetActorLocation)) 0 5.0 false
    (:OnSuccess
      (AI|Components|Blackboard|ClearValue (AI|GetBlackboard (Variables|Default|GetBoarController)) (Utilities|Name|MakeLiteralName "Stop")))))

(event Custom|FogCharge
  (CallFunction|Stun 15.0)
  (for _array_element (Variables|Default|GetPiglets)
    (bind _aspiglet_bp (Utilities|Casting|CastToPigletBP _array_element))
    (Default|SetMoveOutOfWay _aspiglet_bp true))
  (Rendering|SetVisibility (Variables|Default|GetSphere) false true)
  (bind _index (Utilities|DelayedforLoop 1 3 4.0)
    (:LoopBody
      (CallFunction|SpawnFogCharger (+ (Spline|GetLocationatTime (Variables|/Game/Blueprints/Characters/Boar/BoarCircleSpline.BoarCircleSpline_C|GetSpline (Variables|Default|GetCircleSpline)) (* _index (Math|Random|RandomFloatinRange 0.22 0.33)) "World" false) (* (Math|Vector|Normalize (- (+ (Transformation|GetActorLocation (Variables|Default|GetCircleSpline)) (* (Math|Vector|ProjectVectorontoPlane (Math|Random|RandomUnitVector) "0, 0,1.000000") (/ (Variables|/Game/Blueprints/Characters/Boar/BoarCircleSpline.BoarCircleSpline_C|GetRadius (Variables|Default|GetCircleSpline)) 2.0))) (Spline|GetLocationatTime (Variables|/Game/Blueprints/Characters/Boar/BoarCircleSpline.BoarCircleSpline_C|GetSpline (Variables|Default|GetCircleSpline)) (* _index (Math|Random|RandomFloatinRange 0.22 0.33)) "World" false))) -5e+02)) (* (Math|Vector|Normalize (- (+ (Transformation|GetActorLocation (Variables|Default|GetCircleSpline)) (* (Math|Vector|ProjectVectorontoPlane (Math|Random|RandomUnitVector) "0, 0,1.000000") (/ (Variables|/Game/Blueprints/Characters/Boar/BoarCircleSpline.BoarCircleSpline_C|GetRadius (Variables|Default|GetCircleSpline)) 2.0))) (Spline|GetLocationatTime (Variables|/Game/Blueprints/Characters/Boar/BoarCircleSpline.BoarCircleSpline_C|GetSpline (Variables|Default|GetCircleSpline)) (* _index (Math|Random|RandomFloatinRange 0.22 0.33)) "World" false))) 25.0)))
    (:Completed
      (Rendering|SetVisibility (Variables|Default|GetSphere) true true)
      (for _array_element_2 (Variables|Default|GetPiglets)
        (bind _aspiglet_bp_2 (Utilities|Casting|CastToPigletBP _array_element_2))
        (Default|SetMoveOutOfWay _aspiglet_bp_2 false)))))

(event Custom|Turn%20Around%20Loop
  (Utilities|FlowControl|Delay (+ (Variables|Timers|GetTurnAroundInterval) (* (Math|Random|RandomFloatinRange -1.0 1.0) (Variables|Timers|GetTurnAroundDilation))))
  (Utilities|WaitWhileBusy
    (:Complete
      (CallFunction|ChangeDircection)
      (CallFunction|TurnAroundLoop))))

(event Custom|Death
  (CallFunction|Stun 1e+01)
  (bind _scale (Timeline|DeathTimeline PlayFromStart)
    (:Update
      (Transformation|SetActorScale3D _scale))
    (:Finished
      (Effects|SpawnEmitteratLocation "/Game/Engine/StarterContent/Particles/P_Explosion.P_Explosion" (Transformation|GetActorLocation) "0, 0, 0" "10.000000,10.000000,10.000000")
      (bind _returnvalue (Class|TAGGameMode|GetGnomeCharacter (Variables|Default|GetGameMode)))
      (bind _asgnome_character_base (Utilities|Casting|CastToGnomeCharacter_Base _returnvalue))
      (Components|Animation|PlayAnimation (Variables|/Script/Engine.Character|GetMesh _asgnome_character_base) "/Game/Characters/Gnome/Animation/Walking/Gnome_Dance.Gnome_Dance" false)
      (Actor|DestroyActor))))

(event EventBeginPlay
  (bind _returnvalue (Pawn|GetController))
  (Utilities|FlowControl|Sequence
    (:then_0
      (CallFunction|TurnAroundLoop)
      (CallFunction|ChargeLoop)
      (bind _returnvalue_2 (Class|FMODBlueprintStatics|PlayEvent2D "/Game/FMOD/Events/Music/Music_Gloson.Music_Gloson"))
      (bind _output_get (Variables|Default|SetMusic _returnvalue_2))
      (Class|FMODBlueprintStatics|EventInstanceSetParameter _output_get "Lvl int" 1.0))
    (:then_2
      ;[1 1 1] Init BB and vars
      (bind _asboar_aicontroller_bp (Utilities|Casting|CastToBoar_AIControllerBP _returnvalue))
      (Variables|Default|SetBoarController _asboar_aicontroller_bp)
      (AI|Components|Blackboard|SetValueasObject (AI|GetBlackboard _returnvalue) (Utilities|Name|MakeLiteralName "Spline") (Variables|Default|GetCircleSpline))
      (AI|Components|Blackboard|SetValueasVector (AI|GetBlackboard (Variables|Default|GetBoarController)) (Utilities|Name|MakeLiteralName "Origin") (Transformation|GetActorLocation))
      (bind _astaggame_mode_bp (Utilities|Casting|CastToTAGGameMode_BP (Game|GetGameMode)))
      (Variables|Default|SetGameMode _astaggame_mode_bp)
      (CallFunction|StartNextPhase))))

(event Collision|EventActorBeginOverlap
  (params (OtherActor :type Actor%20Object%20Reference)))

(event EventTick
  (params (DeltaSeconds :type Float%20%28single-precision%29))
  (Variables|Default|SetHitDelay (+ DeltaSeconds (Variables|Default|GetHitDelay)))
  (if (Variables|Default|GetFaceEnemy)
    (bind _returnvalue (Class|TAGGameMode|GetTrollCharacter (Variables|Default|GetGameMode)))
    (Transformation|SetActorRotation (Class|KismetMathLibrary|RInterptoConstant (Transformation|GetActorRotation) (Math|Conversions|RotationFromXVector (Math|Vector|Normalize (- (+ (Transformation|GetActorLocation _returnvalue) (Transformation|GetVelocity _returnvalue)) (Transformation|GetActorLocation)))) DeltaSeconds 2e+02))))

(fn ConstructionScript)

(fn SetCharging
  (params (IsCharging :type Boolean))
  (bind _charactermovement (Variables|Character|GetCharacterMovement))
  (bind _output_get (Variables|Default|SetbCharging IsCharging))
  (if _output_get
    (LocalVariables|SetInitialTurnRate (.Yaw (Math|Rotator|BreakRotator (Variables|/Script/Engine.CharacterMovementComponent|GetRotationRate _charactermovement))))
    (Variables|/Script/Engine.CharacterMovementComponent|SetRotationRate _charactermovement (Math|Rotator|MakeRotator 0.0 0.0 (LocalVariables|GetChargeTurnRate)))
    (else
      (Variables|/Script/Engine.CharacterMovementComponent|SetRotationRate (Variables|Character|GetCharacterMovement) (Math|Rotator|MakeRotator 0.0 0.0 (LocalVariables|GetInitialTurnRate))))))

(fn StartNextPhase
  (bind _returnvalue (Transformation|GetActorRotation))
  (bind _returnvalue_2 (Transformation|GetActorLocation))
  (bind _returnvalue_3 (Transformation|GetActorForwardVector))
  (bind _returnvalue_4 (Transformation|GetActorRotation))
  (bind (_roll _pitch _yaw) (Math|Rotator|BreakRotator _returnvalue))
  (bind (_roll_2 _pitch_2 _yaw_2) (Math|Rotator|BreakRotator _returnvalue_4))
  (bind _returnvalue_5 (+ _returnvalue_3 "0, 0,0.100000"))
  (bind _returnvalue_6 (* _returnvalue_5 1e+03))
  (bind _returnvalue_7 (+ _returnvalue_2 _returnvalue_6))
  (Math|Integer|IncrementInt (Variables|Default|GetCurrentPhase)
    (:%20%20
      (Variables|Default|SetHealth (Utilities|Array|Get(acopy) (Variables|Default|GetHealthInPhases) (Variables|Default|GetCurrentPhase)))
      (CallFunction|Stun 6.0)
      (bind _returnvalue_8 (Game|SpawnActorfromClass "/Game/Blueprints/Gameplay/LookAt_BP.LookAt_BP_C" (Math|Transform|MakeTransform "0, 0, 0") "Undefined" 0 0))
      (Variables|/Game/Blueprints/Gameplay/LookAt_BP.LookAt_BP_C|SetTime _returnvalue_8 4.0)
      (Variables|/Game/Blueprints/Gameplay/LookAt_BP.LookAt_BP_C|SetDisable%20Input _returnvalue_8 true)
      (Transformation|SetWorldLocationAndRotation (Variables|/Game/Blueprints/Gameplay/LookAt_BP.LookAt_BP_C|GetArrow _returnvalue_8) _returnvalue_7 (Math|Conversions|RotationFromXVector (- (- _returnvalue_2 _returnvalue_7) "0, 0,250.000000")) false false)
      (Default|Trigger _returnvalue_8)
      (switch int (Variables|Default|GetCurrentPhase)
        (:2
          ;[1 1 1] Phase 2
          (for _index (range 0 2)
            (bind _returnvalue_9 (Class|BoarCharacter|SpawnPiglet (Math|Vector|RotateVectorAroundAxis (* (Transformation|GetActorRightVector) 3e+02) (* _index 1.8e+02) "0, 0,1.000000") (Math|Rotator|MakeRotator 0.0 _pitch _yaw)))
            (bind _aspiglet_bp (Utilities|Casting|CastToPigletBP _returnvalue_9))
            (Variables|/Game/Blueprints/Characters/PigletBP.PigletBP_C|SetCircleSpline _aspiglet_bp (Variables|Default|GetCircleSpline))
            (Default|Init _aspiglet_bp)
            (Class|FMODBlueprintStatics|EventInstanceSetParameter (Variables|Default|GetMusic) "Lvl int" 2.0))
          (Default|DestroyAllinArea (Variables|Default|GetCircleSpline))
          (CallFunction|StunPiglets 5.0)
          (bind _returnvalue_10 (Class|TAGGameMode|GetGnomeCharacter (Variables|Default|GetGameMode)))
          (Class|GnomeCharacter|InstantMount _returnvalue_10))
        (:3
          ;[1 1 1] Phase 3
          (for _index_2 (range 0 5)
            (bind _returnvalue_11 (Class|BoarCharacter|SpawnPiglet (Math|Vector|RotateVectorAroundAxis (* (Transformation|GetActorRightVector) 3e+02) (* _index_2 6e+01) "0, 0,1.000000") (Math|Rotator|MakeRotator 0.0 _pitch_2 _yaw_2)))
            (bind _aspiglet_bp_2 (Utilities|Casting|CastToPigletBP _returnvalue_11))
            (Variables|/Game/Blueprints/Characters/PigletBP.PigletBP_C|SetCircleSpline _aspiglet_bp_2 (Variables|Default|GetCircleSpline))
            (Default|Init _aspiglet_bp_2)
            (Class|FMODBlueprintStatics|EventInstanceSetParameter (Variables|Default|GetMusic) "Lvl int" 3.0))
          (Default|ActivateSmoke (Variables|Default|GetCircleSpline))
          (CallFunction|FogChargeLoop)
          (CallFunction|StunPiglets 5.0)
          (bind _returnvalue_12 (Class|TAGGameMode|GetGnomeCharacter (Variables|Default|GetGameMode)))
          (Class|GnomeCharacter|InstantMount _returnvalue_12))
        (:4
          ;[1 1 1] Death
          (Default|DeactivateSmoke (Variables|Default|GetCircleSpline))
          (for _array_element (Variables|Default|GetPiglets)
            (bind _aspiglet_bp_3 (Utilities|Casting|CastToPigletBP _array_element))
            (Default|SetMoveOutOfWay _aspiglet_bp_3 true))
          (CallFunction|Death))))))

(fn SpawnFogCharger
  (params (Position :type Vector) (Velocity :type Vector))
  (bind _returnvalue (Game|SpawnActorfromClass "/Game/Blueprints/Characters/Boar/ChargingBoar.ChargingBoar_C" (Math|Transform|MakeTransform Position "0, 0, 0" "2.000000,2.000000,2.000000") "Undefined" 0 0))
  (Default|Charge _returnvalue Velocity))

(fn SetFireEffect
  (params (EffectOn :type Boolean))
  (if EffectOn
    (Components|Activation|Activate (Variables|Default|GetFire1) false)
    (Components|Activation|Activate (Variables|Default|GetFire2) false)
    (Components|Activation|Activate (Variables|Default|GetFire3) false)
    (else
      (Components|Activation|Deactivate (Variables|Default|GetFire1))
      (Components|Activation|Deactivate (Variables|Default|GetFire2))
      (Components|Activation|Deactivate (Variables|Default|GetFire3)))))

(fn StunPiglets
  (params (Time :type Float%20%28single-precision%29))
  (for _array_element (Variables|Default|GetPiglets)
    (bind _aspiglet_bp (Utilities|Casting|CastToPigletBP _array_element))
    (Default|Stun _aspiglet_bp Time)))