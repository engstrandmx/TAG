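; Cow AI character (named as a throwaway test) that trolls can knock flying and gnomes can recruit.
; Troll hits launch it along a vector steered by clamped camera aim, previewed as a predicted arc of particles during hit simulation.
; Gnome interaction affects nearby cows, temporarily setting blackboard target, speed boost and hearts; gnome attacks clear these.
; An AI state switch drives the flying blackboard flag and trail, returning to wandering on landing.
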(event OnInteract(InteractScene)
  (params (TriggeringActor :type Actor%20Object%20Reference))
  (Utilities|Casting|CastToGnomeCharacter TriggeringActor)
  (Class|FMODBlueprintStatics|PlayEventatLocation 0 (Transformation|GetActorTransform))
  (bind _outactors (Collision|SphereOverlapActors (Transformation|GetActorLocation) 2e+02 (Utilities|Array|MakeArray "ObjectTypeQuery3") "/Game/Blueprints/Characters/CowBP_Base.CowBP_Base_C"))
  (for _array_element _outactors
    (bind _ascow_bp_base_1 (Utilities|Casting|CastTotestToBeDeleted _array_element))
    (CallFunction|InteractNoAoE _ascow_bp_base_1 TriggeringActor)
    (CallFunction|InteractNoAoE self)))

(event OnSimulateHit(HittableSceneComponent)
  (params (HittingActor :type Actor%20Object%20Reference) (PowerMultiplier :type Float%20%28single-precision%29) (ForwardVector :type Vector :default "0, 0, 0"))
  (bind _returnvalue (Transformation|GetActorLocation))
  ;[1 1 1] On Simulate
  (Variables|Default|SetRotationHitForce PowerMultiplier)
  (if (Utilities|Enum|NotEqual(Enum) (Variables|Default|GetAI%20State) "VE_Floating")
    (Utilities|FlowControl|Sequence
      (:then_0
        (AI|Components|Blackboard|SetValueasBool (AI|GetBlackboard 0) (Utilities|Name|MakeLiteralName "SimulatingHit") true)
        (Utilities|FlowControl|RetriggerableDelay 1.0)
        (AI|Components|Blackboard|SetValueasBool (AI|GetBlackboard 0) (Utilities|Name|MakeLiteralName "SimulatingHit") false))
      (:then_1
        (Variables|Simulation|SetLineRotation (Transformation|GetActorRotation))
        (bind _returnvector (CallFunction|GenerateHitVector HittingActor PowerMultiplier ForwardVector))
        (bind _result (Math|Integer|IncrementInt (Variables|Default|GetSimulationCount))
          (:%20%20
            (if (== _result 3)
              (Variables|Default|SetSimulationCount 0)
              (Variables|Simulation|SetLaunchVelocity _returnvector)
              (Variables|Simulation|SetLaunchLocation _returnvalue)
              (bind _outpathpositions (Class|GameplayStatics|BlueprintPredictProjectilePathbyTraceChannel _returnvalue _returnvector false 1.0 "ECC_WorldDynamic" false 0 "None" 0.0 1e+01 1.0))
              (for _array_element _outpathpositions
                (Effects|SpawnEmitteratLocation "/Game/ParticleSystems/Beam/P_ArcBall.P_ArcBall" _array_element)
                (Variables|Simulation|SetSimulatingHit true)))))))))

(event OnComponentBeginOverlap(Box)
  (params (OverlappedComponent :type Primitive%20Component%20Object%20Reference) (OtherActor :type Actor%20Object%20Reference) (OtherComp :type Primitive%20Component%20Object%20Reference) (OtherBodyIndex :type Integer) (bFromSweep :type Boolean) (SweepResult :type Hit%20Result%20Structure%20%28by%20ref%29))
  (Utilities|Casting|CastToGnomeCharacter_Base OtherActor)
  (Class|FMODBlueprintStatics|PlayEventatLocation 0 (Transformation|GetActorTransform OtherActor)))

(event OnAttack(InteractScene)
  (params (TriggeringActor :type Actor%20Object%20Reference) (Damages :type Float%20%28single-precision%29))
  (bind _cowcontroller (Variables|Default|GetCowController))
  (bind _returnvalue (AI|GetBlackboard _cowcontroller))
  (Utilities|Casting|CastToGnomeCharacter TriggeringActor)
  (CallFunction|SetSpeed 5e+01 true)
  (AI|Components|Blackboard|ClearValue (AI|GetBlackboard (Variables|Default|GetCowController)) (Utilities|Name|MakeLiteralName "Gnome"))
  (Components|Activation|Deactivate (Variables|Default|GetHeartSpray))
  (AI|Components|Blackboard|SetValueasBool _returnvalue (Utilities|Name|MakeLiteralName "IsFlying") true)
  (Utilities|FlowControl|Delay 13.0)
  (AI|Components|Blackboard|SetValueasBool _returnvalue (Utilities|Name|MakeLiteralName "IsFlying") false))

(event OnComponentHit(HittableSceneComponent)
  (params (HittingActor :type Actor%20Object%20Reference) (PowerMultiplier :type Float%20%28single-precision%29) (ForwardVector :type Vector :default "0, 0, 0"))
  (bind _returnvalue (Transformation|GetActorTransform))
  (bind _launchvelocity (Variables|Simulation|GetLaunchVelocity))
  ;[1 1 1] On Component Hit
  (if (Utilities|Enum|NotEqual(Enum) (Variables|Default|GetAI%20State) "VE_Floating")
    (if (Utilities|ClassIsChildOf (Utilities|GetClass HittingActor) "/Script/TAG.TrollCharacter")
      (Components|Movement|StopMovementImmediately (Variables|Character|GetCharacterMovement))
      (if (Variables|Simulation|GetSimulatingHit)
        (Character|LaunchCharacter _launchvelocity false false)
        (Variables|Default|SetLaunchVector _launchvelocity)
        (else
          (bind _returnvector (CallFunction|GenerateHitVector HittingActor PowerMultiplier ForwardVector))
          (Character|LaunchCharacter (Math|Vector|MakeVector (.X (Math|Vector|BreakVector _returnvector)) (.Y (Math|Vector|BreakVector _returnvector)) 9e+02) false false)
          (Variables|Default|SetLaunchVector (Math|Vector|MakeVector (.X (Math|Vector|BreakVector _returnvector)) (.Y (Math|Vector|BreakVector _returnvector)) 9e+02))))
      (CallFunction|ChangeState "VE_Flying")
      (if (> (Math|Vector|VectorLength (Variables|Default|GetLaunchVector)) 9e+02)
        (Class|FMODBlueprintStatics|PlayEventatLocation 0 _returnvalue)
        (elif (> (Math|Vector|VectorLength (Variables|Default|GetLaunchVector)) 6e+02)
          (Class|FMODBlueprintStatics|PlayEventatLocation 0 _returnvalue)
          (else
            (Class|FMODBlueprintStatics|PlayEventatLocation 0 _returnvalue)))))))

(event Custom|InteractNoAoE
  (params (GnomeRef :type Actor%20Object%20Reference))
  (bind _returnvalue (Utilities|Name|MakeLiteralName "Gnome"))
  (bind _cowcontroller (Variables|Default|GetCowController))
  (bind _cowcontroller_2 (Variables|Default|GetCowController))
  (bind _returnvalue_2 (AI|GetBlackboard _cowcontroller_2))
  (bind _returnvalue_3 (AI|GetBlackboard _cowcontroller))
  (Utilities|Casting|CastToGnomeCharacter_Base GnomeRef)
  (Components|Activation|Activate (Variables|Default|GetHeartSpray) false)
  (CallFunction|SetSpeed 1.5e+02 false)
  (AI|Components|Blackboard|SetValueasObject _returnvalue_2 _returnvalue GnomeRef)
  (AI|Components|Blackboard|SetValueasBool _returnvalue_2 (Utilities|Name|MakeLiteralName "IsFlying") false)
  (Utilities|FlowControl|RetriggerableDelay 15.0)
  (CallFunction|SetSpeed 5e+01 true)
  (AI|Components|Blackboard|ClearValue _returnvalue_2 _returnvalue)
  (Components|Activation|Deactivate (Variables|Default|GetHeartSpray))
  (AI|Components|Blackboard|SetValueasBool _returnvalue_3 (Utilities|Name|MakeLiteralName "IsFlying") true)
  (Utilities|FlowControl|Delay 1e+01)
  (AI|Components|Blackboard|SetValueasBool _returnvalue_3 (Utilities|Name|MakeLiteralName "IsFlying") false))

(event EventBeginPlay
  (bind _returnvalue (Math|Float|MakeLiteralFloat 0.05))
  (Components|Activation|Deactivate (Variables|Default|GetHeartSpray))
  (Transformation|SetActorScale3D (+ (Transformation|GetActorScale3D) (Math|Vector|MakeVector (Math|Random|RandomFloatinRange 0.0 _returnvalue) (Math|Random|RandomFloatinRange 0.0 _returnvalue) 0.0)))
  (bind _ascow_aicontroller (Utilities|Casting|CastToCow_AIController (Pawn|GetController)))
  (Variables|Default|SetCowController _ascow_aicontroller)
  (Utilities|FlowControl|Delay (* (Math|Random|RandomFloat) 3e+01))
  (Class|FMODBlueprintStatics|PlayEventAttached 0 (Variables|Character|GetMesh) "None" "0, 0, 0" "KeepRelativeOffset"))

(event EventOnLanded
  (params (Hit :type Hit%20Result%20Structure%20%28by%20ref%29))
  (Class|FMODBlueprintStatics|PlayEventatLocation 0 (Transformation|GetActorTransform))
  (if (Utilities|Enum|NotEqual(Enum) (Variables|Default|GetAI%20State) "VE_Floating")
    (CallFunction|ChangeState "VE_Wandering")))

(fn ConstructionScript
  (bind _charactermovement (Variables|Character|GetCharacterMovement))
  (Variables|Default|SetIntialSpeed (Variables|/Script/Engine.CharacterMovementComponent|GetMaxWalkSpeed _charactermovement))
  (Variables|Default|SetIntialAcceleration (Class|CharacterMovementComponent|GetMaxAcceleration _charactermovement)))

(fn GenerateLine
  (bind _outpathpositions (Class|GameplayStatics|BlueprintPredictProjectilePathbyTraceChannel (Variables|Simulation|GetLaunchLocation) (Variables|Simulation|GetLaunchVelocity) true 1e+01 "ECC_WorldStatic" false 0 "ForOneFrame" 0.0 15.0 1.0))
  (for _array_element _outpathpositions
    (Effects|SpawnEmitteratLocation "/Game/ParticleSystems/Beam/P_ArcBall.P_ArcBall" _array_element)))

(fn ChangeState
  (params (ToState :type EAiState%20Enum :default "VE_Wandering"))
  (bind _returnvalue (Utilities|Name|MakeLiteralName "IsFlying"))
  (bind _trail (Variables|Default|GetTrail))
  (bind _cowcontroller (Variables|Default|GetCowController))
  (bind _returnvalue_2 (AI|GetBlackboard _cowcontroller))
  (bind _output_get (Variables|Default|SetAI%20State ToState))
  (switch Utilities|FlowControl|Switch|SwitchonEAiState _output_get
    (:VE_Wandering
      (Variables|Simulation|SetSimulatingHit false)
      (AI|Components|Blackboard|SetValueasBool _returnvalue_2 _returnvalue false :!label _label)
      (Variables|Default|SetbInAir false)
      (Components|Activation|Deactivate _trail))
    (:VE_Fleeing
      (goto _label))
    (:VE_Flying
      (AI|Components|Blackboard|SetValueasBool _returnvalue_2 _returnvalue true)
      (Variables|Default|SetbInAir true)
      (Components|Activation|Activate _trail true))
    (:VE_Floating
      (Variables|Default|SetbInAir false))))

(fn SetSpeed
  (params (Amount :type Float%20%28single-precision%29) (Reset :type Boolean))
  (bind _charactermovement (Variables|Character|GetCharacterMovement))
  (if Reset
    (Variables|/Script/Engine.CharacterMovementComponent|SetMaxAcceleration _charactermovement (Variables|Default|GetIntialAcceleration))
    (Variables|/Script/Engine.CharacterMovementComponent|SetMaxWalkSpeed _charactermovement (Variables|Default|GetIntialSpeed))
    (else
      (Variables|/Script/Engine.CharacterMovementComponent|SetMaxAcceleration _charactermovement (+ (Variables|Default|GetIntialAcceleration) Amount))
      (Variables|/Script/Engine.CharacterMovementComponent|SetMaxWalkSpeed _charactermovement (+ (Variables|Default|GetIntialSpeed) Amount)))))

(fn GenerateHitVector
  (params (HittingActor :type Actor%20Object%20Reference) (PowerMultiplier :type Float%20%28single-precision%29) (ForwardVector :type Vector))
  (bind _returnvalue (Transformation|GetActorForwardVector HittingActor))
  (bind _returnvalue_2 (Math|Vector|ProjectVectorontoPlane _returnvalue "0,0.000000,1.000000"))
  (bind _returnvalue_3 (Math|Vector|Normalize _returnvalue_2))
  (bind _returnvalue_4 (Math|Conversions|RotationFromXVector _returnvalue_3))
  (bind (_roll _pitch _yaw) (Math|Rotator|BreakRotator _returnvalue_4))
  (bind _astroll_character_base (Utilities|Casting|CastToTrollCharacter_Base HittingActor))
  (if (< (Math|Float|ClampAngle (.Yaw (Math|Rotator|BreakRotator (Transformation|GetWorldRotation (Variables|/Script/TAG.TAGCharacter|GetFollowCamera _astroll_character_base)))) (- _yaw 7e+01) (+ _yaw 7e+01)) 1.8e+02)
    (return (Math|Vector|RotateVector (Math|Vector|RotateVector (Math|Vector|UnrotateVector (* (* (Math|Vector|Normalize (- (Transformation|GetActorLocation) (+ (Transformation|GetActorLocation HittingActor) (Variables|/Game/Blueprints/Gameplay/Components/HittableSceneComponent.HittableSceneComponent_C|GetVectorOffset (Variables|Default|GetHittableSceneComponent))))) (Variables|/Game/Blueprints/Gameplay/Components/HittableSceneComponent.HittableSceneComponent_C|GetHitForce (Variables|Default|GetHittableSceneComponent))) (* (Math|Float|Clamp(Float) (+ (/ (+ (.Pitch (Math|Rotator|BreakRotator (Transformation|GetWorldRotation (Variables|/Script/TAG.TAGCharacter|GetFollowCamera _astroll_character_base)))) 8e+01) 1.1e+02) 0.5)) PowerMultiplier)) (Math|Conversions|RotationFromXVector (* (* (Math|Vector|Normalize (- (Transformation|GetActorLocation) (+ (Transformation|GetActorLocation HittingActor) (Variables|/Game/Blueprints/Gameplay/Components/HittableSceneComponent.HittableSceneComponent_C|GetVectorOffset (Variables|Default|GetHittableSceneComponent))))) (Variables|/Game/Blueprints/Gameplay/Components/HittableSceneComponent.HittableSceneComponent_C|GetHitForce (Variables|Default|GetHittableSceneComponent))) (* (Math|Float|Clamp(Float) (+ (/ (+ (.Pitch (Math|Rotator|BreakRotator (Transformation|GetWorldRotation (Variables|/Script/TAG.TAGCharacter|GetFollowCamera _astroll_character_base)))) 8e+01) 1.1e+02) 0.5)) PowerMultiplier)))) (Variables|/Game/Blueprints/Gameplay/Components/HittableSceneComponent.HittableSceneComponent_C|GetHitRotation (Variables|Default|GetHittableSceneComponent))) (Math|Rotator|Lerp(Rotator) (Math|Rotator|MakeRotator (.Roll (Math|Rotator|BreakRotator (Math|Conversions|RotationFromXVector (* (* (Math|Vector|Normalize (- (Transformation|GetActorLocation) (+ (Transformation|GetActorLocation HittingActor) (Variables|/Game/Blueprints/Gameplay/Components/HittableSceneComponent.HittableSceneComponent_C|GetVectorOffset (Variables|Default|GetHittableSceneComponent))))) (Variables|/Game/Blueprints/Gameplay/Components/HittableSceneComponent.HittableSceneComponent_C|GetHitForce (Variables|Default|GetHittableSceneComponent))) (* (Math|Float|Clamp(Float) (+ (/ (+ (.Pitch (Math|Rotator|BreakRotator (Transformation|GetWorldRotation (Variables|/Script/TAG.TAGCharacter|GetFollowCamera _astroll_character_base)))) 8e+01) 1.1e+02) 0.5)) PowerMultiplier))))) (+ (.Pitch (Math|Rotator|BreakRotator (Transformation|GetWorldRotation (Variables|/Script/TAG.TAGCharacter|GetFollowCamera _astroll_character_base)))) 1e+01) (.Yaw (Math|Rotator|BreakRotator (Math|Conversions|RotationFromXVector (* (* (Math|Vector|Normalize (- (Transformation|GetActorLocation) (+ (Transformation|GetActorLocation HittingActor) (Variables|/Game/Blueprints/Gameplay/Components/HittableSceneComponent.HittableSceneComponent_C|GetVectorOffset (Variables|Default|GetHittableSceneComponent))))) (Variables|/Game/Blueprints/Gameplay/Components/HittableSceneComponent.HittableSceneComponent_C|GetHitForce (Variables|Default|GetHittableSceneComponent))) (* (Math|Float|Clamp(Float) (+ (/ (+ (.Pitch (Math|Rotator|BreakRotator (Transformation|GetWorldRotation (Variables|/Script/TAG.TAGCharacter|GetFollowCamera _astroll_character_base)))) 8e+01) 1.1e+02) 0.5)) PowerMultiplier)))))) (Math|Rotator|MakeRotator _roll _pitch (Math|Float|ClampAngle (.Yaw (Math|Rotator|BreakRotator (Transformation|GetWorldRotation (Variables|/Script/TAG.TAGCharacter|GetFollowCamera _astroll_character_base)))) (- _yaw 7e+01) (+ _yaw 7e+01))) 0.5 true)))
    (else
      (return (Math|Vector|RotateVector (Math|Vector|RotateVector (Math|Vector|UnrotateVector (* (* (Math|Vector|Normalize (- (Transformation|GetActorLocation) (+ (Transformation|GetActorLocation HittingActor) (Variables|/Game/Blueprints/Gameplay/Components/HittableSceneComponent.HittableSceneComponent_C|GetVectorOffset (Variables|Default|GetHittableSceneComponent))))) (Variables|/Game/Blueprints/Gameplay/Components/HittableSceneComponent.HittableSceneComponent_C|GetHitForce (Variables|Default|GetHittableSceneComponent))) (* (Math|Float|Clamp(Float) (+ (/ (+ (.Pitch (Math|Rotator|BreakRotator (Transformation|GetWorldRotation (Variables|/Script/TAG.TAGCharacter|GetFollowCamera _astroll_character_base)))) 8e+01) 1.1e+02) 0.5)) PowerMultiplier)) (Math|Conversions|RotationFromXVector (* (* (Math|Vector|Normalize (- (Transformation|GetActorLocation) (+ (Transformation|GetActorLocation HittingActor) (Variables|/Game/Blueprints/Gameplay/Components/HittableSceneComponent.HittableSceneComponent_C|GetVectorOffset (Variables|Default|GetHittableSceneComponent))))) (Variables|/Game/Blueprints/Gameplay/Components/HittableSceneComponent.HittableSceneComponent_C|GetHitForce (Variables|Default|GetHittableSceneComponent))) (* (Math|Float|Clamp(Float) (+ (/ (+ (.Pitch (Math|Rotator|BreakRotator (Transformation|GetWorldRotation (Variables|/Script/TAG.TAGCharacter|GetFollowCamera _astroll_character_base)))) 8e+01) 1.1e+02) 0.5)) PowerMultiplier)))) (Variables|/Game/Blueprints/Gameplay/Components/HittableSceneComponent.HittableSceneComponent_C|GetHitRotation (Variables|Default|GetHittableSceneComponent))) (Math|Rotator|Lerp(Rotator) (Math|Rotator|MakeRotator (.Roll (Math|Rotator|BreakRotator (Math|Conversions|RotationFromXVector (* (* (Math|Vector|Normalize (- (Transformation|GetActorLocation) (+ (Transformation|GetActorLocation HittingActor) (Variables|/Game/Blueprints/Gameplay/Components/HittableSceneComponent.HittableSceneComponent_C|GetVectorOffset (Variables|Default|GetHittableSceneComponent))))) (Variables|/Game/Blueprints/Gameplay/Components/HittableSceneComponent.HittableSceneComponent_C|GetHitForce (Variables|Default|GetHittableSceneComponent))) (* (Math|Float|Clamp(Float) (+ (/ (+ (.Pitch (Math|Rotator|BreakRotator (Transformation|GetWorldRotation (Variables|/Script/TAG.TAGCharacter|GetFollowCamera _astroll_character_base)))) 8e+01) 1.1e+02) 0.5)) PowerMultiplier))))) (+ (.Pitch (Math|Rotator|BreakRotator (Transformation|GetWorldRotation (Variables|/Script/TAG.TAGCharacter|GetFollowCamera _astroll_character_base)))) 1e+01) (.Yaw (Math|Rotator|BreakRotator (Math|Conversions|RotationFromXVector (* (* (Math|Vector|Normalize (- (Transformation|GetActorLocation) (+ (Transformation|GetActorLocation HittingActor) (Variables|/Game/Blueprints/Gameplay/Components/HittableSceneComponent.HittableSceneComponent_C|GetVectorOffset (Variables|Default|GetHittableSceneComponent))))) (Variables|/Game/Blueprints/Gameplay/Components/HittableSceneComponent.HittableSceneComponent_C|GetHitForce (Variables|Default|GetHittableSceneComponent))) (* (Math|Float|Clamp(Float) (+ (/ (+ (.Pitch (Math|Rotator|BreakRotator (Transformation|GetWorldRotation (Variables|/Script/TAG.TAGCharacter|GetFollowCamera _astroll_character_base)))) 8e+01) 1.1e+02) 0.5)) PowerMultiplier)))))) (Math|Rotator|MakeRotator _roll _pitch (- (Math|Float|ClampAngle (.Yaw (Math|Rotator|BreakRotator (Transformation|GetWorldRotation (Variables|/Script/TAG.TAGCharacter|GetFollowCamera _astroll_character_base)))) (- _yaw 7e+01) (+ _yaw 7e+01)) 3.6e+02)) 0.5 true))))))

(fn OrderMoveto
  (params (Location :type Vector))
  (AI|Components|Blackboard|SetValueasVector (AI|GetBlackboard 0) (Utilities|Name|MakeLiteralName "OrderMoveLocation") Location))