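; PopupSnakeBP is a snake character Blueprint with a stubbed attack.
; On BeginPlay it caches the game mode as TAGGameMode_BP.
; Its Attack event sphere-traces for Pawns from the actor's location to 200 units straight above, ignoring itself.
; The trace result is not used yet, so the attack has no effect, and the overlap and Tick events are empty.
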(event Custom|Attack
  (bind _returnvalue (Transformation|GetActorLocation))
  (bind _outhit (Collision|SphereTraceForObjects _returnvalue (+ _returnvalue "0, 0,200.000000") 0.0 (Utilities|Array|MakeArray "ObjectTypeQuery3") false (Utilities|Array|MakeArray self) "None")))

(event EventBeginPlay
  (bind _astaggame_mode_bp (Utilities|Casting|CastToTAGGameMode_BP (Game|GetGameMode)))
  (Variables|Default|SetGamemode _astaggame_mode_bp))

(event Collision|EventActorBeginOverlap
  (params (OtherActor :type Actor%20Object%20Reference)))

(event EventTick
  (params (DeltaSeconds :type Float%20%28single-precision%29)))

(fn ConstructionScript)