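; Music handler actor that plays the FMOD puzzle music and adapts it to the active Troll or Gnome character.
; MusicTrigger starts Music_puzzle_1, and Lead_music raises its "Lead" parameter.
; Each trigger's DoOnce precedes the character class check, so any first overlapping actor uses it up.
; Tick polls TAGGameMode's player type, with two mutually resetting DoOnce nodes setting "GnomeMusic" only on character switches.
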(event OnComponentBeginOverlap(MusicTrigger)
  (params (OverlappedComponent :type Primitive%20Component%20Object%20Reference) (OtherActor :type Actor%20Object%20Reference) (OtherComp :type Primitive%20Component%20Object%20Reference) (OtherBodyIndex :type Integer) (bFromSweep :type Boolean) (SweepResult :type Hit%20Result%20Structure%20%28by%20ref%29))
  (bind _returnvalue (Utilities|GetClass OtherActor))
  (Utilities|FlowControl|DoOnce false
    (:Completed
      (if (== _returnvalue "/Game/Blueprints/Characters/Instances/TrollCharacter_Instance.TrollCharacter_Instance_C")
        (Class|FMODBlueprintStatics|LoadEventSampleData "/Game/FMOD/Events/Music/Music_puzzle_1.Music_puzzle_1" :!label _label)
        (bind _returnvalue_2 (Class|FMODBlueprintStatics|PlayEvent2D "/Game/FMOD/Events/Music/Music_puzzle_1.Music_puzzle_1"))
        (bind _astaggame_mode (Utilities|Casting|CastToTAGGameMode (Game|GetGameMode)))
        (bind _returnvalue_3 (Class|TAGGameMode|GetCurrentPlayerType _astaggame_mode))
        (switch Utilities|FlowControl|Switch|SwitchonEPlayerType _returnvalue_3
          (:Troll
            (Utilities|FlowControl|DoOnce false :!label _label_2
              (:Completed
                (Class|FMODBlueprintStatics|EventInstanceSetParameter _returnvalue_2 "GnomeMusic" 0.0)
                (goto _label_3 Reset))))
          (:Gnome
            (Utilities|FlowControl|DoOnce false :!label _label_3
              (:Completed
                (Class|FMODBlueprintStatics|EventInstanceSetParameter _returnvalue_2 "GnomeMusic" 1.0)
                (goto _label_2 Reset)))))
        (elif (== _returnvalue "/Game/Blueprints/Characters/Instances/GnomeCharacter_Instance.GnomeCharacter_Instance_C")
          (goto _label))))))

(event OnComponentBeginOverlap(Lead_music)
  (params (OverlappedComponent :type Primitive%20Component%20Object%20Reference) (OtherActor :type Actor%20Object%20Reference) (OtherComp :type Primitive%20Component%20Object%20Reference) (OtherBodyIndex :type Integer) (bFromSweep :type Boolean) (SweepResult :type Hit%20Result%20Structure%20%28by%20ref%29))
  (bind _returnvalue (Utilities|GetClass OtherActor))
  (Utilities|FlowControl|DoOnce false
    (:Completed
      (if (== _returnvalue "/Game/Blueprints/Characters/Instances/TrollCharacter_Instance.TrollCharacter_Instance_C")
        (Class|FMODBlueprintStatics|EventInstanceSetParameter (stale OnComponentBeginOverlap(MusicTrigger) _returnvalue_2) "Lead" 1.0 :!label _label)
        (elif (== _returnvalue "/Game/Blueprints/Characters/Instances/GnomeCharacter_Instance.GnomeCharacter_Instance_C")
          (goto _label))))))

(event EventBeginPlay)

(event Collision|EventActorBeginOverlap
  (params (OtherActor :type Actor%20Object%20Reference)))

(event EventTick
  (params (DeltaSeconds :type Float%20%28single-precision%29))
  (bind _astaggame_mode (Utilities|Casting|CastToTAGGameMode (Game|GetGameMode)))
  (bind _returnvalue (Class|TAGGameMode|GetCurrentPlayerType _astaggame_mode))
  (switch Utilities|FlowControl|Switch|SwitchonEPlayerType _returnvalue
    (:Troll
      (Utilities|FlowControl|DoOnce false :!label _label
        (:Completed
          (Class|FMODBlueprintStatics|EventInstanceSetParameter (stale OnComponentBeginOverlap(MusicTrigger) _returnvalue_2) "GnomeMusic" 0.0)
          (goto _label_2 Reset))))
    (:Gnome
      (Utilities|FlowControl|DoOnce false :!label _label_2
        (:Completed
          (Class|FMODBlueprintStatics|EventInstanceSetParameter (stale OnComponentBeginOverlap(MusicTrigger) _returnvalue_2) "GnomeMusic" 1.0)
          (goto _label Reset))))))

(fn ConstructionScript)