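; Level 3 audio handler that starts FMOD 2D events, including crickets and wind, and drives their parameters.
; Troll and gnome collide events switch the first event's "Lvl int" and toggle BarnReverb, filtered by active player type (on exit, only while the troll is mounting).
; Switchmusiclvl3 collapses and restores HouseTrigger's scale.
; MusicIntro overlap by either character sets "End" on the first event; End_lvl2 sets it on all three.
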(event OnComponentBeginOverlap(MusicIntro)
  (params (OverlappedComponent :type Primitive%20Component%20Object%20Reference) (OtherActor :type Actor%20Object%20Reference) (OtherComp :type Primitive%20Component%20Object%20Reference) (OtherBodyIndex :type Integer) (bFromSweep :type Boolean) (SweepResult :type Hit%20Result%20Structure%20%28by%20ref%29))
  (bind _returnvalue (Utilities|GetClass OtherActor))
  (if (== _returnvalue "/Game/Blueprints/Characters/Instances/TrollCharacter_Instance.TrollCharacter_Instance_C")
    (Class|FMODBlueprintStatics|EventInstanceSetParameter (stale EventBeginPlay _returnvalue) "End" 1.0 :!label _label)
    (elif (== _returnvalue "/Game/Blueprints/Characters/Instances/GnomeCharacter_Instance.GnomeCharacter_Instance_C")
      (goto _label))))

(event Custom|End_lvl2
  (Class|FMODBlueprintStatics|EventInstanceTriggerCue (stale EventBeginPlay _returnvalue))
  (Class|FMODBlueprintStatics|EventInstanceSetParameter (stale EventBeginPlay _returnvalue) "End" 1.0)
  (Class|FMODBlueprintStatics|EventInstanceSetParameter (stale EventBeginPlay _returnvalue_2) "End" 1.0)
  (Class|FMODBlueprintStatics|EventInstanceSetParameter (stale EventBeginPlay _returnvalue_3) "End" 1.0))

(event Custom|TrollCollide
  (bind _astaggame_mode_bp (Utilities|Casting|CastToTAGGameMode_BP (Game|GetGameMode)))
  (bind _returnvalue (Class|TAGGameMode|GetCurrentPlayerType _astaggame_mode_bp))
  (switch Utilities|FlowControl|Switch|SwitchonEPlayerType _returnvalue
    (:Troll
      (Class|FMODBlueprintStatics|EventInstanceSetParameter (stale EventBeginPlay _returnvalue) "Lvl int" 1.0)
      (Class|FMODAudioComponent|Play (Variables|Default|GetBarn_reverb)))))

(event Custom|GnomeCollide
  (bind _astaggame_mode_bp (Utilities|Casting|CastToTAGGameMode_BP (Game|GetGameMode)))
  (bind _returnvalue (Class|TAGGameMode|GetCurrentPlayerType _astaggame_mode_bp))
  (switch Utilities|FlowControl|Switch|SwitchonEPlayerType _returnvalue
    (:Gnome
      (Class|FMODBlueprintStatics|EventInstanceSetParameter (stale EventBeginPlay _returnvalue) "Lvl int" 1.0)
      (Class|FMODAudioComponent|Play (Variables|Default|GetBarn_reverb)))))

(event Custom|Switchmusiclvl3
  (bind _house_trigger (Variables|Default|GetHouse_trigger))
  (Transformation|SetWorldScale3D _house_trigger "0, 0, 0")
  (Transformation|SetWorldScale3D _house_trigger "1.000000,1.000000,1.000000"))

(event Custom|TrollUncollide
  (bind _outactors (Actor|GetAllActorsOfClass "/Game/Blueprints/Characters/Instances/TrollCharacter_Instance.TrollCharacter_Instance_C"))
  (if (Variables|/Game/Blueprints/Characters/TrollCharacter_Base.TrollCharacter_Base_C|GetMounting (Utilities|Array|Get(acopy) _outactors))
    (bind _astaggame_mode_bp (Utilities|Casting|CastToTAGGameMode_BP (Game|GetGameMode)))
    (bind _returnvalue (Class|TAGGameMode|GetCurrentPlayerType _astaggame_mode_bp))
    (switch Utilities|FlowControl|Switch|SwitchonEPlayerType _returnvalue
      (:Troll
        _)))
  (Class|FMODBlueprintStatics|EventInstanceSetParameter (stale EventBeginPlay _returnvalue) "Lvl int" 2.0)
  (Class|FMODAudioComponent|Stop (Variables|Default|GetBarn_reverb)))

(event Custom|GnomeUncollide
  (bind _outactors (Actor|GetAllActorsOfClass "/Game/Blueprints/Characters/Instances/TrollCharacter_Instance.TrollCharacter_Instance_C"))
  (if (Variables|/Game/Blueprints/Characters/TrollCharacter_Base.TrollCharacter_Base_C|GetMounting (Utilities|Array|Get(acopy) _outactors))
    (bind _astaggame_mode_bp (Utilities|Casting|CastToTAGGameMode_BP (Game|GetGameMode)))
    (bind _returnvalue (Class|TAGGameMode|GetCurrentPlayerType _astaggame_mode_bp))
    (switch Utilities|FlowControl|Switch|SwitchonEPlayerType _returnvalue
      (:Gnome
        _)))
  (Class|FMODBlueprintStatics|EventInstanceSetParameter (stale EventBeginPlay _returnvalue) "Lvl int" 2.0)
  (Class|FMODAudioComponent|Stop (Variables|Default|GetBarn_reverb)))

(event EventBeginPlay
  (bind _returnvalue (Class|FMODBlueprintStatics|PlayEvent2D "/Game/FMOD/Events/Ambience/Crickets.Crickets"))
  (bind _returnvalue_2 (Class|FMODBlueprintStatics|PlayEvent2D))
  (bind _returnvalue_3 (Class|FMODBlueprintStatics|PlayEvent2D "/Game/FMOD/Events/Ambience/Wind.Wind")))

(event EventTick
  (params (DeltaSeconds :type Float%20%28single-precision%29)))

(fn ConstructionScript)