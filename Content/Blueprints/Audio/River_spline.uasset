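; River audio actor that keeps a Water sound source at the part of a spline nearest the player camera.
; Each Tick, it finds the closest spline point to the camera and smoothly moves Water toward it with VInterpTo.
; A CallInEditor ClearSpline button resets the spline to two local points.
; An unconnected debug sphere can visualize the target location.
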(event Custom|ClearSpline
  (bind _spline (Variables|Default|GetSpline))
  (Spline|ClearSplinePoints _spline true)
  (Spline|AddSplinePoint _spline (Math|Vector|MakeVector 0.0 0.0 0.0) "Local" true)
  (Spline|AddSplinePoint _spline (Math|Vector|MakeVector 1e+02 0.0 0.0) "Local" true))

(event EventBeginPlay)

(event Collision|EventActorBeginOverlap
  (params (OtherActor :type Actor%20Object%20Reference)))

(event EventTick
  (params (DeltaSeconds :type Float%20%28single-precision%29))
  (bind _returnvalue (Game|GetPlayerCameraManager 0))
  (Utilities|IsValid _returnvalue
    (:Is%20Valid
      (Transformation|SetWorldLocation (Variables|Default|GetWater) (Math|Interpolation|VInterpTo (Transformation|GetWorldLocation (Variables|Default|GetWater)) (Spline|FindLocationClosesttoWorldLocation (Variables|Default|GetSpline) (Transformation|GetWorldLocation (Variables|/Script/Engine.PlayerCameraManager|GetTransformComponent _returnvalue)) "World") (Utilities|Time|GetWorldDeltaSeconds) 1.0) false false) ; Interp the audio source toward the point on the spline\nthat is nearest to the camera
    )))

(fn ConstructionScript)