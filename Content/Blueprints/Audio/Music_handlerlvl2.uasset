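; Level 2 music handler that plays the Miljö_2 FMOD event from BeginPlay and varies it around a barn trigger.
; Entering or leaving MusicTriggerBarn switches the "Lvl int" parameter, only when the overlapping Troll or Gnome matches the game mode's current player type.
; Switchmusiclvl2 collapses and restores the trigger's scale, forcing overlaps to re-evaluate.
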(event OnComponentEndOverlap(MusicTriggerBarn)
  (params (OverlappedComponent :type Primitive%20Component%20Object%20Reference) (OtherActor :type Actor%20Object%20Reference) (OtherComp :type Primitive%20Component%20Object%20Reference) (OtherBodyIndex :type Integer))
  (bind _returnvalue (Utilities|GetClass OtherActor))
  (if (== _returnvalue "/Game/Blueprints/Characters/Instances/TrollCharacter_Instance.TrollCharacter_Instance_C")
    (bind _astaggame_mode_bp (Utilities|Casting|CastToTAGGameMode_BP (Game|GetGameMode)))
    (bind _returnvalue_2 (Class|TAGGameMode|GetCurrentPlayerType _astaggame_mode_bp))
    (switch Utilities|FlowControl|Switch|SwitchonEPlayerType _returnvalue_2
      (:Troll
        (Class|FMODBlueprintStatics|EventInstanceSetParameter (stale EventBeginPlay _returnvalue) "Lvl int" 1.0 :!label _label)))
    (elif (== _returnvalue "/Game/Blueprints/Characters/Instances/GnomeCharacter_Instance.GnomeCharacter_Instance_C")
      (bind _astaggame_mode_bp_2 (Utilities|Casting|CastToTAGGameMode_BP (Game|GetGameMode)))
      (bind _returnvalue_3 (Class|TAGGameMode|GetCurrentPlayerType _astaggame_mode_bp_2))
      (switch Utilities|FlowControl|Switch|SwitchonEPlayerType _returnvalue_3
        (:Gnome
          (goto _label))))))

(event OnComponentBeginOverlap(MusicTriggerBarn)
  (params (OverlappedComponent :type Primitive%20Component%20Object%20Reference) (OtherActor :type Actor%20Object%20Reference) (OtherComp :type Primitive%20Component%20Object%20Reference) (OtherBodyIndex :type Integer) (bFromSweep :type Boolean) (SweepResult :type Hit%20Result%20Structure%20%28by%20ref%29))
  (bind _returnvalue (Utilities|GetClass OtherActor))
  (if (== _returnvalue "/Game/Blueprints/Characters/Instances/TrollCharacter_Instance.TrollCharacter_Instance_C")
    (bind _astaggame_mode_bp (Utilities|Casting|CastToTAGGameMode_BP (Game|GetGameMode)))
    (bind _returnvalue_2 (Class|TAGGameMode|GetCurrentPlayerType _astaggame_mode_bp))
    (switch Utilities|FlowControl|Switch|SwitchonEPlayerType _returnvalue_2
      (:Troll
        (Class|FMODBlueprintStatics|EventInstanceSetParameter (stale EventBeginPlay _returnvalue) "Lvl int" 2.0 :!label _label)))
    (elif (== _returnvalue "/Game/Blueprints/Characters/Instances/GnomeCharacter_Instance.GnomeCharacter_Instance_C")
      (bind _astaggame_mode_bp_2 (Utilities|Casting|CastToTAGGameMode_BP (Game|GetGameMode)))
      (bind _returnvalue_3 (Class|TAGGameMode|GetCurrentPlayerType _astaggame_mode_bp_2))
      (switch Utilities|FlowControl|Switch|SwitchonEPlayerType _returnvalue_3
        (:Gnome
          (goto _label))))))

(event Custom|Switchmusiclvl2
  (bind _musictriggerbarn (Variables|Default|GetMusicTriggerBarn))
  (Transformation|SetWorldScale3D _musictriggerbarn "0, 0, 0")
  (Transformation|SetWorldScale3D _musictriggerbarn "1.000000,1.000000,1.000000"))

(event EventBeginPlay
  (Class|FMODBlueprintStatics|LoadEventSampleData "/Game/FMOD/Events/Music/Miljö_2.Miljö_2")
  (bind _returnvalue (Class|FMODBlueprintStatics|PlayEvent2D "/Game/FMOD/Events/Music/Miljö_2.Miljö_2")))

(event Collision|EventActorBeginOverlap
  (params (OtherActor :type Actor%20Object%20Reference)))

(fn ConstructionScript)