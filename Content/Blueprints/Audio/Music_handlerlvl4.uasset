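; Level 4 audio handler actor that starts the level's ambience and music through FMOD events.
; On BeginPlay it plays 2D cricket, wind howl and lake water beds, plus Kuling, delayed Kuling and music events placed at component locations.
; The stored instances are later faded or stopped through End_lvl4, which only sets each one's end parameter, leaving the transition to the FMOD events.
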(event Custom|End_lvl4
  (Class|FMODBlueprintStatics|EventInstanceSetParameter (stale EventBeginPlay _returnvalue) "End" 1.0)
  (Class|FMODBlueprintStatics|EventInstanceSetParameter (stale EventBeginPlay _returnvalue_2) "End" 1.0)
  (Class|FMODBlueprintStatics|EventInstanceSetParameter (stale EventBeginPlay _returnvalue_3) "End" 1.0)
  (Class|FMODBlueprintStatics|EventInstanceSetParameter (stale EventBeginPlay _returnvalue_4) "End" 1.0)
  (Class|FMODBlueprintStatics|EventInstanceSetParameter (stale EventBeginPlay _returnvalue_5) "End" 1.0)
  (Class|FMODBlueprintStatics|EventInstanceSetParameter (stale EventBeginPlay _returnvalue_6) "End" 1.0)
  (Class|FMODBlueprintStatics|EventInstanceSetParameter (stale EventBeginPlay _returnvalue_7) "End" 1.0)
  (Class|FMODBlueprintStatics|EventInstanceSetParameter (stale EventBeginPlay _returnvalue_8) "End" 1.0)
  ;[1 1 1] Base_pad
  (Class|FMODBlueprintStatics|EventInstanceSetParameter (stale EventBeginPlay _returnvalue_9) "end" 1.0))

(event EventBeginPlay
  (bind _returnvalue (Class|FMODBlueprintStatics|PlayEvent2D "/Game/FMOD/Events/Ambience/Crickets.Crickets")) ; Crickets
  (bind _returnvalue_2 (Class|FMODBlueprintStatics|PlayEvent2D "/Game/FMOD/Events/Ambience/Cave/Wind/Windhowl_lvl4.Windhowl_lvl4"))
  (bind _returnvalue_3 (Class|FMODBlueprintStatics|PlayEvent2D "/Game/FMOD/Events/Ambience/Swamp/Water_lake.Water_lake"))
  (bind _returnvalue_4 (Class|FMODBlueprintStatics|PlayEventatLocation "/Game/FMOD/Events/Ambience/Kuling_3d_lvl4_2.Kuling_3d_lvl4_2" (Math|Conversions|ToTransform(Vector) (Transformation|GetWorldLocation (Variables|Default|GetKuling%201)))))
  (bind _returnvalue_5 (Class|FMODBlueprintStatics|PlayEventatLocation "/Game/FMOD/Events/Ambience/Kuling_3d_lvl4_Delay.Kuling_3d_lvl4_Delay" (Math|Conversions|ToTransform(Vector) (Transformation|GetWorldLocation (Variables|Default|GetDelay%201)))))
  (bind _returnvalue_6 (Class|FMODBlueprintStatics|PlayEventatLocation "/Game/FMOD/Events/Ambience/Kuling_3d_lvl4_Delay.Kuling_3d_lvl4_Delay" (Math|Conversions|ToTransform(Vector) (Transformation|GetWorldLocation (Variables|Default|GetDelay%202)))))
  (bind _returnvalue_7 (Class|FMODBlueprintStatics|PlayEventatLocation "/Game/FMOD/Events/Ambience/Kuling_3d_lvl4_Delay.Kuling_3d_lvl4_Delay" (Math|Conversions|ToTransform(Vector) (Transformation|GetWorldLocation (Variables|Default|GetDelay%203)))))
  (bind _returnvalue_8 (Class|FMODBlueprintStatics|PlayEventatLocation "/Game/FMOD/Events/Ambience/Kuling_3d_lvl4_Delay.Kuling_3d_lvl4_Delay" (Math|Conversions|ToTransform(Vector) (Transformation|GetWorldLocation (Variables|Default|GetDelay%204)))))
  ;[1 1 1] Base_pad
  (bind _returnvalue_9 (Class|FMODBlueprintStatics|PlayEventatLocation "/Game/FMOD/Events/Music/Music_lvl4.Music_lvl4" (Math|Conversions|ToTransform(Vector) (Transformation|GetWorldLocation (Variables|Default|GetPad))))) ; Kuling_3d
)

(event Collision|EventActorBeginOverlap
  (params (OtherActor :type Actor%20Object%20Reference)))

(event EventTick
  (params (DeltaSeconds :type Float%20%28single-precision%29)))

(fn ConstructionScript)