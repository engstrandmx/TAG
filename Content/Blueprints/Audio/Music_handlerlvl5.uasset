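; Level 5 audio handler that runs the cave music and ambience as FMOD-style events.
; BeginPlay starts the music, room tone and placed wind, drip, waterfall and rumble emitters.
; Trigger overlaps set music level and elevator parameters, and EndLvl5 sets an End parameter on the playing events.
; Troll and gnome inside flags toggle a cave reverb snapshot for the current player type, keeping it while the troll is mounting.
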(event OnComponentBeginOverlap(Music_lvl_1)
  (params (OverlappedComponent :type Primitive%20Component%20Object%20Reference) (OtherActor :type Actor%20Object%20Reference) (OtherComp :type Primitive%20Component%20Object%20Reference) (OtherBodyIndex :type Integer) (bFromSweep :type Boolean) (SweepResult :type Hit%20Result%20Structure%20%28by%20ref%29))
  (Class|FMODBlueprintStatics|EventInstanceSetParameter (stale EventBeginPlay _returnvalue_2) "Lvl int" 1.0))

(event OnComponentBeginOverlap(Music_lvl_2)
  (params (OverlappedComponent :type Primitive%20Component%20Object%20Reference) (OtherActor :type Actor%20Object%20Reference) (OtherComp :type Primitive%20Component%20Object%20Reference) (OtherBodyIndex :type Integer) (bFromSweep :type Boolean) (SweepResult :type Hit%20Result%20Structure%20%28by%20ref%29))
  (Class|FMODBlueprintStatics|EventInstanceSetParameter (stale EventBeginPlay _returnvalue_2) "Lvl int" 2.0))

(event OnComponentBeginOverlap(Music_lvl_3)
  (params (OverlappedComponent :type Primitive%20Component%20Object%20Reference) (OtherActor :type Actor%20Object%20Reference) (OtherComp :type Primitive%20Component%20Object%20Reference) (OtherBodyIndex :type Integer) (bFromSweep :type Boolean) (SweepResult :type Hit%20Result%20Structure%20%28by%20ref%29))
  (Class|FMODBlueprintStatics|EventInstanceSetParameter (stale EventBeginPlay _returnvalue_2) "Lvl int" 3.0))

(event OnComponentBeginOverlap(Music_elevator_end)
  (params (OverlappedComponent :type Primitive%20Component%20Object%20Reference) (OtherActor :type Actor%20Object%20Reference) (OtherComp :type Primitive%20Component%20Object%20Reference) (OtherBodyIndex :type Integer) (bFromSweep :type Boolean) (SweepResult :type Hit%20Result%20Structure%20%28by%20ref%29))
  (Utilities|FlowControl|DoOnce bFromSweep
    (:Completed
      (Class|FMODBlueprintStatics|EventInstanceSetParameter (stale EventBeginPlay _returnvalue_2) "Elevator" 1.0))))

(event OnComponentEndOverlap(Music_elevator_end)
  (params (OverlappedComponent :type Primitive%20Component%20Object%20Reference) (OtherActor :type Actor%20Object%20Reference) (OtherComp :type Primitive%20Component%20Object%20Reference) (OtherBodyIndex :type Integer))
  (Utilities|FlowControl|Delay 3.5)
  (Class|FMODBlueprintStatics|EventInstanceSetParameter (stale EventBeginPlay _returnvalue_2) "Elevator" 2.0))

(event Custom|TrollCollide
  ;[1 1 1] Trigger Events
  (Variables|Default|SetTrollInside true)
  (CallFunction|CheckMusic))

(event Custom|End%20Lvl%205
  (Class|FMODBlueprintStatics|EventInstanceSetParameter (stale EventBeginPlay _returnvalue) "End" 1.0)
  (Class|FMODBlueprintStatics|EventInstanceSetParameter (stale EventBeginPlay _returnvalue_2) "End" 1.0)
  (Class|FMODBlueprintStatics|EventInstanceSetParameter (stale EventBeginPlay _returnvalue_3) "End" 1.0)
  (Class|FMODBlueprintStatics|EventInstanceSetParameter (stale EventBeginPlay _returnvalue_4) "End" 1.0)
  (Class|FMODBlueprintStatics|EventInstanceSetParameter (stale EventBeginPlay _returnvalue_5) "End" 1.0)
  (Class|FMODBlueprintStatics|EventInstanceSetParameter :Name "End" :Value 1.0)
  (Class|FMODBlueprintStatics|EventInstanceSetParameter (stale EventBeginPlay _returnvalue_6) "End" 1.0)
  (Class|FMODBlueprintStatics|EventInstanceSetParameter (stale EventBeginPlay _returnvalue_7) "End" 1.0)
  (Class|FMODBlueprintStatics|EventInstanceSetParameter (stale EventBeginPlay _returnvalue_8) "End" 1.0)
  (Class|FMODBlueprintStatics|EventInstanceSetParameter (stale EventBeginPlay _returnvalue_9) "End" 1.0)
  (Class|FMODBlueprintStatics|EventInstanceSetParameter (stale EventBeginPlay _returnvalue_10) "End" 1.0)
  (Class|FMODBlueprintStatics|EventInstanceSetParameter (stale EventBeginPlay _returnvalue_11) "End" 1.0)
  (Class|FMODBlueprintStatics|EventInstanceSetParameter :Name "End" :Value 1.0)
  (Class|FMODBlueprintStatics|EventInstanceSetParameter (stale EventBeginPlay _returnvalue_12) "End" 1.0)
  (Class|FMODBlueprintStatics|EventInstanceSetParameter (stale EventBeginPlay _returnvalue_13) "End" 1.0)
  (Class|FMODBlueprintStatics|EventInstanceSetParameter (stale EventBeginPlay _returnvalue_14) "End" 1.0)
  (Class|FMODBlueprintStatics|EventInstanceSetParameter (stale EventBeginPlay _returnvalue_15) "End" 1.0)
  (Class|FMODBlueprintStatics|EventInstanceSetParameter (stale EventBeginPlay _returnvalue_16) "End" 1.0))

(event Custom|GnomeCollide
  ;[1 1 1] Trigger Events
  (Variables|Default|SetGnomeInside true)
  (CallFunction|CheckMusic))

(event Custom|Switchmusiclvl3
  ;[1 1 1] Trigger Events
  (CallFunction|CheckMusic))

(event Custom|TrollUncollide
  ;[1 1 1] Trigger Events
  (Variables|Default|SetTrollInside false)
  (CallFunction|CheckMusic))

(event Custom|GnomeUncollide
  ;[1 1 1] Trigger Events
  (Variables|Default|SetGnomeInside false)
  (CallFunction|CheckMusic))

(event Custom|CheckMusic
  (bind _cave_reverb (Variables|Default|GetCave_reverb))
  ;[1 1 1] Check Music
  (bind _astaggame_mode_bp (Utilities|Casting|CastToTAGGameMode_BP (Game|GetGameMode)))
  (bind _returnvalue (Class|TAGGameMode|GetCurrentPlayerType _astaggame_mode_bp))
  (switch Utilities|FlowControl|Switch|SwitchonEPlayerType _returnvalue
    (:Troll
      (if (Variables|Default|GetTrollInside)
        (if (not (Variables|Default|GetSnapshotOn))
          (Variables|Default|SetSnapshotOn true)
          (Class|FMODAudioComponent|Play _cave_reverb :!label _label))
        (elif (Variables|Default|GetSnapshotOn)
          (Variables|Default|SetSnapshotOn false)
          (Class|FMODAudioComponent|Stop _cave_reverb :!label _label_2))))
    (:Gnome
      (if (Variables|Default|GetGnomeInside)
        (if (not (Variables|Default|GetSnapshotOn))
          (Variables|Default|SetSnapshotOn true)
          (goto _label))
        (elif (Variables|Default|GetSnapshotOn)
          (bind _outactors (Actor|GetAllActorsOfClass "/Game/Blueprints/Characters/Instances/TrollCharacter_Instance.TrollCharacter_Instance_C"))
          (if (not (Variables|/Game/Blueprints/Characters/TrollCharacter_Base.TrollCharacter_Base_C|GetMounting (Utilities|Array|Get(acopy) _outactors)))
            (Variables|Default|SetSnapshotOn false)
            (goto _label_2)))))))

(event EventBeginPlay
  (bind _returnvalue (Class|FMODBlueprintStatics|PlayEvent2D "/Game/FMOD/Events/Ambience/Cave/Cave_roomtone.Cave_roomtone"))
  (bind _returnvalue_2 (Class|FMODBlueprintStatics|PlayEvent2D "/Game/FMOD/Events/Music/Music_cave_1.Music_cave_1"))
  (bind _returnvalue_3 (Class|FMODBlueprintStatics|PlayEventatLocation "/Game/FMOD/Events/Ambience/Cave/Wind_howle_cave.Wind_howle_cave" (Math|Conversions|ToTransform(Vector) (Transformation|GetWorldLocation (Variables|Default|Getwind_howling)))))
  (bind _returnvalue_4 (Class|FMODBlueprintStatics|PlayEventatLocation "/Game/FMOD/Events/Ambience/Cave/Wind_howle_cave.Wind_howle_cave" (Math|Conversions|ToTransform(Vector) (Transformation|GetWorldLocation (Variables|Default|Getwind_howling_2)))))
  (bind _returnvalue_5 (Class|FMODBlueprintStatics|PlayEventatLocation "/Game/FMOD/Events/Ambience/Cave/Wind_howle_cave.Wind_howle_cave" (Math|Conversions|ToTransform(Vector) (Transformation|GetWorldLocation (Variables|Default|Getwind_howling_3)))))
  (bind _returnvalue_6 (Class|FMODBlueprintStatics|PlayEventatLocation "/Game/FMOD/Events/Ambience/Cave/Dripping_water.Dripping_water" (Math|Conversions|ToTransform(Vector) (Transformation|GetWorldLocation (Variables|Default|GetDripping)))))
  (bind _returnvalue_7 (Class|FMODBlueprintStatics|PlayEventatLocation "/Game/FMOD/Events/Ambience/Cave/Dripping_water.Dripping_water" (Math|Conversions|ToTransform(Vector) (Transformation|GetWorldLocation (Variables|Default|GetDripping_2)))))
  (bind _returnvalue_8 (Class|FMODBlueprintStatics|PlayEventatLocation "/Game/FMOD/Events/Ambience/Cave/Dripping_water.Dripping_water" (Math|Conversions|ToTransform(Vector) (Transformation|GetWorldLocation (Variables|Default|GetDripping_3)))))
  (bind _returnvalue_9 (Class|FMODBlueprintStatics|PlayEventatLocation "/Game/FMOD/Events/Ambience/Cave/Dripping_water.Dripping_water" (Math|Conversions|ToTransform(Vector) (Transformation|GetWorldLocation (Variables|Default|GetDripping%204)))))
  (bind _returnvalue_10 (Class|FMODBlueprintStatics|PlayEventatLocation "/Game/FMOD/Events/Ambience/Cave/Dripping_water.Dripping_water" (Math|Conversions|ToTransform(Vector) (Transformation|GetWorldLocation (Variables|Default|GetDripping%205)))))
  (bind _returnvalue_11 (Class|FMODBlueprintStatics|PlayEventatLocation "/Game/FMOD/Events/Ambience/Waterfall.Waterfall" (Math|Conversions|ToTransform(Vector) (Transformation|GetWorldLocation (Variables|Default|GetWaterfall)))))
  (bind _returnvalue_12 (Class|FMODBlueprintStatics|PlayEventatLocation "/Game/FMOD/Events/Ambience/Waterfall.Waterfall" (Math|Conversions|ToTransform(Vector) (Transformation|GetWorldLocation (Variables|Default|GetWaterfall_2)))))
  (bind _returnvalue_13 (Class|FMODBlueprintStatics|PlayEventatLocation "/Game/FMOD/Events/Ambience/Cave/Rocks_rumble.Rocks_rumble" (Math|Conversions|ToTransform(Vector) (Transformation|GetWorldLocation (Variables|Default|GetRock_rumble)))))
  (bind _returnvalue_14 (Class|FMODBlueprintStatics|PlayEventatLocation "/Game/FMOD/Events/Ambience/Cave/Rocks_rumble.Rocks_rumble" (Math|Conversions|ToTransform(Vector) (Transformation|GetWorldLocation (Variables|Default|GetRock_rumble_2)))))
  (bind _returnvalue_15 (Class|FMODBlueprintStatics|PlayEventatLocation "/Game/FMOD/Events/Ambience/Cave/Rocks_rumble.Rocks_rumble" (Math|Conversions|ToTransform(Vector) (Transformation|GetWorldLocation (Variables|Default|GetRock_rumble_3)))))
  (bind _returnvalue_16 (Class|FMODBlueprintStatics|PlayEventatLocation "/Game/FMOD/Events/Ambience/Cave/Rocks_rumble.Rocks_rumble" (Math|Conversions|ToTransform(Vector) (Transformation|GetWorldLocation (Variables|Default|GetRock_rumble_4))))))

(event Collision|EventActorBeginOverlap
  (params (OtherActor :type Actor%20Object%20Reference)))

(event EventTick
  (params (DeltaSeconds :type Float%20%28single-precision%29)))

(fn ConstructionScript)