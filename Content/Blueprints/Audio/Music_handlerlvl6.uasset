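; Level 6 music handler that drives FMOD events for the cave and crater sections from trigger overlaps.
; Cave triggers set intensity and end parameters, while StartCrater launches a base track plus puzzle layers.
; Four crater zones track troll and gnome presence in per-zone arrays.
; CheckSwitchMusic toggles base and layer intensity by the active character's presence, rechecked on Switchmusiclvl6, and skips the gnome's switch-off while the troll is Mounting.
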(event OnComponentBeginOverlap(lvl1)
  (params (OverlappedComponent :type Primitive%20Component%20Object%20Reference) (OtherActor :type Actor%20Object%20Reference) (OtherComp :type Primitive%20Component%20Object%20Reference) (OtherBodyIndex :type Integer) (bFromSweep :type Boolean) (SweepResult :type Hit%20Result%20Structure%20%28by%20ref%29))
  (bind _returnvalue (Utilities|GetClass OtherActor))
  ;[1 1 1] Music_pre-crater
  (if (== _returnvalue "/Game/Blueprints/Characters/Instances/TrollCharacter_Instance.TrollCharacter_Instance_C")
    (Class|FMODBlueprintStatics|EventInstanceSetParameter (stale EventBeginPlay _returnvalue) "Lvl int" 1.0 :!label _label)
    (elif (== _returnvalue "/Game/Blueprints/Characters/Instances/GnomeCharacter_Instance.GnomeCharacter_Instance_C")
      (goto _label))))

(event OnComponentBeginOverlap(Lvl2_end)
  (params (OverlappedComponent :type Primitive%20Component%20Object%20Reference) (OtherActor :type Actor%20Object%20Reference) (OtherComp :type Primitive%20Component%20Object%20Reference) (OtherBodyIndex :type Integer) (bFromSweep :type Boolean) (SweepResult :type Hit%20Result%20Structure%20%28by%20ref%29))
  (bind _returnvalue (Utilities|GetClass OtherActor))
  ;[1 1 1] Music_pre-crater
  (if (== _returnvalue "/Game/Blueprints/Characters/Instances/TrollCharacter_Instance.TrollCharacter_Instance_C")
    (Class|FMODBlueprintStatics|EventInstanceSetParameter (stale EventBeginPlay _returnvalue) "End" 1.0 :!label _label)
    (elif (== _returnvalue "/Game/Blueprints/Characters/Instances/GnomeCharacter_Instance.GnomeCharacter_Instance_C")
      (goto _label))))

(event OnComponentEndOverlap(Crater_lvl4)
  (params (OverlappedComponent :type Primitive%20Component%20Object%20Reference) (OtherActor :type Actor%20Object%20Reference) (OtherComp :type Primitive%20Component%20Object%20Reference) (OtherBodyIndex :type Integer))
  (bind _returnvalue (Utilities|GetClass OtherActor))
  (bind _trollinsidea (Variables|Default|GetTrollInsideA))
  (bind _gnomeinsidea (Variables|Default|GetGnomeInsideA))
  (bind _snapshotona (Variables|Default|GetSnapshotOnA))
  ;[1 1 1] Music_crater
  (if (== _returnvalue "/Game/Blueprints/Characters/Instances/TrollCharacter_Instance.TrollCharacter_Instance_C")
    (Utilities|Array|SetArrayElem _trollinsidea 3 false)
    (bind _snapshot_switch (CallFunction|CheckSwitchMusic (Utilities|Array|Get(acopy) _trollinsidea 3) (Utilities|Array|Get(acopy) _gnomeinsidea 3) (Utilities|Array|Get(acopy) (Variables|Default|GetSnapshotOnA) 3) (stale Custom|StartCrater _returnvalue_5) :!label _label))
    (switch int _snapshot_switch
      (:1
        (Utilities|Array|SetArrayElem _snapshotona 3 true))
      (:2
        (Utilities|Array|SetArrayElem _snapshotona 3 false)))
    (elif (== _returnvalue "/Game/Blueprints/Characters/Instances/GnomeCharacter_Instance.GnomeCharacter_Instance_C")
      (Utilities|Array|SetArrayElem _gnomeinsidea 3 false)
      (goto _label))))

(event OnComponentBeginOverlap(Crater_lvl4)
  (params (OverlappedComponent :type Primitive%20Component%20Object%20Reference) (OtherActor :type Actor%20Object%20Reference) (OtherComp :type Primitive%20Component%20Object%20Reference) (OtherBodyIndex :type Integer) (bFromSweep :type Boolean) (SweepResult :type Hit%20Result%20Structure%20%28by%20ref%29))
  (bind _returnvalue (Utilities|GetClass OtherActor))
  (bind _trollinsidea (Variables|Default|GetTrollInsideA))
  (bind _gnomeinsidea (Variables|Default|GetGnomeInsideA))
  (bind _snapshotona (Variables|Default|GetSnapshotOnA))
  ;[1 1 1] Music_crater
  (if (== _returnvalue "/Game/Blueprints/Characters/Instances/TrollCharacter_Instance.TrollCharacter_Instance_C")
    (Utilities|Array|SetArrayElem _trollinsidea 3 true)
    (bind _snapshot_switch (CallFunction|CheckSwitchMusic (Utilities|Array|Get(acopy) _trollinsidea 3) (Utilities|Array|Get(acopy) _gnomeinsidea 3) (Utilities|Array|Get(acopy) (Variables|Default|GetSnapshotOnA) 3) (stale Custom|StartCrater _returnvalue_5) :!label _label))
    (switch int _snapshot_switch
      (:1
        (Utilities|Array|SetArrayElem _snapshotona 3 true))
      (:2
        (Utilities|Array|SetArrayElem _snapshotona 3 false)))
    (elif (== _returnvalue "/Game/Blueprints/Characters/Instances/GnomeCharacter_Instance.GnomeCharacter_Instance_C")
      (Utilities|Array|SetArrayElem _gnomeinsidea 3 true)
      (goto _label))))

(event OnComponentBeginOverlap(Crater_lvl1)
  (params (OverlappedComponent :type Primitive%20Component%20Object%20Reference) (OtherActor :type Actor%20Object%20Reference) (OtherComp :type Primitive%20Component%20Object%20Reference) (OtherBodyIndex :type Integer) (bFromSweep :type Boolean) (SweepResult :type Hit%20Result%20Structure%20%28by%20ref%29))
  (bind _returnvalue (Utilities|GetClass OtherActor))
  (bind _trollinsidea (Variables|Default|GetTrollInsideA))
  (bind _gnomeinsidea (Variables|Default|GetGnomeInsideA))
  (bind _snapshotona (Variables|Default|GetSnapshotOnA))
  ;[1 1 1] Music_crater
  (if (== _returnvalue "/Game/Blueprints/Characters/Instances/TrollCharacter_Instance.TrollCharacter_Instance_C")
    (Utilities|Array|SetArrayElem _trollinsidea 0 true)
    (bind _snapshot_switch (CallFunction|CheckSwitchMusic (Utilities|Array|Get(acopy) _trollinsidea) (Utilities|Array|Get(acopy) _gnomeinsidea) (Utilities|Array|Get(acopy) (Variables|Default|GetSnapshotOnA)) (stale Custom|StartCrater _returnvalue_2) :!label _label))
    (switch int _snapshot_switch
      (:1
        (Utilities|Array|SetArrayElem _snapshotona 0 true))
      (:2
        (Utilities|Array|SetArrayElem _snapshotona 0 false)))
    (elif (== _returnvalue "/Game/Blueprints/Characters/Instances/GnomeCharacter_Instance.GnomeCharacter_Instance_C")
      (Utilities|Array|SetArrayElem _gnomeinsidea 0 true)
      (goto _label))))

(event OnComponentBeginOverlap(Crater_lvl2)
  (params (OverlappedComponent :type Primitive%20Component%20Object%20Reference) (OtherActor :type Actor%20Object%20Reference) (OtherComp :type Primitive%20Component%20Object%20Reference) (OtherBodyIndex :type Integer) (bFromSweep :type Boolean) (SweepResult :type Hit%20Result%20Structure%20%28by%20ref%29))
  (bind _returnvalue (Utilities|GetClass OtherActor))
  (bind _trollinsidea (Variables|Default|GetTrollInsideA))
  (bind _gnomeinsidea (Variables|Default|GetGnomeInsideA))
  (bind _snapshotona (Variables|Default|GetSnapshotOnA))
  ;[1 1 1] Music_crater
  (if (== _returnvalue "/Game/Blueprints/Characters/Instances/TrollCharacter_Instance.TrollCharacter_Instance_C")
    (Utilities|Array|SetArrayElem _trollinsidea 1 true)
    (bind _snapshot_switch (CallFunction|CheckSwitchMusic (Utilities|Array|Get(acopy) _trollinsidea 1) (Utilities|Array|Get(acopy) _gnomeinsidea 1) (Utilities|Array|Get(acopy) (Variables|Default|GetSnapshotOnA) 1) (stale Custom|StartCrater _returnvalue_3) :!label _label))
    (switch int _snapshot_switch
      (:1
        (Utilities|Array|SetArrayElem _snapshotona 1 true))
      (:2
        (Utilities|Array|SetArrayElem _snapshotona 1 false)))
    (elif (== _returnvalue "/Game/Blueprints/Characters/Instances/GnomeCharacter_Instance.GnomeCharacter_Instance_C")
      (Utilities|Array|SetArrayElem _gnomeinsidea 1 true)
      (goto _label))))

(event OnComponentBeginOverlap(Crater_lvl3)
  (params (OverlappedComponent :type Primitive%20Component%20Object%20Reference) (OtherActor :type Actor%20Object%20Reference) (OtherComp :type Primitive%20Component%20Object%20Reference) (OtherBodyIndex :type Integer) (bFromSweep :type Boolean) (SweepResult :type Hit%20Result%20Structure%20%28by%20ref%29))
  (bind _returnvalue (Utilities|GetClass OtherActor))
  (bind _trollinsidea (Variables|Default|GetTrollInsideA))
  (bind _gnomeinsidea (Variables|Default|GetGnomeInsideA))
  (bind _snapshotona (Variables|Default|GetSnapshotOnA))
  ;[1 1 1] Music_crater
  (if (== _returnvalue "/Game/Blueprints/Characters/Instances/TrollCharacter_Instance.TrollCharacter_Instance_C")
    (Utilities|Array|SetArrayElem _trollinsidea 2 true)
    (bind _snapshot_switch (CallFunction|CheckSwitchMusic (Utilities|Array|Get(acopy) _trollinsidea 2) (Utilities|Array|Get(acopy) _gnomeinsidea 2) (Utilities|Array|Get(acopy) (Variables|Default|GetSnapshotOnA) 2) (stale Custom|StartCrater _returnvalue_4) :!label _label))
    (switch int _snapshot_switch
      (:1
        (Utilities|Array|SetArrayElem _snapshotona 2 true))
      (:2
        (Utilities|Array|SetArrayElem _snapshotona 2 false)))
    (elif (== _returnvalue "/Game/Blueprints/Characters/Instances/GnomeCharacter_Instance.GnomeCharacter_Instance_C")
      (Utilities|Array|SetArrayElem _gnomeinsidea 2 true)
      (goto _label))))

(event OnComponentEndOverlap(Crater_lvl1)
  (params (OverlappedComponent :type Primitive%20Component%20Object%20Reference) (OtherActor :type Actor%20Object%20Reference) (OtherComp :type Primitive%20Component%20Object%20Reference) (OtherBodyIndex :type Integer))
  (bind _returnvalue (Utilities|GetClass OtherActor))
  (bind _trollinsidea (Variables|Default|GetTrollInsideA))
  (bind _gnomeinsidea (Variables|Default|GetGnomeInsideA))
  (bind _snapshotona (Variables|Default|GetSnapshotOnA))
  ;[1 1 1] Music_crater
  (if (== _returnvalue "/Game/Blueprints/Characters/Instances/TrollCharacter_Instance.TrollCharacter_Instance_C")
    (Utilities|Array|SetArrayElem _trollinsidea 0 false)
    (bind _snapshot_switch (CallFunction|CheckSwitchMusic (Utilities|Array|Get(acopy) _trollinsidea) (Utilities|Array|Get(acopy) _gnomeinsidea) (Utilities|Array|Get(acopy) (Variables|Default|GetSnapshotOnA)) (stale Custom|StartCrater _returnvalue_2) :!label _label))
    (switch int _snapshot_switch
      (:1
        (Utilities|Array|SetArrayElem _snapshotona 0 true))
      (:2
        (Utilities|Array|SetArrayElem _snapshotona 0 false)))
    (elif (== _returnvalue "/Game/Blueprints/Characters/Instances/GnomeCharacter_Instance.GnomeCharacter_Instance_C")
      (Utilities|Array|SetArrayElem _gnomeinsidea 0 false)
      (goto _label))))

(event OnComponentEndOverlap(Crater_lvl2)
  (params (OverlappedComponent :type Primitive%20Component%20Object%20Reference) (OtherActor :type Actor%20Object%20Reference) (OtherComp :type Primitive%20Component%20Object%20Reference) (OtherBodyIndex :type Integer))
  (bind _returnvalue (Utilities|GetClass OtherActor))
  (bind _trollinsidea (Variables|Default|GetTrollInsideA))
  (bind _gnomeinsidea (Variables|Default|GetGnomeInsideA))
  (bind _snapshotona (Variables|Default|GetSnapshotOnA))
  ;[1 1 1] Music_crater
  (if (== _returnvalue "/Game/Blueprints/Characters/Instances/TrollCharacter_Instance.TrollCharacter_Instance_C")
    (Utilities|Array|SetArrayElem _trollinsidea 1 false)
    (bind _snapshot_switch (CallFunction|CheckSwitchMusic (Utilities|Array|Get(acopy) _trollinsidea 1) (Utilities|Array|Get(acopy) _gnomeinsidea 1) (Utilities|Array|Get(acopy) (Variables|Default|GetSnapshotOnA) 1) (stale Custom|StartCrater _returnvalue_3) :!label _label))
    (switch int _snapshot_switch
      (:1
        (Utilities|Array|SetArrayElem _snapshotona 1 true))
      (:2
        (Utilities|Array|SetArrayElem _snapshotona 1 false)))
    (elif (== _returnvalue "/Game/Blueprints/Characters/Instances/GnomeCharacter_Instance.GnomeCharacter_Instance_C")
      (Utilities|Array|SetArrayElem _gnomeinsidea 1 false)
      (goto _label))))

(event OnComponentEndOverlap(Crater_lvl3)
  (params (OverlappedComponent :type Primitive%20Component%20Object%20Reference) (OtherActor :type Actor%20Object%20Reference) (OtherComp :type Primitive%20Component%20Object%20Reference) (OtherBodyIndex :type Integer))
  (bind _returnvalue (Utilities|GetClass OtherActor))
  (bind _trollinsidea (Variables|Default|GetTrollInsideA))
  (bind _gnomeinsidea (Variables|Default|GetGnomeInsideA))
  (bind _snapshotona (Variables|Default|GetSnapshotOnA))
  ;[1 1 1] Music_crater
  (if (== _returnvalue "/Game/Blueprints/Characters/Instances/TrollCharacter_Instance.TrollCharacter_Instance_C")
    (Utilities|Array|SetArrayElem _trollinsidea 2 false)
    (bind _snapshot_switch (CallFunction|CheckSwitchMusic (Utilities|Array|Get(acopy) _trollinsidea 2) (Utilities|Array|Get(acopy) _gnomeinsidea 2) (Utilities|Array|Get(acopy) (Variables|Default|GetSnapshotOnA) 2) (stale Custom|StartCrater _returnvalue_4) :!label _label))
    (switch int _snapshot_switch
      (:1
        (Utilities|Array|SetArrayElem _snapshotona 2 true))
      (:2
        (Utilities|Array|SetArrayElem _snapshotona 2 false)))
    (elif (== _returnvalue "/Game/Blueprints/Characters/Instances/GnomeCharacter_Instance.GnomeCharacter_Instance_C")
      (Utilities|Array|SetArrayElem _gnomeinsidea 2 false)
      (goto _label))))

(event Custom|TrollCollide
  ;[1 1 1] Music_system_characters
)

(event Custom|StartCrater
  ;[1 1 1] Music_crater
  (Variables|Default|SetinCrater true)
  (bind _returnvalue (Class|FMODBlueprintStatics|PlayEvent2D "/Game/FMOD/Events/Music/Crater_lvl1.Crater_lvl1"))
  (Variables|Default|SetMusic_normal _returnvalue)
  (bind _returnvalue_2 (Class|FMODBlueprintStatics|PlayEvent2D "/Game/FMOD/Events/Crater_woods.Crater_woods"))
  (bind _returnvalue_3 (Class|FMODBlueprintStatics|PlayEvent2D "/Game/FMOD/Events/Crater_strings.Crater_strings"))
  (bind _returnvalue_4 (Class|FMODBlueprintStatics|PlayEvent2D))
  (bind _returnvalue_5 (Class|FMODBlueprintStatics|PlayEvent2D "/Game/FMOD/Events/Crater__brass.Crater__brass")))

(event Custom|GnomeCollide
  ;[1 1 1] Music_system_characters
)

(event Custom|TrollUncollide
  ;[1 1 1] Music_system_characters
)

(event Custom|GnomeUncollide
  ;[1 1 1] Music_system_characters
)

(event Custom|Switchmusiclvl6
  (bind _snapshotona (Variables|Default|GetSnapshotOnA))
  (bind _snapshotona_2 (Variables|Default|GetSnapshotOnA))
  (bind _snapshotona_3 (Variables|Default|GetSnapshotOnA))
  (bind _snapshotona_4 (Variables|Default|GetSnapshotOnA))
  ;[1 1 1] Switch Character Check
  (if (Variables|Default|GetinCrater)
    (Utilities|FlowControl|Sequence
      (:then_0
        (bind _snapshot_switch (CallFunction|CheckSwitchMusic (Utilities|Array|Get(acopy) (Variables|Default|GetTrollInsideA)) (Utilities|Array|Get(acopy) (Variables|Default|GetGnomeInsideA)) (Utilities|Array|Get(acopy) (Variables|Default|GetSnapshotOnA)) (stale Custom|StartCrater _returnvalue_2)))
        (switch int _snapshot_switch
          (:1
            (Utilities|Array|SetArrayElem _snapshotona_2 0 true))
          (:2
            (Utilities|Array|SetArrayElem _snapshotona_2 0 false))))
      (:then_1
        (bind _snapshot_switch_2 (CallFunction|CheckSwitchMusic (Utilities|Array|Get(acopy) (Variables|Default|GetTrollInsideA) 1) (Utilities|Array|Get(acopy) (Variables|Default|GetGnomeInsideA) 1) (Utilities|Array|Get(acopy) (Variables|Default|GetSnapshotOnA) 1) (stale Custom|StartCrater _returnvalue_3)))
        (switch int _snapshot_switch_2
          (:1
            (Utilities|Array|SetArrayElem _snapshotona_3 1 true))
          (:2
            (Utilities|Array|SetArrayElem _snapshotona_3 1 false))))
      (:then_2
        (bind _snapshot_switch_3 (CallFunction|CheckSwitchMusic (Utilities|Array|Get(acopy) (Variables|Default|GetTrollInsideA) 2) (Utilities|Array|Get(acopy) (Variables|Default|GetGnomeInsideA) 2) (Utilities|Array|Get(acopy) (Variables|Default|GetSnapshotOnA) 2) (stale Custom|StartCrater _returnvalue_4)))
        (switch int _snapshot_switch_3
          (:1
            (Utilities|Array|SetArrayElem _snapshotona_4 2 true))
          (:2
            (Utilities|Array|SetArrayElem _snapshotona_4 2 false))))
      (:then_3
        (bind _snapshot_switch_4 (CallFunction|CheckSwitchMusic (Utilities|Array|Get(acopy) (Variables|Default|GetTrollInsideA) 3) (Utilities|Array|Get(acopy) (Variables|Default|GetGnomeInsideA) 3) (Utilities|Array|Get(acopy) (Variables|Default|GetSnapshotOnA) 3) (stale Custom|StartCrater _returnvalue_5)))
        (switch int _snapshot_switch_4
          (:1
            (Utilities|Array|SetArrayElem _snapshotona 3 true))
          (:2
            (Utilities|Array|SetArrayElem _snapshotona 3 false)))))))

(event EventBeginPlay
  ;[1 1 1] Music_pre-crater
  (bind _returnvalue (Class|FMODBlueprintStatics|PlayEvent2D "/Game/FMOD/Events/Music/Cave_lvl6.Cave_lvl6")))

(event Collision|EventActorBeginOverlap
  (params (OtherActor :type Actor%20Object%20Reference)))

(event EventTick
  (params (DeltaSeconds :type Float%20%28single-precision%29)))

(fn ConstructionScript)

(fn CheckSwitchMusic
  (params (Troll%20Inside :type Boolean) (Gnome%20Inside :type Boolean) (Snapshot%20On :type Boolean) (Music_puzzle :type FMOD%20Event%20Instance%20Structure))
  (bind _music_normal (Variables|Default|GetMusic_normal))
  (bind _astaggame_mode_bp (Utilities|Casting|CastToTAGGameMode_BP (Game|GetGameMode)))
  (bind _returnvalue (Class|TAGGameMode|GetCurrentPlayerType _astaggame_mode_bp))
  (switch Utilities|FlowControl|Switch|SwitchonEPlayerType _returnvalue
    (:Troll
      (if Troll%20Inside
        (if (not Snapshot%20On)
          (Class|FMODBlueprintStatics|EventInstanceSetParameter _music_normal "Lvl int" 1.0 :!label _label)
          (Class|FMODBlueprintStatics|EventInstanceSetParameter Music_puzzle "Lvl int" 1.0)
          (return 1))
        (elif Snapshot%20On
          (Class|FMODBlueprintStatics|EventInstanceSetParameter _music_normal "Lvl int" 0.0 :!label _label_2)
          (Class|FMODBlueprintStatics|EventInstanceSetParameter Music_puzzle "Lvl int" 0.0)
          (return 2))))
    (:Gnome
      (if Gnome%20Inside
        (if (not Snapshot%20On)
          (goto _label))
        (elif Snapshot%20On
          (bind _outactors (Actor|GetAllActorsOfClass "/Game/Blueprints/Characters/Instances/TrollCharacter_Instance.TrollCharacter_Instance_C"))
          (if (not (Variables|/Game/Blueprints/Characters/TrollCharacter_Base.TrollCharacter_Base_C|GetMounting (Utilities|Array|Get(acopy) _outactors)))
            (goto _label_2)))))))