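; Destructible target actor that moves back and forth and can be destroyed with a particle effect.
; After a random start delay, MoveTo eases the static mesh between its original position and MoveDist while rotating it, then calls itself with the direction flipped to loop endlessly.
; A Destroy event, with no caller in this graph, spawns an enlarged emitter at the mesh location and removes the actor.
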(event Custom|MoveTo
  (params (Return :type Boolean))
  (if Return
    _
    (else
      _))
  (Components|MoveComponentTo (Variables|Default|GetStaticMesh) (Math|Vector|SelectVector (Variables|Default|GetOriginalPosition) (Variables|Default|GetMoveDist) Return) (Math|Rotator|SelectRotator "0,360.000000, 0" "0,180.000000, 0" Return) true true (Variables|Default|GetTime) false)
  (CallFunction|Moveto (not Return)))

(event Custom|Destroy
  (Effects|SpawnEmitteratLocation (Variables|Default|GetDestroyParticles) (Transformation|GetWorldLocation (Variables|Default|GetStaticMesh)) "0, 0, 0" "4.000000,4.000000,4.000000")
  (Actor|DestroyActor))

(event EventBeginPlay
  (Utilities|FlowControl|Delay (Math|Random|RandomFloatinRange 0.0 (Variables|Default|GetStartDelayRange)))
  (CallFunction|Moveto false))

(event Collision|EventActorBeginOverlap
  (params (OtherActor :type Actor%20Object%20Reference)))

(fn ConstructionScript)