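; Bush actor that plays a rustle sound when the player moves quickly close to it.
; Each Tick measures the player pawn's distance to the location cached at BeginPlay and reads Velocity from the PlayerVelocity material parameter collection.
; High velocity in range fires the Bush FMOD event on the static mesh through a DoOnce.
; The DoOnce re-arms when velocity drops below a lower threshold or the player leaves range, preventing repeated triggers.
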(event EventBeginPlay
  (Variables|Default|SetInitialLocation (Transformation|GetActorLocation)))

(event Collision|EventActorBeginOverlap
  (params (OtherActor :type Actor%20Object%20Reference)))

(event EventTick
  (params (DeltaSeconds :type Float%20%28single-precision%29))
  ;[1 1 1] Bush sound effect trigger
  (if (< (Math|Vector|VectorLength (- (Transformation|GetActorLocation (Pawn|GetControlledPawn (Game|GetPlayerController 0))) (Variables|Default|GetInitialLocation))) 1.3e+02)
    (bind _returnvalue (Rendering|Material|GetScalarParameterValue "/Game/Environment/Models/Undervegitation/PlayerVelocity.PlayerVelocity" "Velocity" :!class /Script/Engine.KismetMaterialLibrary))
    (if (> _returnvalue 0.99)
      (Utilities|FlowControl|DoOnce false :!label _label
        (:Completed
          (Class|FMODBlueprintStatics|PlayEventAttached "/Game/FMOD/Events/Sfx/Bush.Bush" (Variables|Debug|GetStaticMeshComponent) "None" "0, 0, 0" "KeepRelativeOffset")))
      (elif (< _returnvalue 0.7)
        (goto _label Reset)))
    (else
      (goto _label Reset))))

(fn ConstructionScript)