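; HittableSceneComponent is a scene component that makes its parent primitive react to hits from the TrollCharacter.
; On a hit it either calls the ComponentHit dispatcher, when OverrideOnHit is set, or applies a mass-independent impulse to the parent.
; The impulse points away from the attacker's offset location, scaled by HitForce and PowerMultiplier.
; Simulated hits only forward to their own dispatcher when OverrideSimulateHit is set, without checking the attacker's class.
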(event Custom|OnComponentHitEvent
  (params (HittingActor :type Actor%20Object%20Reference) (PowerMultiplier :type Float%20%28single-precision%29))
  (if (== (Utilities|GetClass HittingActor) "/Game/Blueprints/Characters/TrollCharacter.TrollCharacter_C")
    (if (Variables|Default|GetOverrideOnHit)
      (Default|CallOnComponentHit HittingActor PowerMultiplier)
      (else
        (bind _asprimitive_component (Utilities|Casting|CastToPrimitiveComponent (Transformation|GetAttachParent)))
        (Physics|AddImpulse _asprimitive_component (* (* (Math|Vector|Normalize (- (Transformation|GetWorldLocation) (+ (Transformation|GetActorLocation HittingActor) (Variables|Default|GetVectorOffset)))) (Variables|Default|GetHitForce)) PowerMultiplier) "None" true)))))

(event Custom|OnSimulateHitEvent
  (params (HittingActor :type Actor%20Object%20Reference) (PowerMultiplier :type Float%20%28single-precision%29))
  (if (Variables|Default|GetOverrideSimulateHit)
    (Default|CallOnSimulateHit HittingActor PowerMultiplier)))

(event EventTick
  (params (DeltaSeconds :type Float%20%28single-precision%29)))