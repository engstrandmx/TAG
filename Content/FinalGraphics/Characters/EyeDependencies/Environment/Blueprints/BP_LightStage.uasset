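; BP_LightStage is an environment lighting rig combining an HDRI or black skybox, sun, skylight, atmospheric fog and height fog.
; The construction script configures everything from exposed settings, adding template component variants for options like stationary sun, with GlobalBrightness as master multiplier.
; Actor pitch samples curves for sun color and fog brightness; sun color also tints the preview arrow and optionally fog.
; The skylight recaptures the sky unless overridden by a cubemap.
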(fn ConstructionScript
  (bind _returnvalue (Math|Transform|MakeTransform "0, 0, 0"))
  (bind _sundirectionallight (Variables|Default|GetSunDirectionalLight))
  (bind _shadowdistance (Variables|Sun|GetShadowdistance))
  (bind _sundirectionallight_2 (Variables|Default|GetSunDirectionalLight))
  (Utilities|FlowControl|Sequence
    (:then_0
      (Transformation|SetWorldRotation (Variables|Default|GetSkybox) "0, 0, 0" false false)
      (bind _returnvalue_2 (Rendering|Material|CreateDynamicMaterialInstance (select (Variables|HDRI|GetUse_HDRI) (Variables|Default|GetMIC_HDRI) (Variables|Default|GetMIC_Black)) :!class /Script/Engine.KismetMaterialLibrary))
      (Variables|Default|SetSkyboxMaterial _returnvalue_2)
      (Rendering|Material|SetMaterial (Variables|Default|GetSkybox) 0 (Variables|Default|GetSkyboxMaterial))
      (Rendering|Material|SetScalarParameterValue (Variables|Default|GetSkyboxMaterial) "HDRI_Brightness" (* (Variables|HDRI|GetHDRI_Brightness) (Variables|Global|GetGlobalBrightness)) :!class /Script/Engine.MaterialInstanceDynamic)
      (Rendering|Material|SetVectorParameterValue (Variables|Default|GetSkyboxMaterial) "HDRI_Tint" (Variables|HDRI|GetHDRI_Tint) :!class /Script/Engine.MaterialInstanceDynamic)
      (Rendering|Material|SetTextureParameterValue (Variables|Default|GetSkyboxMaterial) "HDRI_Cubemap" (Variables|HDRI|GetHDRI_Cubemap))
      (Rendering|Material|SetScalarParameterValue (Variables|Default|GetSkyboxMaterial) "CubemapRotation" (+ (/ (.Yaw (Math|Rotator|BreakRotator (Transformation|GetWorldRotation (Variables|BP_DayLight|GetPrevisArrow)))) -3.6e+02) (Variables|HDRI|GetHDRI_Rotation)) :!class /Script/Engine.MaterialInstanceDynamic)
      (Rendering|Material|SetScalarParameterValue (Variables|Default|GetSkyboxMaterial) "HDRI_Contrast" (Variables|HDRI|GetHDRI_Contrast) :!class /Script/Engine.MaterialInstanceDynamic))
    (:then_1
      (CallFunction|AtmosphereDensity)
      (Rendering|SetVisibility (Variables|Default|GetAtmosphericFog) (Variables|Atmosphere|GetUseAtmosphere) false)
      (Transformation|SetWorldLocation (Variables|Default|GetAtmosphericFog) (Math|Vector|MakeVector 0.0 0.0 (Variables|Atmosphere|GetAtmosphereAltitude)) false false)
      (Class|AtmosphericFogComponent|SetDefaultBrightness (Variables|Default|GetAtmosphericFog) (* (Variables|Global|GetGlobalBrightness) (Variables|Atmosphere|GetAtmosphereBrightness)))
      (Class|AtmosphericFogComponent|DisableSunDisk (Variables|Default|GetAtmosphericFog) (Variables|Sun|GetDisableSunDisk))
      (Class|AtmosphericFogComponent|DisableGroundScattering (Variables|Default|GetAtmosphericFog) (Variables|Atmosphere|GetDisableGroundScattering))
      (Class|AtmosphericFogComponent|SetSunMultiplier (Variables|Default|GetAtmosphericFog) (Variables|Atmosphere|GetAtmosphereBrightness))
      (Class|AtmosphericFogComponent|SetDefaultLightColor (Variables|Default|GetAtmosphericFog) (Variables|Atmosphere|GetAtmosphereTint))
      (Class|AtmosphericFogComponent|SetDistanceScale (Variables|Default|GetAtmosphericFog) (Variables|Atmosphere|GetAtmosphereDistanceScale))
      (Class|AtmosphericFogComponent|SetDensityMultiplier (Variables|Default|GetAtmosphericFog) (Variables|Atmosphere|GetAtmosphereDensityMultiplier))
      (Class|AtmosphericFogComponent|SetFogMultiplier (Variables|Default|GetAtmosphericFog) (Variables|Atmosphere|GetAtmosphereFogMultiplier)))
    (:then_2
      (if (Variables|Sun|GetUseSunLight)
        (CallFunction|SunMobility)
        (CallFunction|CalculateSunColor)
        (Rendering|Components|Light|SetIntensity (Variables|Default|GetSunDirectionalLight) (* (Variables|Sun|GetSunBrightness) (Variables|Global|GetGlobalBrightness)))
        (Rendering|Components|Light|SetLightColor _sundirectionallight_2 (Variables|Default|GetLightColor) true)
        (Class|DirectionalLightComponent|SetDynamicShadowDistanceMovableLight _sundirectionallight_2 _shadowdistance)
        (Class|DirectionalLightComponent|SetDynamicShadowDistanceStationaryLight _sundirectionallight_2 _shadowdistance)
        (Class|LightComponent|SetEnableLightShaftBloom _sundirectionallight (Variables|LightShafts|GetLightShaftBloom))
        (Class|DirectionalLightComponent|SetEnableLightShaftOcclusion _sundirectionallight (Variables|LightShafts|GetLightShaftOcclusion))
        (Class|DirectionalLightComponent|SetOcclusionMaskDarkness _sundirectionallight (Variables|LightShafts|GetOcclusionMaskDarkness))
        (Class|LightComponent|SetBloomScale _sundirectionallight (Variables|LightShafts|GetBloomScale))
        (Class|LightComponent|SetBloomThreshold _sundirectionallight (Variables|LightShafts|GetBloomThreshold))
        (Class|LightComponent|SetBloomTint _sundirectionallight (Variables|LightShafts|GetBloomTint))
        (Rendering|Components|Light|SetLightFunctionMaterial (Variables|Default|GetSunDirectionalLight) (Variables|Sun|GetLightFunctionMaterial))))
    (:then_3
      (bind _returnvalue_3 (Rendering|Material|CreateDynamicMaterialInstance "/Game/FinalGraphics/Characters/EyeDependencies/Environment/Materials/M_LightStage_Arrows.M_LightStage_Arrows" :!class /Script/Engine.KismetMaterialLibrary))
      (Variables|Default|SetPrevisArrowMaterial _returnvalue_3)
      (Rendering|Material|SetMaterial (Variables|BP_DayLight|GetPrevisArrow) 0 (Variables|Default|GetPrevisArrowMaterial))
      (Rendering|Material|SetVectorParameterValue (Variables|Default|GetPrevisArrowMaterial) "SunColor" (Variables|Default|GetLightColor) :!class /Script/Engine.MaterialInstanceDynamic))
    (:then_4
      (Rendering|SetVisibility (Variables|BP_DayLight|GetExponentialHeightFog1) (Variables|Fog|GetUseFog) false)
      (Class|ExponentialHeightFogComponent|SetFogInscatteringColor (Variables|BP_DayLight|GetExponentialHeightFog1) (* (Math|Color|Lerp(LinearColor) "(R=1.000000,G=1.000000,B=1.000000,A=1.000000)" (Variables|Default|GetLightColor) (Variables|Fog|GetLightColorModulatesFog)) (* (Variables|Fog|GetFogTint) (Math|Conversions|ToLinearColor(Float) (* (Variables|Global|GetGlobalBrightness) (* (Variables|Fog|GetFogBrightness) (Math|Curves|GetFloatValue (Variables|Default|GetFogBrightnessCurve) (CallFunction|NormalizedSunAngle))))))))
      (Class|ExponentialHeightFogComponent|SetFogMaxOpacity (Variables|BP_DayLight|GetExponentialHeightFog1) (Variables|Fog|GetFogMaxOpacity))
      (Class|ExponentialHeightFogComponent|SetFogHeightFalloff (Variables|BP_DayLight|GetExponentialHeightFog1) (Variables|Fog|GetFogHeightFalloff))
      (Class|ExponentialHeightFogComponent|SetFogDensity (Variables|BP_DayLight|GetExponentialHeightFog1) (Variables|Fog|GetFogDensity))
      (Class|ExponentialHeightFogComponent|SetStartDistance (Variables|BP_DayLight|GetExponentialHeightFog1) (Variables|Fog|GetFogStartDistance))
      (Transformation|SetWorldLocation (Variables|BP_DayLight|GetExponentialHeightFog1) (Math|Vector|MakeVector 0.0 0.0 (Variables|Fog|GetFogAltitude)) false false))
    (:then_5
      (if (Variables|SkyLight|GetOverrideSkylight)
        (if (Variables|Default|GetLowerHemisphereIsBlack)
          (bind _returnvalue_4 (AddComponent|AddSkyLightComponent false _returnvalue))
          (Variables|Default|SetSkylightComponentVar _returnvalue_4)
          (else
            (bind _returnvalue_5 (AddComponent|AddSkyLightComponent false))
            (Variables|Default|SetSkylightComponentVar _returnvalue_5)))
        (Class|SkyLightComponent|SetCubemap (Variables|Default|GetSkylightComponentVar) (Variables|SkyLight|GetSkylightHDRI))
        (else
          (bind _returnvalue_6 (AddComponent|AddSkyLightComponent false _returnvalue))
          (Variables|Default|SetSkylightComponentVar _returnvalue_6)
          (Class|SkyLightComponent|RecaptureSky (Variables|Default|GetSkylightComponentVar))))
      (Rendering|Components|Light|SetIntensity (Variables|Default|GetSkylightComponentVar) (* (Variables|SkyLight|GetSkylightIntensity) (Variables|Global|GetGlobalBrightness))))))

(fn CalculateSunColor
  (bind _angle (CallFunction|NormalizedSunAngle))
  (bind _suncolorcurve (Variables|Default|GetSunColorCurve))
  (bind _returnvalue (Math|Curves|GetLinearColorValue _suncolorcurve _angle))
  (bind (_r _g _b) (Math|Color|BreakColor _returnvalue))
  (Variables|Default|SetLightColor (Math|Color|SelectColor (Variables|Sun|GetSunTint) (* (Math|Color|MakeColor _r _g _b) (Variables|Sun|GetSunTint)) (Variables|Sun|GetOverrideSunColor))))

(fn SunMobility
  (bind _returnvalue (Math|Transform|MakeTransform "0, 0, 0"))
  (if (Variables|Sun|GetStationaryLightForSun)
    (bind _returnvalue_2 (AddComponent|AddDirectionalLightComponent false _returnvalue))
    (Variables|Default|SetSunDirectionalLight _returnvalue_2)
    (else
      (bind _returnvalue_3 (AddComponent|AddDirectionalLightComponent false _returnvalue))
      (Variables|Default|SetSunDirectionalLight _returnvalue_3))))

(fn NormalizedSunAngle
  (return (+ (Math|Float|Absolute(Float) (/ (Math|Float|Absolute(Float) (- (.Pitch (Math|Rotator|BreakRotator (Transformation|GetActorRotation))) 9e+01)) 9e+01)) -1.0)))

(fn AtmosphereDensity
  (bind _returnvalue (Math|Transform|MakeTransform "0, 0, 0"))
  (if (Variables|Atmosphere|GetHighDensityAtmosphere)
    (bind _returnvalue_2 (AddComponent|AddAtmosphericFogComponent false _returnvalue))
    (Variables|Default|SetAtmosphericFog _returnvalue_2)
    (Class|AtmosphericFogComponent|SetPrecomputeParams (Variables|Default|GetAtmosphericFog) (Variables|Atmosphere|GetAtmosphereDensityHeight) (Variables|Atmosphere|GetAtmosphereMaxScatteringOrder) (Variables|Atmosphere|GetAtmosphereAltitudeSampleNumber))
    (else
      (bind _returnvalue_3 (AddComponent|AddAtmosphericFogComponent false _returnvalue))
      (Variables|Default|SetAtmosphericFog _returnvalue_3))))