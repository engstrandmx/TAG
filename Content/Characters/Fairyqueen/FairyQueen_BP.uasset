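; Fairy Queen character Blueprint that plays a scripted animation performance on its FairyqueenBase skeletal mesh.
; It loops an idle animation from BeginPlay.
; The TriggerAnimations event switches to a looping conversation, then uses fixed delays to play a one-shot spellcast and return to the conversation loop.
; Animations are set directly with PlayAnimation, while a PlayMontage node for FairyQueenMontage is left unconnected.
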(event Custom|TriggerAnimations
  (Components|Animation|PlayAnimation (Variables|Default|GetFairyqueen_base) "/Game/Characters/Fairyqueen/Fairyqueen_conversation.Fairyqueen_conversation" true)
  (Utilities|FlowControl|Delay 20.3)
  (Components|Animation|PlayAnimation (Variables|Default|GetFairyqueen_base) "/Game/Characters/Fairyqueen/Fairyqueen_spellcasting.Fairyqueen_spellcasting" false)
  (Utilities|FlowControl|Delay 6.0)
  (Components|Animation|PlayAnimation (Variables|Default|GetFairyqueen_base) "/Game/Characters/Fairyqueen/Fairyqueen_conversation.Fairyqueen_conversation" true))

(event EventBeginPlay
  (Components|Animation|PlayAnimation (Variables|Default|GetFairyqueen_base) "/Game/Characters/Fairyqueen/Fairyqueen_idle.Fairyqueen_idle" true))

(event Collision|EventActorBeginOverlap
  (params (OtherActor :type Actor%20Object%20Reference)))

(event EventTick
  (params (DeltaSeconds :type Float%20%28single-precision%29)))

(fn ConstructionScript)